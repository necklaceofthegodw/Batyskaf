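; BP_AI_Pawn is an AI pawn, filed under Eel, that wanders around its spawn point.
; From BeginPlay it loops: pick a random point in a sphere around the start, rotate toward it, then move there.
; Two chained timelines drive rotation and position by lerp, without navigation or collision sweep.
; IsSeeingPlayer is checked before each leg; when true the loop ends, with no chase or restart here.
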(event Custom|MoveToRandomPoint
  (bind _returnvalue (Transformation|GetActorLocation))
  (Variables|Default|SetStartingLocation _returnvalue)
  (Variables|Default|SetCurrentLocation _returnvalue :!label _label)
  (if (not (Variables|Default|GetIsSeeingPlayer?))
    (Variables|Default|SetRandom%20Location (CallFunction|GetRandomLocationinSphere (Variables|Default|GetStartingLocation) 2.5e+03))
    (Variables|Default|SetStartRotation (Transformation|GetActorRotation))
    (bind _rotationz (Timeline|RotatePawn PlayFromStart)
      (:Update
        (Transformation|SetActorRotation (Math|Rotator|Lerp(Rotator) (Variables|Default|GetStartRotation) (Math|Rotator|FindLookatRotation (Variables|Default|GetCurrentLocation) (Variables|Default|GetRandom%20Location)) _rotationz true)))
      (:Finished
        (bind _newtrack_0 (Timeline|MoveTimeline PlayFromStart)
          (:Update
            (Transformation|SetActorLocation (Math|Vector|Lerp(Vector) (Variables|Default|GetCurrentLocation) (Variables|Default|GetRandom%20Location) _newtrack_0) false false))
          (:Finished
            (goto _label)))))))

(event EventBeginPlay
  (CallFunction|MovetoRandomPoint))

(event Collision|EventActorBeginOverlap
  (params (OtherActor :type Actor%20Object%20Reference)))

(event EventTick
  (params (DeltaSeconds :type Float%20%28single-precision%29)))

(fn ConstructionScript)