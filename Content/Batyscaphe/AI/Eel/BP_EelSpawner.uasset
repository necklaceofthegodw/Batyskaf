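; BP_EelSpawner is a placed actor that spawns a single BP_Eel when the player's submarine comes near.
; A looping half-second timer, rather than Tick, polls the submarine pawn's distance against MinDistToPlayer.
; On the first success it spawns the eel at a random point in a sphere around itself, owned by the player pawn, then sets EelSpawned and clears the timer.
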(event Custom|CheckToSpawnEel
  (if (not (Variables|Default|GetEelSpawned))
    (bind _outshouldspawn (CallFunction|IsCloseEnoughtoSpawn))
    (if _outshouldspawn
      (Game|SpawnActorfromClass "/Game/Batyscaphe/AI/Eel/BP_Eel.BP_Eel_C" (Math|Conversions|ToTransform(Vector) (CallFunction|GetRandomLocationinSphere (.Location (Math|Transform|BreakTransform (Transformation|GetActorTransform))) 2.5e+03)) "Undefined" "MultiplyWithRoot" (Game|Player|GetPlayerPawn 0) 0)
      (Variables|Default|SetEelSpawned true)
      (Utilities|Time|ClearandInvalidateTimerbyHandle (Variables|Default|GetEelTimerHandle)))))

(event EventBeginPlay
  (Variables|Default|SetPlayerPawn (CallFunction|GetSubmarinePawn))
  (bind _returnvalue (Utilities|Time|SetTimerbyEvent (EventDispatchers|CreateEvent :!event Custom|CheckToSpawnEel) 0.5 true))
  (Variables|Default|SetEelTimerHandle _returnvalue))

(event Collision|EventActorBeginOverlap
  (params (OtherActor :type Actor%20Object%20Reference)))

(event EventTick
  (params (DeltaSeconds :type Float%20%28single-precision%29)))

(fn ConstructionScript)

(fn IsCloseEnoughtoSpawn
  (bind _playerpawn (Variables|Default|GetPlayerPawn))
  (Utilities|IsValid _playerpawn
    (:Is%20Valid
      (return (< (Math|Vector|Distance(Vector) (Transformation|GetActorLocation _playerpawn) (Transformation|GetActorLocation)) (Variables|Default|GetMinDistToPlayer))))
    (:Is%20Not%20Valid
      (return false))))