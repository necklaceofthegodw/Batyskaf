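; Beholder enemy monster that shoots lasers at the player's submarine and dies to a rocket hit.
; Sphere overlap or pawn sensing starts looping timers to face the submarine and fire impulse-driven bullets, capped by live count, until it leaves range.
; A rocket hit or exceeding despawn distance shares one path: hide the monster, stop timers, scatter depth-based collectibles, then destroy them and itself after a delay.
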(event OnComponentBeginOverlap(Box)
  (params (OverlappedComponent :type Primitive%20Component%20Object%20Reference) (OtherActor :type Actor%20Object%20Reference) (OtherComp :type Primitive%20Component%20Object%20Reference) (OtherBodyIndex :type Integer) (bFromSweep :type Boolean) (SweepResult :type Hit%20Result%20Structure%20%28by%20ref%29))
  (bind _asbp_rocket (Utilities|Casting|CastToBP_Rocket OtherActor))
  (Variables|Default|SetRocketThatHit _asbp_rocket)
  (CallFunction|OnShot (CallFunction|GetSubmarinePawn)))

(event OnSeePawn(PawnSensing)
  (params (Pawn :type Pawn%20Object%20Reference))
  (bind _asbp_submarine_pawn (Utilities|Casting|CastToBP_SubmarinePawn Pawn))
  (Variables|Default|SetPawnSeen _asbp_submarine_pawn)
  (if (not (Utilities|Time|IsValidTimerHandle (Variables|Default|GetRotatePawnHandle)))
    (bind _returnvalue (Utilities|Time|SetTimerbyEvent (delegate Custom|CheckDistanceToPawn) 0.03 true))
    (Variables|Default|SetRotatePawnHandle _returnvalue)
    (Variables|Default|SetIsSeeingPlayer? true)
    (Development|PrintString "KILL")
    (bind _returnvalue_2 (Utilities|Time|SetTimerbyEvent (EventDispatchers|CreateEvent :!event Custom|ShootLasers) 1.0 true))
    (Variables|Default|SetShootLasersHandle _returnvalue_2)
    (if (not (Class|KismetSystemLibrary|TimerExistsHandle (Variables|Default|GetDespawnHandle)))
      (bind _returnvalue_3 (Utilities|Time|SetTimerbyEvent (EventDispatchers|CreateEvent :!event Custom|CheckDespawnDistance) 1.0 true))
      (Variables|Default|SetDespawnHandle _returnvalue_3))))

(event OnComponentBeginOverlap(DetectPawnSphere)
  (params (OverlappedComponent :type Primitive%20Component%20Object%20Reference) (OtherActor :type Actor%20Object%20Reference) (OtherComp :type Primitive%20Component%20Object%20Reference) (OtherBodyIndex :type Integer) (bFromSweep :type Boolean) (SweepResult :type Hit%20Result%20Structure%20%28by%20ref%29))
  (bind _asbp_submarine_pawn (Utilities|Casting|CastToBP_SubmarinePawn OtherActor))
  (Variables|Default|SetPawnSeen _asbp_submarine_pawn)
  (if (not (Utilities|Time|IsValidTimerHandle (Variables|Default|GetRotatePawnHandle)))
    (bind _returnvalue (Utilities|Time|SetTimerbyEvent (delegate Custom|CheckDistanceToPawn) 0.03 true))
    (Variables|Default|SetRotatePawnHandle _returnvalue)
    (Variables|Default|SetIsSeeingPlayer? true)
    (Development|PrintString "KILL")
    (bind _returnvalue_2 (Utilities|Time|SetTimerbyEvent (EventDispatchers|CreateEvent :!event Custom|ShootLasers) 1.0 true))
    (Variables|Default|SetShootLasersHandle _returnvalue_2)
    (if (not (Class|KismetSystemLibrary|TimerExistsHandle (Variables|Default|GetDespawnHandle)))
      (bind _returnvalue_3 (Utilities|Time|SetTimerbyEvent (EventDispatchers|CreateEvent :!event Custom|CheckDespawnDistance) 1.0 true))
      (Variables|Default|SetDespawnHandle _returnvalue_3))))

(event Custom|CheckDistanceToPawn
  (bind _skeletalmesh (Variables|Default|GetSkeletalMesh))
  (bind _pawnseen (Variables|Default|GetPawnSeen))
  (bind _returnvalue (Transformation|GetActorLocation _pawnseen))
  (bind _returnvalue_2 (Transformation|GetActorLocation _pawnseen))
  (bind _returnvalue_3 (Transformation|GetSocketLocation _skeletalmesh "LaserSocket"))
  (bind _returnvalue_4 (Math|Rotator|FindLookatRotation _returnvalue_3 _returnvalue))
  (if (< (Math|Vector|Distance(Vector) (Transformation|GetWorldLocation (Variables|Default|GetBox)) _returnvalue_2) (Variables|Default|GetMaxShootingDistance))
    (Variables|Default|SetBulletSpawnRotation _returnvalue_4)
    (Transformation|SetActorRotation _returnvalue_4)
    (Variables|Default|SetStartLocation _returnvalue_3)
    (Variables|Default|SetEndLocation _returnvalue_2)
    (else
      (Utilities|Time|ClearandInvalidateTimerbyHandle (Variables|Default|GetRotatePawnHandle))
      (Utilities|Time|ClearandInvalidateTimerbyHandle (Variables|Default|GetShootLasersHandle))
      (Variables|Default|SetIsSeeingPlayer? false)
      (Development|PrintString "STOP KILL")
      (CallFunction|MovetoRandomPoint))))

(event Custom|DestroyCollectablesDelayed
  (Utilities|FlowControl|Delay 8.0)
  (for _array_element (Variables|Default|GetCollectablesSpawned)
    (Utilities|IsValid _array_element
      (:Is%20Valid
        (Actor|DestroyActor _array_element))))
  (Utilities|Array|Clear (Variables|Default|GetCollectablesSpawned))
  (Actor|DestroyActor))

(event Custom|ShootBullet
  (params (StartLocation :type Vector) (TargetLocation :type Vector) (BulletRef :type BP%20Laser%20Bullet%20Object%20Reference))
  (Physics|AddImpulse (Variables|/Game/Batyscaphe/AI/Beholder/BP_LaserBullet.BP_LaserBullet_C|GetBox BulletRef) (* (Math|Vector|GetUnitDirection(Vector) StartLocation TargetLocation) (Variables|Default|GetBulletSpeed)) "None" false))

(event Custom|ShootLasers
  (if (< (Utilities|Array|Length (Variables|Default|GetBulletsAlive)) (Variables|Default|GetMaxBulletsAlive))
    (if (Utilities|Time|IsValidTimerHandle (Variables|Default|GetShootLasersHandle))
      (bind _returnvalue (Game|SpawnActorfromClass "/Game/Batyscaphe/AI/Beholder/BP_LaserBullet.BP_LaserBullet_C" (Math|Transform|MakeTransform (Variables|Default|GetStartLocation) (Variables|Default|GetBulletSpawnRotation)) "Undefined" "MultiplyWithRoot" 0 self 0))
      (CallFunction|ShootBullet (Variables|Default|GetStartLocation) (Variables|Default|GetEndLocation) _returnvalue)
      (Utilities|Array|Add (Variables|Default|GetBulletsAlive) _returnvalue))))

(event Custom|CheckDespawnDistance
  (if (> (Transformation|GetDistanceTo (Variables|Default|GetPawnSeen) self) (Variables|Default|GetDespawnDistance))
    (Collision|SetActorEnableCollision false)
    (Development|SetHiddeninGame (Variables|Default|GetSkeletalMesh) true false)
    (Class|PawnSensingComponent|SetSensingUpdatesEnabled (Variables|Default|GetPawnSensing) false)
    (Utilities|Time|ClearandInvalidateTimerbyHandle (Variables|Default|GetDespawnHandle))
    (Utilities|Time|ClearandInvalidateTimerbyHandle (Variables|Default|GetRotatePawnHandle))
    (Utilities|Time|ClearandInvalidateTimerbyHandle (Variables|Default|GetShootLasersHandle))
    (Variables|Default|SetIsSeeingPlayer? false)
    (Utilities|FlowControl|Delay 0.2)
    (CallFunction|SpawnCollectibles)
    (CallFunction|DestroyCollectablesDelayed)))

(event EventBeginPlay
  (|CallParentFunction))

(event Collision|EventActorBeginOverlap
  (params (OtherActor :type Actor%20Object%20Reference))
  (|CallParentFunction OtherActor) ; This node is disabled and will not be called.\nDrag off pins to build functionality.
)

(event EventOnShot
  (params (SubmarineShooting :type BP%20Submarine%20Pawn%20Object%20Reference))
  (Default|CallOnChoiceMade SubmarineShooting true)
  (Default|DestroyProjectile (Variables|Default|GetRocketThatHit))
  (GameplayCue|ExecuteGameplayCueOnActor(Burst) (CallFunction|GetSubmarinePawn) "(TagName=\"GameplayCue.ShotBig\")" (Ability|GameplayCue|MakeGameplayCueParameters :Location (Transformation|GetActorLocation)))
  (Collision|SetActorEnableCollision false)
  (Development|SetHiddeninGame (Variables|Default|GetSkeletalMesh) true false)
  (Class|PawnSensingComponent|SetSensingUpdatesEnabled (Variables|Default|GetPawnSensing) false)
  (Utilities|Time|ClearandInvalidateTimerbyHandle (Variables|Default|GetDespawnHandle))
  (Utilities|Time|ClearandInvalidateTimerbyHandle (Variables|Default|GetRotatePawnHandle))
  (Utilities|Time|ClearandInvalidateTimerbyHandle (Variables|Default|GetShootLasersHandle))
  (Variables|Default|SetIsSeeingPlayer? false)
  (Utilities|FlowControl|Delay 0.2)
  (CallFunction|SpawnCollectibles)
  (CallFunction|DestroyCollectablesDelayed))

(fn ConstructionScript
  (|CallParentFunction))

(fn SpawnCollectibles
  (bind _returnvalue (Transformation|GetActorLocation))
  (for _index (range 0 3)
    (bind _returnvalue_2 (Game|SpawnActorfromClass "/Game/Batyscaphe/Collectables/BP_Collectable2.BP_Collectable2_C" (Math|Conversions|ToTransform(Vector) (CallFunction|GetRandomLocationinSphere _returnvalue 5e+03)) "Undefined" "MultiplyWithRoot" (Game|Player|GetPlayerPawn 0) (CallFunction|GetCollectableTypebyDepth (CallFunction|ConvertLocationZtoDepth (.Z (Math|Vector|BreakVector _returnvalue)))) 0))
    (Utilities|Array|Add (Variables|Default|GetCollectablesSpawned) _returnvalue_2)))

(fn RemoveBullet
  (params (Item :type BP%20Laser%20Bullet%20Object%20Reference%20%28by%20ref%29))
  (Utilities|Array|RemoveItem (Variables|Default|GetBulletsAlive) Item))