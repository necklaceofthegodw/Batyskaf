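; Laser bullet for the Beholder monster that resolves as a hit or a miss against the player's submarine.
; A box overlap with the submarine reports a successful choice event, lowers one of its stats and fires the Shot gameplay cue.
; A short lifetime timer started on BeginPlay reports a failed choice instead.
; Both outcomes deregister the bullet from its parent monster and destroy it, but only while that parent is valid.
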(event OnComponentBeginOverlap(Box)
  (params (OverlappedComponent :type Primitive%20Component%20Object%20Reference) (OtherActor :type Actor%20Object%20Reference) (OtherComp :type Primitive%20Component%20Object%20Reference) (OtherBodyIndex :type Integer) (bFromSweep :type Boolean) (SweepResult :type Hit%20Result%20Structure%20%28by%20ref%29))
  (bind _outsubmarinepawn (CallFunction|GetSubmarinePawn))
  (bind _monsterparent (Variables|Default|GetMonsterParent))
  (bind _asbp_submarine_pawn (Utilities|Casting|CastToBP_SubmarinePawn OtherActor))
  (Default|CallOnChoiceMade _asbp_submarine_pawn true)
  (Default|AddStat (Variables|/Game/Batyscaphe/submarine/BP_SubmarinePawn.BP_SubmarinePawn_C|GetBP_AttributeManager _asbp_submarine_pawn) "NewEnumerator3" -2.0)
  (GameplayCue|ExecuteGameplayCueOnActor(Burst) _outsubmarinepawn "(TagName=\"GameplayCue.Shot\")" (Ability|GameplayCue|MakeGameplayCueParameters :Location (Transformation|GetActorLocation _outsubmarinepawn)))
  (Utilities|IsValid _monsterparent
    (:Is%20Valid
      (Default|RemoveBullet _monsterparent self)
      (Actor|DestroyActor))))

(event Custom|DestroyDelayed
  (bind _monsterparent (Variables|Default|GetMonsterParent))
  (Utilities|FlowControl|Delay 3.0)
  (Default|CallOnChoiceMade (CallFunction|GetSubmarinePawn) false)
  (Utilities|IsValid _monsterparent
    (:Is%20Valid
      (Default|RemoveBullet _monsterparent self)
      (Actor|DestroyActor))))

(event EventBeginPlay
  (CallFunction|DestroyDelayed))

(event Collision|EventActorBeginOverlap
  (params (OtherActor :type Actor%20Object%20Reference)))

(event EventTick
  (params (DeltaSeconds :type Float%20%28single-precision%29)))

(fn ConstructionScript)