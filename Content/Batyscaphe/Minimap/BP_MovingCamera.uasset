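; BP_MovingCamera is a minimap camera actor in the bathyscaphe game that tracks the submarine.
; BeginPlay caches the submarine pawn and the first BP_PipeSystemsSpawner found, though the spawner reference is not used afterwards.
; Each Tick, if the pawn is valid, the actor copies its X and Z while keeping its own Y, following in a fixed plane.
; A SceneCaptureComponent2D show-only call is left unconnected.
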(event EventBeginPlay
  (bind _outactors (Actor|GetAllActorsOfClass "/Game/Batyscaphe/PipeSystem/BP_PipeSystemsSpawner.BP_PipeSystemsSpawner_C"))
  (Variables|Default|SetPipeSystemSpawner (Utilities|Array|Get(acopy) _outactors))
  (Variables|Default|SetSubmarinePawn (CallFunction|GetSubmarinePawn)))

(event Collision|EventActorBeginOverlap
  (params (OtherActor :type Actor%20Object%20Reference)))

(event EventTick
  (params (DeltaSeconds :type Float%20%28single-precision%29))
  (bind _submarinepawn (Variables|Default|GetSubmarinePawn))
  (bind _returnvalue (Transformation|GetActorLocation _submarinepawn))
  (bind (_x _y _z) (Math|Vector|BreakVector _returnvalue))
  (Utilities|IsValid _submarinepawn
    (:Is%20Valid
      (Transformation|SetActorLocation (Math|Vector|MakeVector _x (.Y (Math|Vector|BreakVector (Transformation|GetActorLocation))) _z) false false))))

(fn ConstructionScript)