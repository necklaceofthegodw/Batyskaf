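; Tunnel manager that builds a chain of tunnel parts for the player submarine, starting from a placed part.
; On BeginPlay it spawns BP_TunnelPart actors end to end at each one's down socket.
; MoveTunnelParts recycles the first three parts onto the chain's end and reorders the array, but nothing in this graph actively calls it.
; Debug prints log Z positions, and an unfinished teleport shifting pawn and tunnel upward is disconnected.
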(event EventBeginPlay
  (bind _startingtunnelpart (Variables|Default|GetstartingTunnelPart))
  (bind _asbp_submarine_pawn (Utilities|Casting|CastToBP_SubmarinePawn (Game|Player|GetPlayerPawn 0)))
  (Variables|Default|SetSubmarinePawn _asbp_submarine_pawn)
  (Utilities|IsValid _startingtunnelpart
    (:Is%20Valid
      (Utilities|Array|Add (Variables|Default|GetTunnelParts) _startingtunnelpart)
      (CallFunction|SpawnTunnelParts (Default|GetSocketTransformDown _startingtunnelpart)))
    (:Is%20Not%20Valid
      (Development|PrintString "Tunnel Manager: assign starting tunnel part"))))

(event Collision|EventActorBeginOverlap
  (params (OtherActor :type Actor%20Object%20Reference)))

(event EventTick
  (params (DeltaSeconds :type Float%20%28single-precision%29)))

(fn ConstructionScript)

(fn SpawnTunnelParts
  (params (SpawnTransform :type Transform))
  (LocalVariables|SetCurrentSpawnTransformL SpawnTransform)
  (for _index (range 0 8)
    (bind _returnvalue (Game|SpawnActorfromClass "/Game/Batyscaphe/World/BP_TunnelPart.BP_TunnelPart_C" (LocalVariables|GetCurrentSpawnTransformL) "Undefined" "MultiplyWithRoot" 0 0))
    (LocalVariables|SetCurrentSpawnTransformL (Default|GetSocketTransformDown _returnvalue))
    (Utilities|Array|Add (Variables|Default|GetTunnelParts) _returnvalue))
  (Development|PrintString " tunnel parts Z val: ")
  (for _array_element (Variables|Default|GetTunnelParts)
    (Development|PrintString (Utilities|String|Append "    " (Utilities|String|ToString(Float) (.Z (Math|Vector|BreakVector (.Location (Math|Transform|BreakTransform (Transformation|GetActorTransform _array_element)))))) "     ") true true "(R=1.000000,G=0.217256,B=0.848903,A=1.000000)" 1e+01)))

(fn MoveTunnelParts
  ;[0.15 0.15 0.15 0.5] add parts to move
  (for _index (range 0 2)
    (Utilities|Array|Add (LocalVariables|GetTunnelPartsToMoveL) (Utilities|Array|Get(acopy) (Variables|Default|GetTunnelParts) _index)))
  ;[0.15 0.15 0.15 0.5] attach first 3 tunnel parts starting from the last previous tunnel part
  (LocalVariables|SetLastTunnelL (Utilities|Array|Get(acopy) (Variables|Default|GetTunnelParts) (Utilities|Array|LastIndex (Variables|Default|GetTunnelParts))))
  (for _array_element (LocalVariables|GetTunnelPartsToMoveL)
    (Transformation|SetActorTransform _array_element (Default|GetSocketTransformDown (LocalVariables|GetLastTunnelL)))
    (LocalVariables|SetLastTunnelL _array_element))
  ;[0.15 0.15 0.15 0.5] reorder tunnel parts in the array
  (for _index_2 (range 3 9)
    (Utilities|Array|Add (LocalVariables|GetTunnelPartsL) (Utilities|Array|Get(acopy) (Variables|Default|GetTunnelParts) _index_2)))
  (for _array_element_2 (LocalVariables|GetTunnelPartsToMoveL)
    (Utilities|Array|Add (LocalVariables|GetTunnelPartsL) _array_element_2))
  (Variables|Default|SetTunnelParts (LocalVariables|GetTunnelPartsL))
  (Development|PrintString "New tunnel parts Z val: ")
  (for _array_element_3 (Variables|Default|GetTunnelParts)
    (Development|PrintString (Utilities|String|Append "    " (Utilities|String|ToString(Float) (.Z (Math|Vector|BreakVector (.Location (Math|Transform|BreakTransform (Transformation|GetActorTransform _array_element_3)))))) "     ") true true "(R=0.533881,G=1.000000,B=0.389840,A=1.000000)" 1e+01))
  (Development|PrintString "Pawn Z val: ")
  (Development|PrintString (Utilities|String|Append "    " (Utilities|String|ToString(Float) (.Z (Math|Vector|BreakVector (.Location (Math|Transform|BreakTransform (Transformation|GetActorTransform (Variables|Default|GetSubmarinePawn))))))) "     ") true true "(R=0.533881,G=1.000000,B=0.389840,A=1.000000)" 1e+01))