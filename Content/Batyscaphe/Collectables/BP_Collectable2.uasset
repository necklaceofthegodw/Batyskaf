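; BP_Collectable2 is an interactable pickup in the submarine game that pays out money.
; Its construction script finds the DT_Collectables row matching its CollectableType, then synchronously loads and applies that row's mesh and first material.
; StartInteract applies an outline overlay material and immediately adds the row's MarketPrice to the submarine game instance, without removing the actor.
; EndInteract clears the outline.
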(event EventBeginPlay)

(event Collision|EventActorBeginOverlap
  (params (OtherActor :type Actor%20Object%20Reference)))

(event EventTick
  (params (DeltaSeconds :type Float%20%28single-precision%29)))

(event EventStartInteract
  (CallFunction|HighlightMesh true)
  (CallFunction|Collect))

(event EventEndInteract
  (CallFunction|HighlightMesh false))

(fn ConstructionScript
  (bind _sm_collectablemesh (Variables|Default|GetSM_CollectableMesh))
  (bind _outrownames (DataTable|GetDataTableRowNames "/Game/Batyscaphe/Collectables/Data/DT_Collectables.DT_Collectables"))
  (for _array_element _outrownames
    (bind _returnvalue (Utilities|GetDataTableRow "/Game/Batyscaphe/Collectables/Data/DT_Collectables.DT_Collectables" _array_element)
      (:then
        (if (Utilities|Enum|Equal(Enum) (.Type (Utilities|Struct|BreakS_Collectable _returnvalue)) (Variables|Default|GetCollectableType))
          (bind _output_get (Variables|Default|SetCollectableRow _returnvalue))
          (bind _returnvalue_2 (Utilities|LoadAssetBlocking (.StaticMesh (Utilities|Struct|BreakS_Collectable _output_get))))
          (bind _asstatic_mesh (Utilities|Casting|CastToStaticMesh _returnvalue_2))
          (Components|StaticMesh|SetStaticMesh _sm_collectablemesh _asstatic_mesh)
          (Rendering|Material|SetMaterial _sm_collectablemesh 0 (Rendering|Material|GetMaterial _asstatic_mesh 0)))))))

(fn Collect
  (Default|AddMoney (CallFunction|GetSubmarineGameInstance) (.MarketPrice (Utilities|Struct|BreakS_Collectable (Variables|Default|GetCollectableRow))))
  (Development|PrintString "collected"))

(fn HighlightMesh
  (params (IsHighlighting :type Boolean))
  (Rendering|Material|SetOverlayMaterial (Variables|Default|GetSM_CollectableMesh) (select IsHighlighting "/Game/Batyscaphe/Collectables/M_OutlineInst.M_OutlineInst" 0) :!class /Script/Engine.MeshComponent))