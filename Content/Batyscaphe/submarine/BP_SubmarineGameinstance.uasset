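; Submarine game instance that holds money, energy, upgrades and level progress, loading them from a save slot on init or creating a new save.
; Setters fire change calls for money and upgrades; saves write to disk only when IsGameSaved is set.
; LoadNewLevel halts the pawn, advances the level index and streams in the next level behind a HUD screen.
; The index is never copied into the save object here, and the win screen is a TODO.
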(event Custom|LoadNewLevel
  (bind _outsubmarinepawn (CallFunction|GetSubmarinePawn))
  (Input|DisableInput _outsubmarinepawn (Game|GetPlayerController 0))
  (Components|Movement|StopMovementImmediately (Variables|/Game/Batyscaphe/submarine/BP_SubmarinePawn.BP_SubmarinePawn_C|GetFloatingPawnMovement _outsubmarinepawn))
  (Class|Pawn|ConsumeMovementInputVector _outsubmarinepawn)
  (Variables|Default|SetLevelToUnload (CallFunction|GetCurrentLevelName))
  (Save|AddandSaveCurrentLevel)
  (Default|ShowStartOverScreen (CallFunction|GetSubmarineHUDWidget) true true)
  (Game|LoadStreamLevel(byName) (CallFunction|GetCurrentLevelName) true true)
  (Input|EnableInput _outsubmarinepawn (Game|GetPlayerController 0))
  (Default|ShowStartOverScreen (CallFunction|GetSubmarineHUDWidget) false true))

(event EventInit
  (save|LoadDatafromSave))

(fn UpdateMoney
  (params (Money :type Integer))
  (bind _output_get (Variables|Save|SetMoney Money))
  (Default|CallOnMoneyChanged _output_get))

(fn UpdateUpgradesandLevels
  (params (UpgradesAndLevels :type Map%20of%20E_UpgradeType%20Enums%20to%20Integers :default "NewEnumerator0"))
  (bind _output_get (Variables|Save|SetUpgradesAndLevels UpgradesAndLevels))
  (Default|CallOnUpgradesandLevelsChanged _output_get))

(fn LoadDatafromSave
  (bind _savegameslot (Variables|Save|GetSaveGameSlot))
  (bind _returnvalue (SaveGame|DoesSaveGameExist _savegameslot))
  (if _returnvalue
    (bind _returnvalue_2 (SaveGame|LoadGamefromSlot _savegameslot))
    (bind _asbp_save_game (Utilities|Casting|CastToBP_SaveGame _returnvalue_2))
    (bind _output_get (Variables|Save|SetBP_SaveGame _asbp_save_game))
    (Variables|Save|SetUpgradesAndLevels (Variables|/Game/Batyscaphe/UI/UpgradeSystem/BP_SaveGame.BP_SaveGame_C|GetUpgradesAndLevels _output_get))
    (Variables|Save|SetMoney (Variables|/Game/Batyscaphe/UI/UpgradeSystem/BP_SaveGame.BP_SaveGame_C|GetMoney _output_get))
    (Variables|Default|SetisGameSaved (Variables|/Game/Batyscaphe/UI/UpgradeSystem/BP_SaveGame.BP_SaveGame_C|GetIsGameSaved _output_get))
    (Variables|Save|SetLevelIndex (Variables|/Game/Batyscaphe/UI/UpgradeSystem/BP_SaveGame.BP_SaveGame_C|GetLevelIndex _output_get))
    (else
      (bind _returnvalue_3 (SaveGame|CreateSaveGameObject "/Game/Batyscaphe/UI/UpgradeSystem/BP_SaveGame.BP_SaveGame_C"))
      (Variables|Save|SetBP_SaveGame _returnvalue_3)
      (Development|PrintString "create save slot")
      ;[0.15 0.15 0.15 0.5] testing initial value
      (Variables|Save|SetMoney 1800))))

(fn SaveUpgradeData
  (params (UpgradesAndLevels :type Map%20of%20E_UpgradeType%20Enums%20to%20Integers :default "NewEnumerator0") (Money :type Integer))
  (bind _bp_savegame (Variables|Save|GetBP_SaveGame))
  (Variables|Save|SetUpgradesAndLevels UpgradesAndLevels)
  (Variables|Save|SetMoney Money)
  (Variables|/Game/Batyscaphe/UI/UpgradeSystem/BP_SaveGame.BP_SaveGame_C|SetUpgradesAndLevels _bp_savegame (Variables|Save|GetUpgradesAndLevels))
  (Variables|/Game/Batyscaphe/UI/UpgradeSystem/BP_SaveGame.BP_SaveGame_C|SetMoney _bp_savegame (Variables|Save|GetMoney))
  (Variables|/Game/Batyscaphe/UI/UpgradeSystem/BP_SaveGame.BP_SaveGame_C|SetIsGameSaved _bp_savegame (Variables|Default|GetisGameSaved))
  (if (Variables|Default|GetisGameSaved)
    (SaveGame|SaveGametoSlot _bp_savegame (Variables|Save|GetSaveGameSlot))
    (Development|PrintString "save game")))

(fn DeleteSave
  (SaveGame|DeleteGameinSlot (Variables|Save|GetSaveGameSlot)))

(fn AddMoney
  (params (MoneyAdded :type Integer))
  (bind _output_get (Variables|Save|SetMoney (+ (Variables|Save|GetMoney) MoneyAdded)))
  (Default|CallOnMoneyChanged _output_get))

(fn AddEnergy
  (params (EnergyToAdd :type Float%20%28double-precision%29))
  (Variables|Default|SetEnergy (Math|Float|Clamp(Float) (+ (Variables|Default|GetEnergy) EnergyToAdd))))

(fn AddandSaveCurrentLevel
  (if (> (+ (Variables|Save|GetLevelIndex) 1) (- (Utilities|Array|Length (Variables|Default|GetLevelNames)) 1))
    ;[0.15 0.15 0.15 0.5] TODO add win screen
    (Development|PrintString "YOU WON, congratulations")
    (else
      (Math|Integer|IncrementInt (Variables|Save|GetLevelIndex)
        (:%20%20
          _))))
  (if (Variables|Default|GetisGameSaved)
    (SaveGame|SaveGametoSlot (Variables|Save|GetBP_SaveGame) (Variables|Save|GetSaveGameSlot))
    (Development|PrintString "save game")))

(fn GetCurrentLevelName
  (return (Utilities|Array|Get(acopy) (Variables|Default|GetLevelNames) (Variables|Save|GetLevelIndex))))

(fn GetPreviousLevelName
  (return (Utilities|Array|Get(acopy) (Variables|Default|GetLevelNames) (Math|Integer|Clamp(Integer) (- (Variables|Save|GetLevelIndex) 1) 0 4))))