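; Pawn component that manages the submarine's upgradeable stats and abilities through the Gameplay Ability System.
; On BeginPlay it grants abilities, activating monitoring ones once, then sets each stat from DT_Upgrades using levels stored in the game instance.
; SetStat, AddStat and AddStatDOT switch on upgrade type to apply override, additive or DOT GameplayEffects, with magnitudes passed by SetByCaller tags.
; Separate max battery capacity functions exist outside those switches.
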(event EventBeginPlay
  (bind _asbp_submarine_pawn (Utilities|Casting|CastToBP_SubmarinePawn (Components|GetOwner)))
  (Variables|Default|SetSubmarinePawn _asbp_submarine_pawn)
  (CallFunction|InitAbilities)
  (CallFunction|LoadSavedStats))

(event EventTick
  (params (DeltaSeconds :type Float%20%28single-precision%29)))

(fn AddSpeedDOT
  (params (SpeedToAdd :type Float%20%28single-precision%29))
  (bind _submarinepawn (Variables|Default|GetSubmarinePawn))
  (bind _returnvalue (Ability|GetAbilitySystemComponent _submarinepawn))
  (Utilities|IsValid _returnvalue
    (:Is%20Valid
      (bind _returnvalue_2 (Ability|GameplayEffect|AssignTagSetbyCallerMagnitude (GameplayEffects|MakeOutgoingSpec _returnvalue "/Game/Batyscaphe/GAS/GameplayEffects/DOTs/GE_AddMaxSpeedDOT.GE_AddMaxSpeedDOT_C" 1.0 (GameplayEffects|MakeEffectContext _returnvalue)) "(TagName=\"Gamedata.MaxSpeed\")" SpeedToAdd))
      (GameplayEffects|ApplyGameplayEffectSpecToSelf _returnvalue _returnvalue_2))))

(fn AddStatDOT
  (params (UpgradeType :type E_UpgradeType%20Enum :default "NewEnumerator0") (Val :type Float%20%28double-precision%29))
  (switch Utilities|FlowControl|Switch|SwitchonE_UpgradeType UpgradeType
    (:NewEnumerator0
      (DOTs|AddSpeedDOT Val))
    (:NewEnumerator1
      ;[0.15 0.15 0.15 0.5] TODO add postAttribute change and clamp to a min val
      (DOTs|AddAerodynamicsDOT Val))
    (:NewEnumerator2
      (DOTs|AddAccelerationDOT Val))
    (:NewEnumerator3
      (DOTs|AddBatteryCapacityDOT Val))
    (:NewEnumerator4
      (DOTs|AddSonarRangeDOT Val))
    (:NewEnumerator5
      ;[0.15 0.15 0.15 0.5] change to int
      (DOTs|AddCapacityDOT Val))))

(fn AddAccelerationDOT
  (params (AccelerationToAdd :type Float%20%28single-precision%29))
  (bind _submarinepawn (Variables|Default|GetSubmarinePawn))
  (bind _returnvalue (Ability|GetAbilitySystemComponent _submarinepawn))
  (Utilities|IsValid _returnvalue
    (:Is%20Valid
      (bind _returnvalue_2 (Ability|GameplayEffect|AssignTagSetbyCallerMagnitude (GameplayEffects|MakeOutgoingSpec _returnvalue "/Game/Batyscaphe/GAS/GameplayEffects/DOTs/GE_AddMaxAccelerationDOT.GE_AddMaxAccelerationDOT_C" 1.0 (GameplayEffects|MakeEffectContext _returnvalue)) "(TagName=\"Gamedata.MaxAcceleration\")" AccelerationToAdd))
      (GameplayEffects|ApplyGameplayEffectSpecToSelf _returnvalue _returnvalue_2))))

(fn AddAerodynamicsDOT
  (params (AerodynamicsToAdd :type Float%20%28single-precision%29))
  (bind _submarinepawn (Variables|Default|GetSubmarinePawn))
  (bind _returnvalue (Ability|GetAbilitySystemComponent _submarinepawn))
  (Utilities|IsValid _returnvalue
    (:Is%20Valid
      (bind _returnvalue_2 (Ability|GameplayEffect|AssignTagSetbyCallerMagnitude (GameplayEffects|MakeOutgoingSpec _returnvalue "/Game/Batyscaphe/GAS/GameplayEffects/DOTs/GE_AddAerodynamicsDOT.GE_AddAerodynamicsDOT_C" 1.0 (GameplayEffects|MakeEffectContext _returnvalue)) "(TagName=\"Gamedata.Aerodynamics\")" AerodynamicsToAdd))
      (GameplayEffects|ApplyGameplayEffectSpecToSelf _returnvalue _returnvalue_2))))

(fn AddMaxBatteryCapacityDOT
  (params (BatteryCapacityToAdd :type Float%20%28single-precision%29))
  (bind _submarinepawn (Variables|Default|GetSubmarinePawn))
  (bind _returnvalue (Ability|GetAbilitySystemComponent _submarinepawn))
  (Utilities|IsValid _returnvalue
    (:Is%20Valid
      (bind _returnvalue_2 (Ability|GameplayEffect|AssignTagSetbyCallerMagnitude (GameplayEffects|MakeOutgoingSpec _returnvalue "/Game/Batyscaphe/GAS/GameplayEffects/DOTs/GE_AddMaxBatteryCapacityDOT.GE_AddMaxBatteryCapacityDOT_C" 1.0 (GameplayEffects|MakeEffectContext _returnvalue)) "(TagName=\"Gamedata.BatteryCapacity\")" BatteryCapacityToAdd))
      (GameplayEffects|ApplyGameplayEffectSpecToSelf _returnvalue _returnvalue_2))))

(fn AddCapacityDOT
  (params (MaxCapacityToAdd :type Float%20%28single-precision%29))
  (bind _submarinepawn (Variables|Default|GetSubmarinePawn))
  (bind _returnvalue (Ability|GetAbilitySystemComponent _submarinepawn))
  (Utilities|IsValid _returnvalue
    (:Is%20Valid
      (bind _returnvalue_2 (Ability|GameplayEffect|AssignTagSetbyCallerMagnitude (GameplayEffects|MakeOutgoingSpec _returnvalue "/Game/Batyscaphe/GAS/GameplayEffects/DOTs/GE_AddMaxCapacityDOT.GE_AddMaxCapacityDOT_C" 1.0 (GameplayEffects|MakeEffectContext _returnvalue)) "(TagName=\"Gamedata.MaxCapacity\")" MaxCapacityToAdd))
      (GameplayEffects|ApplyGameplayEffectSpecToSelf _returnvalue _returnvalue_2))))

(fn AddSonarRangeDOT
  (params (SonarRangeToAdd :type Float%20%28single-precision%29))
  (bind _submarinepawn (Variables|Default|GetSubmarinePawn))
  (bind _returnvalue (Ability|GetAbilitySystemComponent _submarinepawn))
  (Utilities|IsValid _returnvalue
    (:Is%20Valid
      (bind _returnvalue_2 (Ability|GameplayEffect|AssignTagSetbyCallerMagnitude (GameplayEffects|MakeOutgoingSpec _returnvalue "/Game/Batyscaphe/GAS/GameplayEffects/DOTs/GE_AddSonarRangeDOT.GE_AddSonarRangeDOT_C" 1.0 (GameplayEffects|MakeEffectContext _returnvalue)) "(TagName=\"Gamedata.MaxSonarRange\")" SonarRangeToAdd))
      (GameplayEffects|ApplyGameplayEffectSpecToSelf _returnvalue _returnvalue_2))))

(fn AddStat
  (params (UpgradeType :type E_UpgradeType%20Enum :default "NewEnumerator0") (Val :type Float%20%28double-precision%29))
  (switch Utilities|FlowControl|Switch|SwitchonE_UpgradeType UpgradeType
    (:NewEnumerator0
      (INSTANT|AddSpeed Val false))
    (:NewEnumerator1
      (INSTANT|AddAerodynamics Val false))
    (:NewEnumerator2
      (INSTANT|AddAcceleration Val false))
    (:NewEnumerator3
      (INSTANT|AddBatteryCapacity Val false))
    (:NewEnumerator4
      (INSTANT|AddSonarRange Val false))
    (:NewEnumerator5
      (INSTANT|AddCapacity Val false))))

(fn SetStat
  (params (UpgradeType :type E_UpgradeType%20Enum :default "NewEnumerator0") (Val :type Float%20%28double-precision%29))
  (switch Utilities|FlowControl|Switch|SwitchonE_UpgradeType UpgradeType
    (:NewEnumerator0
      (INSTANT|AddSpeed Val true))
    (:NewEnumerator1
      (INSTANT|AddAerodynamics Val true))
    (:NewEnumerator2
      (INSTANT|AddAcceleration Val true))
    (:NewEnumerator3
      (INSTANT|AddBatteryCapacity Val true))
    (:NewEnumerator4
      (INSTANT|AddSonarRange Val true))
    (:NewEnumerator5
      (INSTANT|AddCapacity Val true))))

(fn InitAbilities
  (bind _submarinepawn (Variables|Default|GetSubmarinePawn))
  (bind _abilitysystem (Variables|/Game/Batyscaphe/submarine/BP_SubmarinePawn.BP_SubmarinePawn_C|GetAbilitySystem _submarinepawn))
  (for _array_element (Variables|Default|GetMonitoringAbilities)
    (Class|AbilitySystemComponent|GiveAbilityandActivateOnce _abilitysystem _array_element 0 -1))
  (for _array_element_2 (Variables|Default|GetOtherAbilities)
    (GameplayAbilities|GiveAbility _abilitysystem _array_element_2 0 -1)))

(fn AddSpeed
  (params (ValToAdd :type Float%20%28single-precision%29) (bOverrideVal :type Boolean))
  (bind _submarinepawn (Variables|Default|GetSubmarinePawn))
  (bind _returnvalue (Ability|GetAbilitySystemComponent _submarinepawn))
  (Utilities|IsValid _returnvalue
    (:Is%20Valid
      (bind _returnvalue_2 (Ability|GameplayEffect|AssignTagSetbyCallerMagnitude (GameplayEffects|MakeOutgoingSpec _returnvalue (select bOverrideVal "/Game/Batyscaphe/GAS/GameplayEffects/OverrideVal/GE_SetMaxSpeed.GE_SetMaxSpeed_C" "/Game/Batyscaphe/GAS/GameplayEffects/Instant/GE_AddMaxSpeed.GE_AddMaxSpeed_C") 1.0 (GameplayEffects|MakeEffectContext _returnvalue)) "(TagName=\"Gamedata.MaxSpeed\")" ValToAdd))
      (GameplayEffects|ApplyGameplayEffectSpecToSelf _returnvalue _returnvalue_2))))

(fn AddAcceleration
  (params (ValToAdd :type Float%20%28single-precision%29) (bOverrideVal :type Boolean))
  (bind _submarinepawn (Variables|Default|GetSubmarinePawn))
  (bind _returnvalue (Ability|GetAbilitySystemComponent _submarinepawn))
  (Utilities|IsValid _returnvalue
    (:Is%20Valid
      (bind _returnvalue_2 (Ability|GameplayEffect|AssignTagSetbyCallerMagnitude (GameplayEffects|MakeOutgoingSpec _returnvalue (select bOverrideVal "/Game/Batyscaphe/GAS/GameplayEffects/OverrideVal/GE_SetMaxAcceleration.GE_SetMaxAcceleration_C" "/Game/Batyscaphe/GAS/GameplayEffects/Instant/GE_AddMaxAcceleration.GE_AddMaxAcceleration_C") 1.0 (GameplayEffects|MakeEffectContext _returnvalue)) "(TagName=\"Gamedata.MaxAcceleration\")" ValToAdd))
      (GameplayEffects|ApplyGameplayEffectSpecToSelf _returnvalue _returnvalue_2))))

(fn AddAerodynamics
  (params (ValToAdd :type Float%20%28single-precision%29) (bOverrideVal :type Boolean))
  (bind _submarinepawn (Variables|Default|GetSubmarinePawn))
  (bind _returnvalue (Ability|GetAbilitySystemComponent _submarinepawn))
  (Utilities|IsValid _returnvalue
    (:Is%20Valid
      (bind _returnvalue_2 (Ability|GameplayEffect|AssignTagSetbyCallerMagnitude (GameplayEffects|MakeOutgoingSpec _returnvalue (select bOverrideVal "/Game/Batyscaphe/GAS/GameplayEffects/OverrideVal/GE_SetAerodynamics.GE_SetAerodynamics_C" "/Game/Batyscaphe/GAS/GameplayEffects/Instant/GE_AddAerodynamics.GE_AddAerodynamics_C") 1.0 (GameplayEffects|MakeEffectContext _returnvalue)) "(TagName=\"Gamedata.Aerodynamics\")" ValToAdd))
      (GameplayEffects|ApplyGameplayEffectSpecToSelf _returnvalue _returnvalue_2))))

(fn AddMaxBatteryCapacity
  (params (ValToAdd :type Float%20%28single-precision%29) (bOverrideVal :type Boolean))
  (bind _submarinepawn (Variables|Default|GetSubmarinePawn))
  (bind _returnvalue (Ability|GetAbilitySystemComponent _submarinepawn))
  (Utilities|IsValid _returnvalue
    (:Is%20Valid
      (bind _returnvalue_2 (Ability|GameplayEffect|AssignTagSetbyCallerMagnitude (GameplayEffects|MakeOutgoingSpec _returnvalue (select bOverrideVal "/Game/Batyscaphe/GAS/GameplayEffects/OverrideVal/GE_SetMaxBatteryCapacity.GE_SetMaxBatteryCapacity_C" "/Game/Batyscaphe/GAS/GameplayEffects/Instant/GE_AddMaxBatteryCapacity.GE_AddMaxBatteryCapacity_C") 1.0 (GameplayEffects|MakeEffectContext _returnvalue)) "(TagName=\"Gamedata.BatteryCapacity\")" ValToAdd))
      (GameplayEffects|ApplyGameplayEffectSpecToSelf _returnvalue _returnvalue_2))))

(fn AddCapacity
  (params (AccelerationToAdd :type Float%20%28single-precision%29) (bOverrideVal :type Boolean))
  (bind _submarinepawn (Variables|Default|GetSubmarinePawn))
  (bind _returnvalue (Ability|GetAbilitySystemComponent _submarinepawn))
  (Utilities|IsValid _returnvalue
    (:Is%20Valid
      (bind _returnvalue_2 (Ability|GameplayEffect|AssignTagSetbyCallerMagnitude (GameplayEffects|MakeOutgoingSpec _returnvalue (select bOverrideVal "/Game/Batyscaphe/GAS/GameplayEffects/OverrideVal/GE_SetMaxCapacity.GE_SetMaxCapacity_C" "/Game/Batyscaphe/GAS/GameplayEffects/Instant/GE_AddMaxCapacity.GE_AddMaxCapacity_C") 1.0 (GameplayEffects|MakeEffectContext _returnvalue)) "(TagName=\"Gamedata.MaxCapacity\")" AccelerationToAdd))
      (GameplayEffects|ApplyGameplayEffectSpecToSelf _returnvalue _returnvalue_2))))

(fn AddSonarRange
  (params (ValToAdd :type Float%20%28single-precision%29) (bOverrideVal :type Boolean))
  (bind _submarinepawn (Variables|Default|GetSubmarinePawn))
  (bind _returnvalue (Ability|GetAbilitySystemComponent _submarinepawn))
  (Utilities|IsValid _returnvalue
    (:Is%20Valid
      (bind _returnvalue_2 (Ability|GameplayEffect|AssignTagSetbyCallerMagnitude (GameplayEffects|MakeOutgoingSpec _returnvalue (select bOverrideVal "/Game/Batyscaphe/GAS/GameplayEffects/OverrideVal/GE_SetMaxSonarRange.GE_SetMaxSonarRange_C" "/Game/Batyscaphe/GAS/GameplayEffects/Instant/GE_AddMaxSonarRange.GE_AddMaxSonarRange_C") 1.0 (GameplayEffects|MakeEffectContext _returnvalue)) "(TagName=\"Gamedata.MaxSonarRange\")" ValToAdd))
      (GameplayEffects|ApplyGameplayEffectSpecToSelf _returnvalue _returnvalue_2))))

(fn LoadSavedStats
  (bind _outrownames (DataTable|GetDataTableRowNames "/Game/Batyscaphe/UI/UpgradeSystem/Data/DT_Upgrades.DT_Upgrades"))
  (for _array_element _outrownames
    (bind _returnvalue (Utilities|GetDataTableRow "/Game/Batyscaphe/UI/UpgradeSystem/Data/DT_Upgrades.DT_Upgrades" _array_element)
      (:then
        (CallFunction|SetStat (.UpgradeType (Utilities|Struct|BreakS_UpgradeRow _returnvalue)) (Math|Conversions|ToFloat(Integer) (Utilities|Array|Get(acopy) (.Value (Utilities|Struct|BreakS_UpgradeRow _returnvalue)) (.Value (Utilities|Map|Find (Variables|/Game/Batyscaphe/submarine/BP_SubmarineGameinstance.BP_SubmarineGameinstance_C|GetUpgradesAndLevels (CallFunction|GetSubmarineGameInstance)) (.UpgradeType (Utilities|Struct|BreakS_UpgradeRow _returnvalue)))))))))))

(fn AddBatteryCapacity
  (params (ValToAdd :type Float%20%28single-precision%29) (bOverrideVal :type Boolean))
  (bind _submarinepawn (Variables|Default|GetSubmarinePawn))
  (bind _returnvalue (Ability|GetAbilitySystemComponent _submarinepawn))
  (Utilities|IsValid _returnvalue
    (:Is%20Valid
      (bind _returnvalue_2 (Ability|GameplayEffect|AssignTagSetbyCallerMagnitude (GameplayEffects|MakeOutgoingSpec _returnvalue (select bOverrideVal "/Game/Batyscaphe/GAS/GameplayEffects/OverrideVal/GE_SetBatteryCapacity.GE_SetBatteryCapacity_C" "/Game/Batyscaphe/GAS/GameplayEffects/Instant/GE_AddBatteryCapacity.GE_AddBatteryCapacity_C") 1.0 (GameplayEffects|MakeEffectContext _returnvalue)) "(TagName=\"Gamedata.BatteryCapacity\")" ValToAdd))
      (GameplayEffects|ApplyGameplayEffectSpecToSelf _returnvalue _returnvalue_2))))

(fn AddBatteryCapacityDOT
  (params (BatteryCapacityToAdd :type Float%20%28single-precision%29))
  (bind _submarinepawn (Variables|Default|GetSubmarinePawn))
  (bind _returnvalue (Ability|GetAbilitySystemComponent _submarinepawn))
  (Utilities|IsValid _returnvalue
    (:Is%20Valid
      (bind _returnvalue_2 (Ability|GameplayEffect|AssignTagSetbyCallerMagnitude (GameplayEffects|MakeOutgoingSpec _returnvalue "/Game/Batyscaphe/GAS/GameplayEffects/DOTs/GE_AddBatteryCapacityDOT.GE_AddBatteryCapacityDOT_C" 1.0 (GameplayEffects|MakeEffectContext _returnvalue)) "(TagName=\"Gamedata.BatteryCapacity\")" BatteryCapacityToAdd))
      (GameplayEffects|ApplyGameplayEffectSpecToSelf _returnvalue _returnvalue_2))))