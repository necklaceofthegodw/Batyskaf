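; Battery component for the submarine pawn that tracks energy level and signals when power runs out.
; Draining, step charging and full charging update the HUD, using a gameplay attribute from the Ability System as maximum capacity.
; A looping timer is set at BeginPlay, and an energy check fires OutOfEnergy once, flagging a return to surface.
; Only a full charge restores the has-energy state after depletion.
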(event Custom|CheckEnergy
  (if (not (Variables|Default|GetHasEnergy))
    (if (not (Variables|Default|GetIsReturningToSurface))
      (Variables|Default|SetIsReturningToSurface true)
      (Default|CallOutOfEnergy))))

(event EventBeginPlay
  (Variables|Default|SetWBP_SubmarineHUD (CallFunction|GetSubmarineHUDWidget))
  (bind _asbp_submarine_pawn (Utilities|Casting|CastToBP_SubmarinePawn (Components|GetOwner)))
  (Variables|Default|SetSubmarinePawn _asbp_submarine_pawn)
  (Utilities|Time|SetTimerbyEvent (EventDispatchers|CreateEvent :!event Custom|CheckEnergy) 5.0 true))

(event EventTick
  (params (DeltaSeconds :type Float%20%28single-precision%29)))

(fn DrainBattery
  (params (val :type Float%20%28double-precision%29))
  (bind _submarinepawn (Variables|Default|GetSubmarinePawn))
  (bind _abilitysystem (Variables|/Game/Batyscaphe/submarine/BP_SubmarinePawn.BP_SubmarinePawn_C|GetAbilitySystem _submarinepawn))
  (bind _returnvalue (Class|AbilitySystemComponent|GetGameplayAttributeValue _abilitysystem "(AttributeName=\"BatteryCapacity\",Attribute=/Script/Batyskaf.SubmarineAttributeSet:BatteryCapacity,AttributeOwner=\"/Script/CoreUObject.Class'/Script/Batyskaf.SubmarineAttributeSet'\")"))
  (if (Variables|Default|GetHasEnergy)
    (bind _output_get (Variables|Default|SetBatteryLevel (Math|Float|Clamp(Float) (- (Variables|Default|GetBatteryLevel) (* val (LocalVariables|GetDecreaseMultiplierL))) 0.0 _returnvalue)))
    (Variables|Default|SetHasEnergy (> _output_get 0.0))
    (Default|UpdateBatteryVal (Variables|Default|GetWBP_SubmarineHUD) (/ (Variables|Default|GetBatteryLevel) _returnvalue))
    (return (Variables|Default|GetHasEnergy))
    (else
      (return false))))

(fn ChargeBattery
  (bind _submarinepawn (Variables|Default|GetSubmarinePawn))
  (bind _returnvalue (Ability|GetAbilitySystemComponent _submarinepawn))
  (bind _returnvalue_2 (Class|AbilitySystemComponent|GetGameplayAttributeValue _returnvalue "(AttributeName=\"BatteryCapacity\",Attribute=/Script/Batyskaf.SubmarineAttributeSet:BatteryCapacity,AttributeOwner=\"/Script/CoreUObject.Class'/Script/Batyskaf.SubmarineAttributeSet'\")"))
  (Variables|Default|SetBatteryLevel (Math|Float|Clamp(Float) (+ (Variables|Default|GetBatteryLevel) (/ _returnvalue_2 1e+01)) 0.0 _returnvalue_2))
  (Default|UpdateBatteryVal (Variables|Default|GetWBP_SubmarineHUD) (/ (Variables|Default|GetBatteryLevel) _returnvalue_2)))

(fn FullyCharge
  (Variables|Default|SetBatteryLevel (.ReturnValue (Class|AbilitySystemComponent|GetGameplayAttributeValue (Ability|GetAbilitySystemComponent (Variables|Default|GetSubmarinePawn)) "(AttributeName=\"BatteryCapacity\",Attribute=/Script/Batyskaf.SubmarineAttributeSet:BatteryCapacity,AttributeOwner=\"/Script/CoreUObject.Class'/Script/Batyskaf.SubmarineAttributeSet'\")")))
  (Variables|Default|SetHasEnergy true)
  (Variables|Default|SetIsReturningToSurface false)
  (Default|UpdateBatteryVal (Variables|Default|GetWBP_SubmarineHUD) 1.0)
  (Development|PrintString "battery fully charge"))