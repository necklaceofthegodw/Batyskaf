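; Player submarine pawn with battery, flashlight, camera zoom, propeller animation, and HUD depth and speed readouts with RPM-driven engine audio.
; Tick cone-traces ahead at an ability-attribute range, pulling interactables in by timeline and destroying them, with eels recharging the battery.
; An empty battery or ReturnToSurface respawns pipe systems, teleports the sub beside the upgrade controller and recharges it.
; Turn drag and rope inventory are disconnected; sonar-range and capacity setters are stubs.
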(event Custom|MoveObjectToPawn
  (params (ActorToMove :type Actor%20Object%20Reference))
  (Variables|Hoover|SetInitialCollectableLocation (Transformation|GetActorLocation ActorToMove))
  (Variables|Hoover|SetCollectableActor ActorToMove)
  (bind _distance (Timeline|MoveCollectable PlayFromStart)
    (:Update
      (Utilities|IsValid (Variables|Hoover|GetCollectableActor)
        (:Is%20Valid
          (Transformation|SetActorLocation (Variables|Hoover|GetCollectableActor) (Math|Vector|Lerp(Vector) (Variables|Hoover|GetInitialCollectableLocation) (Transformation|GetActorLocation) _distance) false false))))
    (:Finished
      (Utilities|Casting|CastToBP_Eel (Variables|Hoover|GetCollectableActor)
        (:then
          (CallFunction|ChargeBattery)
          (CallFunction|ShowEnergyImpact "NewEnumerator0"))
        (:CastFailed
          _))
      (Utilities|IsValid (Variables|Hoover|GetCollectableActor)
        (:Is%20Valid
          (Actor|DestroyActor (Variables|Hoover|GetCollectableActor)))
        (:Is%20Not%20Valid
          _))
      (Variables|Hoover|SetCollectableActor 0))))

(event Custom|OutOfBattery
  (bind _returnvalue (Game|GetPlayerController 0))
  (Variables|Default|SetIs%20New%20Level false)
  (Input|DisableInput _returnvalue)
  (Components|Movement|StopMovementImmediately (Variables|Default|GetFloatingPawnMovement))
  (Class|Pawn|ConsumeMovementInputVector)
  (Default|ShowStartOverScreen (Variables|Default|GetWBP_SubmarineHUD) true (Variables|Default|GetIs%20New%20Level))
  (Utilities|FlowControl|Delay 1.0)
  (bind _returnvalue_2 (Actor|GetActorOfClass "/Game/Batyscaphe/PipeSystem/BP_PipeSystemsSpawner.BP_PipeSystemsSpawner_C"))
  (if (Variables|Default|GetIs%20New%20Level)
    (Default|SetupDatatablesforLevel _returnvalue_2 (Default|GetCurrentLevelName (CallFunction|GetSubmarineGameInstance))))
  (Default|DeleteAllSystems _returnvalue_2)
  (Default|SpawnNextPipeSystems _returnvalue_2)
  (Utilities|FlowControl|Delay 1.0)
  (bind _returnvalue_3 (Actor|GetActorOfClass "/Game/Batyscaphe/UI/UpgradeSystem/BP_UpgradeController.BP_UpgradeController_C"))
  (Transformation|SetActorLocation (+ (Transformation|GetActorLocation _returnvalue_3) (* (Math|Vector|NegateVector (Transformation|GetActorForwardVector _returnvalue_3)) 3e+03)) false true)
  (Utilities|FlowControl|Delay 2.0)
  (Default|FullyCharge (Variables|Default|GetBP_BatteryComponent))
  (Default|ShowStartOverScreen (Variables|Default|GetWBP_SubmarineHUD) false (Variables|Default|GetIs%20New%20Level))
  (Input|EnableInput _returnvalue)
  (CallFunction|UpdateWaterShader))

(event Custom|SubmarineBackOnSurface
  ;[0.15 0.15 0.15 0.5] doesnt work because the construction of pipes changed
  (Default|FullyCharge (Variables|Default|GetBP_BatteryComponent)))

(event Custom|SlowDown
  (bind _floatingpawnmovement (Variables|Default|GetFloatingPawnMovement))
  (Variables|/Script/Engine.FloatingPawnMovement|SetMaxSpeed _floatingpawnmovement 3e+03)
  (Variables|/Script/Engine.FloatingPawnMovement|SetDeceleration _floatingpawnmovement 8e+03))

(event Custom|ReturnToSurface
  (params (IsNewLevel :type Boolean))
  (bind _returnvalue (Game|GetPlayerController 0))
  (Variables|Default|SetIs%20New%20Level IsNewLevel)
  (Input|DisableInput _returnvalue)
  (Components|Movement|StopMovementImmediately (Variables|Default|GetFloatingPawnMovement))
  (Class|Pawn|ConsumeMovementInputVector)
  (Default|ShowStartOverScreen (Variables|Default|GetWBP_SubmarineHUD) true (Variables|Default|GetIs%20New%20Level))
  (Utilities|FlowControl|Delay 1.0)
  (bind _returnvalue_2 (Actor|GetActorOfClass "/Game/Batyscaphe/PipeSystem/BP_PipeSystemsSpawner.BP_PipeSystemsSpawner_C"))
  (if (Variables|Default|GetIs%20New%20Level)
    (Default|SetupDatatablesforLevel _returnvalue_2 (Default|GetCurrentLevelName (CallFunction|GetSubmarineGameInstance))))
  (Default|DeleteAllSystems _returnvalue_2)
  (Default|SpawnNextPipeSystems _returnvalue_2)
  (Utilities|FlowControl|Delay 1.0)
  (bind _returnvalue_3 (Actor|GetActorOfClass "/Game/Batyscaphe/UI/UpgradeSystem/BP_UpgradeController.BP_UpgradeController_C"))
  (Transformation|SetActorLocation (+ (Transformation|GetActorLocation _returnvalue_3) (* (Math|Vector|NegateVector (Transformation|GetActorForwardVector _returnvalue_3)) 3e+03)) false true)
  (Utilities|FlowControl|Delay 2.0)
  (Default|FullyCharge (Variables|Default|GetBP_BatteryComponent))
  (Default|ShowStartOverScreen (Variables|Default|GetWBP_SubmarineHUD) false (Variables|Default|GetIs%20New%20Level))
  (Input|EnableInput _returnvalue)
  (CallFunction|UpdateWaterShader))

(event EventBeginPlay
  (Variables|Default|SetWBP_SubmarineHUD (CallFunction|GetSubmarineHUDWidget))
  (Variables|Default|SetMAX_SPEED (.ReturnValue (Class|AbilitySystemComponent|GetGameplayAttributeValue (Variables|Default|GetAbilitySystem) "(AttributeName=\"MaxSpeed\",Attribute=/Script/Batyskaf.SubmarineAttributeSet:MaxSpeed,AttributeOwner=\"/Script/CoreUObject.Class'/Script/Batyskaf.SubmarineAttributeSet'\")")))
  (Utilities|Time|SetTimerbyFunctionName 0 "RotatePropeller" 0.01 true)
  (EventDispatchers|BindEventtoOutOfEnergy (Variables|Default|GetBP_BatteryComponent) (EventDispatchers|CreateEvent :!event Custom|OutOfBattery)))

(event Collision|EventActorBeginOverlap
  (params (OtherActor :type Actor%20Object%20Reference)))

(event EventTick
  (params (DeltaSeconds :type Float%20%28single-precision%29))
  (CallFunction|UpdateDepth)
  (CallFunction|UpdateSpeedMeter DeltaSeconds)
  (Utilities|IsValid (Variables|Hoover|GetCollectableActor)
    (:Is%20Not%20Valid
      (bind _outhits (Class|CollisionLibrary|ConeTraceMulti (Transformation|GetActorLocation) (Math|Rotator|MakeRotfromX (Transformation|GetActorForwardVector)) (.ReturnValue (Class|AbilitySystemComponent|GetGameplayAttributeValue (Variables|Default|GetAbilitySystem) "(AttributeName=\"MaxSonarRange\",Attribute=/Script/Batyskaf.SubmarineAttributeSet:MaxSonarRange,AttributeOwner=\"/Script/CoreUObject.Class'/Script/Batyskaf.SubmarineAttributeSet'\")")) 45.0 "TraceTypeQuery1" false (Utilities|Array|MakeArray self) "None" true))
      (for _array_element _outhits
        (bind _asbpi_interactable (Utilities|Casting|CastToBPI_Interactable (.HitActor (Collision|BreakHitResult _array_element))))
        (Default|StartInteract _asbpi_interactable)
        (CallFunction|MoveObjecttoPawn (.HitActor (Collision|BreakHitResult _array_element)))))))

(fn ConstructionScript)

(fn MoveCamera
  (params (val :type Float%20%28double-precision%29))
  (bind _output_get (Variables|Default|SetScrollVal (+ (Variables|Default|GetScrollVal) (* val 0.02))))
  (Variables|/Script/Engine.SpringArmComponent|SetTargetArmLength (Variables|Default|GetSpringArm) (Math|Float|Lerp (LocalVariables|GetcameraMin) (LocalVariables|GetcameraMax) _output_get)))

(fn ToggleFlashlight
  (bind _output_get (Variables|Default|SetbFlashlightOn (not (Variables|Default|GetbFlashlightOn))))
  (Rendering|SetVisibility (Variables|Default|GetSpotLight) _output_get false))

(fn SetMaxSpeed
  (params (MaxSpeedToSet :type Float%20%28single-precision%29))
  (Variables|/Script/Engine.FloatingPawnMovement|SetMaxSpeed (Variables|Default|GetFloatingPawnMovement) MaxSpeedToSet))

(fn SetAcceleration
  (params (AccelerationToSet :type Float%20%28single-precision%29))
  (Variables|/Script/Engine.FloatingPawnMovement|SetAcceleration (Variables|Default|GetFloatingPawnMovement) AccelerationToSet))

(fn DrainBattery
  (params (val :type Float%20%28double-precision%29))
  (if (< (Variables|Default|GetSubmarineDepth) 0.0)
    (bind _hasenergy (Default|DrainBattery (Variables|Default|GetBP_BatteryComponent) val))
    (return _hasenergy)
    (else
      (return true))))

(fn UpdateDepth
  (bind _wbp_submarinehud (Variables|Default|GetWBP_SubmarineHUD))
  (bind _output_get (Variables|Default|SetSubmarineDepth (CallFunction|ConvertLocationZtoDepth (.Z (Math|Vector|BreakVector (Transformation|GetActorLocation))))))
  (Utilities|IsValid _wbp_submarinehud
    (:Is%20Valid
      (Default|UpdateDepth _wbp_submarinehud (Math|Float|Clamp(Float) (/ _output_get (Variables|/Game/Batyscaphe/submarine/BP_SubmarineGameinstance.BP_SubmarineGameinstance_C|GetMaxDepth (CallFunction|GetSubmarineGameInstance)))) (Variables|Default|GetSubmarineDepth)))))

(fn UpdateWaterShader
  (bind _returnvalue (Actor|GetActorOfClass "/Script/Engine.PostProcessVolume"))
  (bind _output_get (LocalVariables|SetPostProcessVolumeL _returnvalue))
  (if (> (CallFunction|ConvertLocationZtoDepth (.Z (Math|Vector|BreakVector (Transformation|GetActorLocation)))) 0.0)
    (if (Utilities|Array|ContainsItem (Utilities|Struct|BreakWeightedBlendables (Utilities|Struct|BreakPostProcessSettings (Variables|/Script/Engine.PostProcessVolume|GetSettings _returnvalue))) (Variables|Default|GetAddedWeightedBlendable))
      (Utilities|Array|RemoveItem (Utilities|Struct|BreakWeightedBlendables (Utilities|Struct|BreakPostProcessSettings (Variables|/Script/Engine.PostProcessVolume|GetSettings _returnvalue))) (Variables|Default|GetAddedWeightedBlendable)))
    (elif (not (Utilities|Array|ContainsItem (Utilities|Struct|BreakWeightedBlendables (Utilities|Struct|BreakPostProcessSettings (Variables|/Script/Engine.PostProcessVolume|GetSettings _output_get))) (Variables|Default|GetAddedWeightedBlendable)))
      (Utilities|Array|Add (Utilities|Struct|BreakWeightedBlendables (Utilities|Struct|BreakPostProcessSettings (Variables|/Script/Engine.PostProcessVolume|GetSettings _output_get))) (Variables|Default|GetAddedWeightedBlendable))
      (Audio|PlaySoundatLocation "/Game/Batyscaphe/Sounds/10_splash_14.10_splash_14" (Transformation|GetActorLocation) "0, 0, 0" 1.0 1.0 0.0 0 0 0 0))))

(fn UpdateSpeedMeter
  (params (DeltaTime :type Float%20%28double-precision%29))
  (bind _floatingpawnmovement (Variables|Default|GetFloatingPawnMovement))
  (bind _abilitysystem (Variables|Default|GetAbilitySystem))
  (bind _wbp_submarinehud (Variables|Default|GetWBP_SubmarineHUD))
  (bind _returnvalue (Class|AbilitySystemComponent|GetGameplayAttributeValue _abilitysystem "(AttributeName=\"MaxSpeed\",Attribute=/Script/Batyskaf.SubmarineAttributeSet:MaxSpeed,AttributeOwner=\"/Script/CoreUObject.Class'/Script/Batyskaf.SubmarineAttributeSet'\")"))
  (bind _velocity (Variables|/Script/Engine.MovementComponent|GetVelocity _floatingpawnmovement))
  (bind _returnvalue_2 (Math|Vector|VectorLength _velocity))
  (bind _returnvalue_3 (/ _returnvalue_2 _returnvalue))
  (bind _returnvalue_4 (Math|Float|Clamp(Float) _returnvalue_3))
  (Utilities|IsValid _wbp_submarinehud
    (:Is%20Valid
      (Default|UpdateSpeedMeter _wbp_submarinehud _returnvalue_2)
      (Variables|Default|SetSmoothRPM _returnvalue_4)
      (Audio|Parameter|SetFloatParameter (Variables|Default|GetThrottleAudioComp) "RPM" (Math|Interpolation|FInterpTo (Variables|Default|GetSmoothRPM) _returnvalue_4 DeltaTime 2.5) :!class /Script/AudioExtensions.AudioParameterControllerInterface))))

(fn ChargeBattery
  (Default|ChargeBattery (Variables|Default|GetBP_BatteryComponent)))

(fn SetDeceleration
  (params (DecelerationToSet :type Float%20%28single-precision%29))
  (Variables|/Script/Engine.FloatingPawnMovement|SetDeceleration (Variables|Default|GetFloatingPawnMovement) DecelerationToSet))

(fn UpdateIsAccelerating
  (bind _floatingpawnmovement (Variables|Default|GetFloatingPawnMovement))
  (bind _velocity (Variables|/Script/Engine.MovementComponent|GetVelocity _floatingpawnmovement))
  (bind _returnvalue (Math|Vector|VectorLength _velocity))
  (Variables|Default|SetIsAccelerating (> _returnvalue (Variables|Default|GetCurrentSpeed)))
  (Variables|Default|SetCurrentSpeed _returnvalue))

(fn RotatePropeller
  (CallFunction|UpdateIsAccelerating)
  (Transformation|AddLocalRotation (Variables|Default|GetSM_Propeller) (* (Math|Rotator|SelectRotator "0.000000,0.000000,7.000000" "0.000000,0.000000,2.000000" (Variables|Default|GetIsAccelerating)) (Math|Float|MapRangeClamped (Math|Vector|VectorLength (Variables|/Script/Engine.MovementComponent|GetVelocity (Variables|Default|GetFloatingPawnMovement))) 0.0 1e+04 1.0 3.0)) false false))

(fn SetSonarRange
  (params (RangeToSet :type Float%20%28double-precision%29)))

(fn SetCapacity
  (params (CapacityToSet :type Float%20%28double-precision%29)))

(fn ShowEnergyImpact
  (params (Color :type E_EnergyColor%20Enum :default "NewEnumerator0"))
  (bind _p_energyblast_impact (Variables|Default|GetP_EnergyBlast_Impact))
  (Effects|Components|ParticleSystem|SetColorParameter _p_energyblast_impact "BlastColor" (.Value (Utilities|Map|Find (LocalVariables|GetEnumToColorL) Color)))
  (Components|Activation|Activate _p_energyblast_impact true))

(fn SetRocket
  (params (BP_RocketToSet :type BP%20Rocket%20Object%20Reference))
  (Variables|Default|SetCurrentRocket BP_RocketToSet))

(fn UpdateTurnDrag
  (bind _returnvalue (Pawn|GetControlRotation :!class /Script/Engine.Pawn))
  (bind _floatingpawnmovement (Variables|Default|GetFloatingPawnMovement))
  (bind _velocity (Variables|/Script/Engine.MovementComponent|GetVelocity _floatingpawnmovement))
  (LocalVariables|SetVelocityL _velocity)
  (LocalVariables|SetSpeedL (Math|Vector|VectorLength _velocity))
  (if (> (LocalVariables|GetSpeedL) 1e+01)
    (LocalVariables|SetDotL (Math|Float|Clamp(Float) (Math|Vector|DotProduct (Math|Vector|Normalize (LocalVariables|GetVelocityL)) (Math|Vector|GetForwardVector (Math|Rotator|MakeRotator 0.0 (.pitch _returnvalue) (.yaw _returnvalue))))))
    (LocalVariables|SetTurnSharpnessL (- (Math|Float|MakeLiteralFloat 1.0) (LocalVariables|GetDotL)))
    (LocalVariables|SetSpeedMultiplierL (- (Math|Float|MakeLiteralFloat 1.0) (* (LocalVariables|GetTurnSharpnessL) (LocalVariables|GetShaprTurnSpeedLossL))))
    (Default|SetStat (Variables|Default|GetBP_AttributeManager) "NewEnumerator0" (* (Variables|Default|GetMAX_SPEED) (LocalVariables|GetSpeedMultiplierL)))
    (else
      (Default|SetStat (Variables|Default|GetBP_AttributeManager) "NewEnumerator0" (Variables|Default|GetMAX_SPEED)))))