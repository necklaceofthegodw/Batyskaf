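; Blueprint function library of shared helpers for the submarine game.
; Getters return the cast game instance, player pawn, player controller and HUD widget, while depth conversion maps world Z using game instance limits.
; Disc and collectable lookups scan DataTable rows in order, keeping the last whose MinDepth exceeds the spawn depth and stopping at the first that fails.
; Other helpers find an upgrade row by type and pick a random point within a sphere.
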(fn GetRandomLocationinSphere
  (params (Center :type Vector) (Radius :type Float%20%28double-precision%29))
  (return (+ Center (* (Math|Random|RandomUnitVector) (* Radius (Math|Random|RandomFloat))))))

(fn GetSubmarineGameInstance
  (bind _asbp_submarine_gameinstance (Utilities|Casting|CastToBP_SubmarineGameinstance (Game|GetGameInstance (LocalVariables|Get__WorldContext))))
  (return _asbp_submarine_gameinstance))

(fn GetSubmarinePawn
  (bind _asbp_submarine_pawn (Utilities|Casting|CastToBP_SubmarinePawn (Game|Player|GetPlayerPawn (LocalVariables|Get__WorldContext))))
  (return _asbp_submarine_pawn))

(fn GetSubmarinePlayerController
  (bind _asbp_submarine_player_controller (Utilities|Casting|CastToBP_SubmarinePlayerController (Game|GetPlayerController (LocalVariables|Get__WorldContext))))
  (return _asbp_submarine_player_controller))

(fn GetSubmarineHUDWidget
  (bind _asbp_submarine_hud (Utilities|Casting|CastToBP_SubmarineHUD (HUD|GetHUD (Game|GetPlayerController (LocalVariables|Get__WorldContext)))))
  (return (Variables|/Game/Batyscaphe/submarine/BP_SubmarineHUD.BP_SubmarineHUD_C|GetWBP_HUD _asbp_submarine_hud)))

(fn ConvertLocationZtoDepth
  (params (LocationZ :type Float%20%28double-precision%29))
  (bind ___worldcontext (LocalVariables|Get__WorldContext))
  (bind _outsubmarinegameinstance (CallFunction|GetSubmarineGameInstance ___worldcontext))
  (return (Math|Float|MapRangeUnclamped LocationZ (LocalVariables|GetInitialZL) (Variables|/Game/Batyscaphe/submarine/BP_SubmarineGameinstance.BP_SubmarineGameinstance_C|GetMaxZ _outsubmarinegameinstance) 0.0 (Variables|/Game/Batyscaphe/submarine/BP_SubmarineGameinstance.BP_SubmarineGameinstance_C|GetMaxDepth _outsubmarinegameinstance))))

(fn GetDiscTypebyDepth
  (params (SpawnLocationDepth :type Float%20%28double-precision%29))
  (bind _outrownames (DataTable|GetDataTableRowNames "/Game/Batyscaphe/Obstacles/Disc/Data/DT_Discs.DT_Discs"))
  (bind _array_element (Utilities|Array|ForEachLoopwithBreak _outrownames :!label _label)
    (:LoopBody
      (bind _returnvalue (Utilities|GetDataTableRow "/Game/Batyscaphe/Obstacles/Disc/Data/DT_Discs.DT_Discs" _array_element)
        (:then
          (if (< SpawnLocationDepth (.MinDepth (Utilities|Struct|BreakS_Disc _returnvalue)))
            (LocalVariables|SetDiscInfoL _returnvalue)
            (else
              (goto _label Break))))))
    (:Completed
      (return (LocalVariables|GetDiscInfoL)))))

(fn GetCollectableTypebyDepth
  (params (SpawnLocationDepth :type Float%20%28double-precision%29))
  (bind _outrownames (DataTable|GetDataTableRowNames "/Game/Batyscaphe/Collectables/Data/DT_Collectables.DT_Collectables"))
  (bind _array_element (Utilities|Array|ForEachLoopwithBreak _outrownames :!label _label)
    (:LoopBody
      (bind _returnvalue (Utilities|GetDataTableRow "/Game/Batyscaphe/Collectables/Data/DT_Collectables.DT_Collectables" _array_element)
        (:then
          (if (< SpawnLocationDepth (.MinDepth (Utilities|Struct|BreakS_Collectable _returnvalue)))
            (LocalVariables|SetFoundItemType (.Type (Utilities|Struct|BreakS_Collectable _returnvalue)))
            (else
              (goto _label Break))))))
    (:Completed
      (return (LocalVariables|GetFoundItemType)))))

(fn GetUpgradeRowfromUpgradeType
  (params (UpgradeTypeToCheck :type E_UpgradeType%20Enum :default "NewEnumerator0"))
  (bind _outrownames (DataTable|GetDataTableRowNames "/Game/Batyscaphe/UI/UpgradeSystem/Data/DT_Upgrades.DT_Upgrades"))
  (for _array_element _outrownames
    (bind _returnvalue (Utilities|GetDataTableRow "/Game/Batyscaphe/UI/UpgradeSystem/Data/DT_Upgrades.DT_Upgrades" _array_element)
      (:then
        (if (Utilities|Enum|Equal(Enum) (.UpgradeType (Utilities|Struct|BreakS_UpgradeRow _returnvalue)) UpgradeTypeToCheck)
          (return _returnvalue))))))