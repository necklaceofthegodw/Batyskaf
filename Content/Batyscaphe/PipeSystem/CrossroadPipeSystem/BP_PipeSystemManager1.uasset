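; Crossroad pipe section manager that builds a branching tunnel and reports the submarine's left or right choice to its pawn.
; On BeginPlay it chains BP_Pipe actors socket to socket from data table rows and enables the end piece's collision sphere.
; Left and right triggers each fire once, and destruction removes the pipes.
; Functions for spawning discs, monsters, meteors, coral and eels exist but are not called from the event graph.
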(event OnComponentBeginOverlap(TriggerLeft)
  (params (OverlappedComponent :type Primitive%20Component%20Object%20Reference) (OtherActor :type Actor%20Object%20Reference) (OtherComp :type Primitive%20Component%20Object%20Reference) (OtherBodyIndex :type Integer) (bFromSweep :type Boolean) (SweepResult :type Hit%20Result%20Structure%20%28by%20ref%29))
  (bind _asbp_submarine_pawn (Utilities|Casting|CastToBP_SubmarinePawn OtherActor))
  (Utilities|FlowControl|DoOnce false
    (:Completed
      (Default|CallOnChoiceMade _asbp_submarine_pawn true))))

(event OnComponentBeginOverlap(TriggerRight)
  (params (OverlappedComponent :type Primitive%20Component%20Object%20Reference) (OtherActor :type Actor%20Object%20Reference) (OtherComp :type Primitive%20Component%20Object%20Reference) (OtherBodyIndex :type Integer) (bFromSweep :type Boolean) (SweepResult :type Hit%20Result%20Structure%20%28by%20ref%29))
  (bind _asbp_submarine_pawn (Utilities|Casting|CastToBP_SubmarinePawn OtherActor))
  (Utilities|FlowControl|DoOnce false
    (:Completed
      (Default|CallOnChoiceMade _asbp_submarine_pawn false))))

(event EventBeginPlay
  (Rendering|Material|SetMaterial (Variables|Default|GetSM_StartCrossroad) 0 (Variables|Default|GetPipeMaterial))
  (CallFunction|SpawnPipes (Variables|Default|GetPipeTable))
  (Transformation|SetActorScale3D "2.300000,2.300000,2.300000"))

(event Collision|EventActorBeginOverlap
  (params (OtherActor :type Actor%20Object%20Reference)))

(event EventTick
  (params (DeltaSeconds :type Float%20%28single-precision%29)))

(event EventDestroyed
  (for _array_element (Variables|Default|GetPipes)
    (Actor|DestroyActor _array_element))
  (|CallParentFunction))

(fn ConstructionScript)

(fn SpawnPipes
  (params (CrossroadDatatable :type Data%20Table%20Object%20Reference))
  (bind _pipes (Variables|Default|GetPipes))
  (Variables|Default|SetPreviousSocketTransform (Transformation|GetSocketTransform (Variables|Default|GetSM_StartCrossroad) "Socket2" "RTS_World"))
  (bind _outrownames (DataTable|GetDataTableRowNames CrossroadDatatable))
  (for _array_element _outrownames
    (bind _returnvalue (Utilities|GetDataTableRow CrossroadDatatable _array_element)
      (:then
        (bind _returnvalue_2 (Game|SpawnActorfromClass "/Game/Batyscaphe/PipeSystem/BP_Pipe.BP_Pipe_C" (Math|Transform|MakeTransform (.Location (Math|Transform|BreakTransform (Variables|Default|GetPreviousSocketTransform))) (.PipeRotation (Utilities|Struct|BreakS_PipeAttachmentInfo _returnvalue)) (.Scale (Math|Transform|BreakTransform (Variables|Default|GetPreviousSocketTransform)))) "Undefined" "MultiplyWithRoot" 0 (.Value (Utilities|Map|Find (Variables|Default|GetPipeTypeToMesh) (.PipeType (Utilities|Struct|BreakS_PipeAttachmentInfo _returnvalue)))) (Variables|Default|GetPipeMaterial) (.PipeType (Utilities|Struct|BreakS_PipeAttachmentInfo _returnvalue)) true 0))
        (CallFunction|SetActorLocationtoSocket (.PreviousPipeSocket (Utilities|Struct|BreakS_PipeAttachmentInfo _returnvalue)))
        (Utilities|Array|Add (Variables|Default|GetPipes) _returnvalue_2)
        (Variables|Default|SetPreviousSocketTransform (Transformation|GetSocketTransform (Variables|/Game/Batyscaphe/PipeSystem/BP_Pipe.BP_Pipe_C|GetSM_Pipe _returnvalue_2) (.PreviousPipeSocket (Utilities|Struct|BreakS_PipeAttachmentInfo _returnvalue)) "RTS_World"))
        (Transformation|AttachActorToActor _returnvalue_2 self (.PreviousPipeSocket (Utilities|Struct|BreakS_PipeAttachmentInfo _returnvalue)) "KeepWorld" "KeepWorld" "KeepRelative" true)
        (if (Utilities|Enum|Equal(Enum) (.PipeType (Utilities|Struct|BreakS_PipeAttachmentInfo _returnvalue)) "NewEnumerator4")
          (bind _output_get (Variables|Default|SetEndCrossroad (Utilities|Array|Get(acopy) _pipes (Utilities|Array|LastIndex _pipes))))
          (Default|EnableCollisionSphere _output_get true))))))

(fn SpawnMonstersandMeteors
  (for _array_element (Variables|Default|GetPipes)
    (for _array_element_2 (Transformation|GetAllSocketNames (Variables|/Game/Batyscaphe/PipeSystem/BP_Pipe.BP_Pipe_C|GetSM_Pipe _array_element))
      (if (Utilities|String|Contains (Utilities|String|ToString(Name) _array_element_2) "Spawn")
        (bind _returnvalue (Game|SpawnActorfromClass "/Game/Batyscaphe/Obstacles/MeteorObstacle/BP_MeteorSpawner.BP_MeteorSpawner_C" (Math|Transform|MakeTransform (Default|GetObstacleSpawnLocation _array_element)) "Undefined" "MultiplyWithRoot" 0 _array_element 0 0))
        (Utilities|Array|Add (Variables|Default|GetActorsSpawned) _returnvalue)
        (Utilities|FlowControl|Sequence
          (:then_0
            (bind _returnvalue_2 (Game|SpawnActorfromClass "/Game/Batyscaphe/AI/Beholder/BP_Monster.BP_Monster_C" (Math|Conversions|ToTransform(Vector) (- (Transformation|GetSocketLocation (Variables|/Game/Batyscaphe/PipeSystem/BP_Pipe.BP_Pipe_C|GetSM_Pipe _array_element) _array_element_2) (* (Math|Vector|GetForwardVector (Variables|/Game/Batyscaphe/PipeSystem/BP_Pipe.BP_Pipe_C|GetSM_Pipe _array_element)) -1.25e+04))) "Undefined" "MultiplyWithRoot" 0 0))
            (Utilities|Array|Add (Variables|Default|GetActorsSpawned) _returnvalue_2))
          (:then_1
            (bind _returnvalue_3 (Game|SpawnActorfromClass "/Game/Batyscaphe/Obstacles/CoralReef/BP_CoralReef.BP_CoralReef_C" (Math|Transform|MakeTransform (+ (Transformation|GetSocketLocation (Variables|/Game/Batyscaphe/PipeSystem/BP_Pipe.BP_Pipe_C|GetSM_Pipe _array_element) _array_element_2) (+ (* (Math|Vector|GetUpVector (Variables|/Game/Batyscaphe/PipeSystem/BP_Pipe.BP_Pipe_C|GetSM_Pipe _array_element)) 2.5e+03) (* (Math|Vector|GetForwardVector (Variables|/Game/Batyscaphe/PipeSystem/BP_Pipe.BP_Pipe_C|GetSM_Pipe _array_element)) -8.5e+03)))) "Undefined" "MultiplyWithRoot" 0 0))
            (Utilities|Array|Add (Variables|Default|GetActorsSpawned) _returnvalue_3)))))))

(fn GetSocketName
  (params (bFirstSocket :type Boolean))
  (return (Utilities|String|SelectName "Socket2" "Socket1" bFirstSocket)))

(fn SetActorLocationtoSocket
  (params (AttachSocketName1 :type Name))
  (bind _pipes (Variables|Default|GetPipes))
  (bind _returnvalue (Utilities|Array|LastIndex _pipes))
  (bind _returnvalue_2 (- _returnvalue 1))
  (bind _output (Utilities|Array|Get(acopy) _pipes _returnvalue_2))
  (LocalVariables|SetAttachSocketName AttachSocketName1)
  (Utilities|IsValid _output
    (:Is%20Valid
      (Transformation|SetActorLocation (Utilities|Array|Get(acopy) _pipes _returnvalue) (Transformation|GetSocketLocation (Variables|/Game/Batyscaphe/PipeSystem/BP_Pipe.BP_Pipe_C|GetSM_Pipe _output) (LocalVariables|GetAttachSocketName)) false false))))

(fn SpawnObstacles
  (bind _output_get (Variables|Default|SetShuffledPipes (SpawningObstacles|GetShuffledPipes)))
  (SpawningObstacles|SpawnDiscsandOtherThings _output_get)
  (SpawningObstacles|SpawnMonstersandMeteors)
  (SpawningObstacles|SpawnEels))

(fn SpawnDiscsandOtherThings
  (params (PipesUsed :type Array%20of%20BP%20Pipe%20Object%20References))
  (LocalVariables|SetChanceL (Math|Random|RandomFloatfromStream (Math|Random|MakeRandomStream 3554)))
  (for _array_element PipesUsed
    (if (> (LocalVariables|GetChanceL) 0.35)
      (bind _returnvalue (Game|SpawnActorfromClass "/Game/Batyscaphe/Obstacles/ChoiceObstacle/BP_ChoiceDisc.BP_ChoiceDisc_C" (Math|Transform|MakeTransform (Default|GetObstacleSpawnLocation _array_element) (Math|Rotator|MakeRotator 0.0 (+ (.Pitch (Math|Rotator|BreakRotator (Math|Rotator|MakeRotfromXZ (Transformation|GetActorForwardVector _array_element) (Math|Vector|GetUpVector "0, 0, 0")))) 9e+01) 0.0) "0.950000,0.950000,0.950000") "Undefined" "MultiplyWithRoot" (Game|Player|GetPlayerPawn 0) 0))
      (Utilities|Array|Add (Variables|Default|GetActorsSpawned) _returnvalue)
      (else
        (bind _returnvalue_2 (Game|SpawnActorfromClass "/Game/Batyscaphe/Obstacles/Disc/BP_Disc.BP_Disc_C" (Math|Transform|MakeTransform (Default|GetObstacleSpawnLocation _array_element) (Math|Rotator|MakeRotator 0.0 (+ (.Pitch (Math|Rotator|BreakRotator (Math|Rotator|MakeRotfromXZ (Transformation|GetActorForwardVector _array_element) (Math|Vector|GetUpVector "0, 0, 0")))) 9e+01) 0.0)) "Undefined" "MultiplyWithRoot" (Game|Player|GetPlayerPawn 0) (CallFunction|GetDiscTypebyDepth (CallFunction|ConvertLocationZtoDepth (.Z (Math|Vector|BreakVector (Default|GetObstacleSpawnLocation _array_element))))) 0))
        (Utilities|Array|Add (Variables|Default|GetActorsSpawned) _returnvalue_2)))))

(fn GetShuffledPipes
  (for _array_element (Variables|Default|GetPipes)
    (if (not (or (Utilities|Enum|Equal(Enum) (Variables|/Game/Batyscaphe/PipeSystem/BP_Pipe.BP_Pipe_C|GetPipeType _array_element) "NewEnumerator3") (Utilities|Enum|Equal(Enum) (Variables|/Game/Batyscaphe/PipeSystem/BP_Pipe.BP_Pipe_C|GetPipeType _array_element) "NewEnumerator4")))
      (Utilities|Array|Add (LocalVariables|GetPipesL) _array_element)))
  (Utilities|Array|Shuffle (LocalVariables|GetPipesL))
  (return (LocalVariables|GetPipesL)))

(fn SpawnEels
  (for _array_element (Variables|Default|GetShuffledPipes)
    (bind _returnvalue (Game|SpawnActorfromClass "/Game/Batyscaphe/AI/Eel/BP_EelSpawner.BP_EelSpawner_C" (Math|Conversions|ToTransform(Vector) (+ (Default|GetObstacleSpawnLocation _array_element) (* (Transformation|GetActorForwardVector _array_element) 6e+03))) "Undefined" "MultiplyWithRoot" (Game|Player|GetPlayerPawn 0) 0))
    (Utilities|Array|Add (Variables|Default|GetActorsSpawned) _returnvalue)))

(fn SpawnChoiceDiscs
  (params (PipesUsed :type Array%20of%20BP%20Pipe%20Object%20References))
  (for _index (range 0 3)
    (Utilities|IsValid (Utilities|Array|Get(acopy) PipesUsed _index)
      (:Is%20Valid
        (Game|SpawnActorfromClass "/Game/Batyscaphe/Obstacles/Disc/BP_Disc.BP_Disc_C" (Math|Transform|MakeTransform (Default|GetObstacleSpawnLocation (Utilities|Array|Get(acopy) PipesUsed _index)) (Math|Rotator|MakeRotfromX (Transformation|GetActorUpVector (Utilities|Array|Get(acopy) PipesUsed _index)))) "Undefined" "MultiplyWithRoot" (Game|Player|GetPlayerPawn 0) (CallFunction|GetDiscTypebyDepth (CallFunction|ConvertLocationZtoDepth (.Z (Math|Vector|BreakVector (Default|GetObstacleSpawnLocation (Utilities|Array|Get(acopy) PipesUsed _index)))))) 0)))))

(fn AddtoActorsSpawned
  (params (NewActor :type Actor%20Object%20Reference%20%28by%20ref%29))
  (Utilities|Array|Add (Variables|Default|GetActorsSpawned) NewActor))