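; Crossroad pipe manager that builds branching chains of BP_Pipe actors from a start crossroad mesh in the bathyscaphe pipe system.
; SpawnPipes reads left and right data tables, spawning a pipe per row with its type mesh and rotation, attached by socket.
; AddPipe, AttachPipe and the Switch functions build a chain piece by piece, changing the last pipe's mesh, socket position and rotation.
; The event graph is empty, so these functions run only when called.
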(event EventBeginPlay
  (|CallParentFunction) ; This node is disabled and will not be called.\nDrag off pins to build functionality.
)

(event Collision|EventActorBeginOverlap
  (params (OtherActor :type Actor%20Object%20Reference))
  (|CallParentFunction OtherActor) ; This node is disabled and will not be called.\nDrag off pins to build functionality.
)

(event EventTick
  (params (DeltaSeconds :type Float%20%28single-precision%29))
  (|CallParentFunction DeltaSeconds) ; This node is disabled and will not be called.\nDrag off pins to build functionality.
)

(fn ConstructionScript
  (|CallParentFunction))

(fn SpawnPipes
  (CallFunction|SpawnPipesfromTable (Variables|Default|GetLeftTable) false)
  (CallFunction|SpawnPipesfromTable (Variables|Default|GetRightTable) true))

(fn SpawnPipesfromTable
  (params (DataTable :type Data%20Table%20Object%20Reference) (IsRight :type Boolean))
  (LocalVariables|SetPreviousSocketTransform (Transformation|GetActorTransform))
  (bind _outrownames (DataTable|GetDataTableRowNames DataTable))
  (for _array_element _outrownames
    (bind _returnvalue (Utilities|GetDataTableRow DataTable _array_element)
      (:then
        (bind _returnvalue_2 (Game|SpawnActorfromClass "/Game/Batyscaphe/PipeSystem/BP_Pipe.BP_Pipe_C" (Math|Transform|MakeTransform (.Location (Math|Transform|BreakTransform (LocalVariables|GetPreviousSocketTransform))) (.PipeRotation (Utilities|Struct|BreakS_PipeAttachmentInfo _returnvalue)) (.Scale (Math|Transform|BreakTransform (LocalVariables|GetPreviousSocketTransform)))) "Undefined" "MultiplyWithRoot" 0 (.Value (Utilities|Map|Find (Variables|Default|GetPipeTypeToMesh) (.PipeType (Utilities|Struct|BreakS_PipeAttachmentInfo _returnvalue)))) 0))
        (Utilities|Array|Add (Variables|Default|GetPipes) _returnvalue_2)
        (Utilities|IsValid (LocalVariables|GetPreviousPipe)
          (:Is%20Valid
            (LocalVariables|SetPreviousSocketTransform (Transformation|GetSocketTransform (Variables|/Game/Batyscaphe/PipeSystem/BP_Pipe.BP_Pipe_C|GetSM_Pipe (LocalVariables|GetPreviousPipe)) (.PreviousPipeSocket (Utilities|Struct|BreakS_PipeAttachmentInfo _returnvalue)) "RTS_World"))
            (Transformation|AttachActorToActor _returnvalue_2 (LocalVariables|GetPreviousPipe) (.PreviousPipeSocket (Utilities|Struct|BreakS_PipeAttachmentInfo _returnvalue)) "SnapToTarget" "KeepWorld" "KeepRelative" true)
            (LocalVariables|SetPreviousPipe _returnvalue_2))
          (:Is%20Not%20Valid
            (bind _output_get (LocalVariables|SetPreviousPipe _returnvalue_2))
            (LocalVariables|SetPreviousSocketTransform (Transformation|GetSocketTransform (Variables|/Game/Batyscaphe/PipeSystem/BP_Pipe.BP_Pipe_C|GetSM_Pipe _output_get) (.PreviousPipeSocket (Utilities|Struct|BreakS_PipeAttachmentInfo _returnvalue)) "RTS_World"))
            ;[0.15 0.15 0.15 0.5] Socket1 - right
            (Transformation|AttachComponentToComponent _output_get (Variables|Default|GetSM_StartCrossroad) (Utilities|String|SelectName "Socket1" "Socket2" IsRight) "SnapToTarget" "KeepWorld" "KeepRelative" true)))))))

(fn AddPipe
  (if (> (Utilities|Array|Length (Variables|Default|GetPipes)) 0)
    (Pipetool|AttachPipe)
    (else
      (Variables|Default|SetPreviousSocketTransform (Transformation|GetSocketTransform (Variables|Default|GetSM_StartCrossroad) (PipeTool|GetSocketName (Variables|Default|GetIsRight)) "RTS_World"))))
  (bind _returnvalue (Game|SpawnActorfromClass "/Game/Batyscaphe/PipeSystem/BP_Pipe.BP_Pipe_C" (Math|Transform|MakeTransform (.Location (Math|Transform|BreakTransform (Variables|Default|GetPreviousSocketTransform))) "0, 0, 0" (.Scale (Math|Transform|BreakTransform (Variables|Default|GetPreviousSocketTransform)))) "Undefined" "MultiplyWithRoot" 0 (.Value (Utilities|Map|Find (Variables|Default|GetPipeTypeToMesh) (Variables|Default|GetCurrentPipeType))) 0))
  (Utilities|Array|Add (Variables|Default|GetPipes) _returnvalue))

(fn AttachPipe
  (bind _pipes (Variables|Default|GetPipes))
  (bind _isright (Variables|Default|GetIsRight))
  (bind _returnvalue (Utilities|Array|LastIndex _pipes))
  (bind _outsocketname (PipeTool|GetSocketName _isright))
  (bind _output (Utilities|Array|Get(acopy) _pipes _returnvalue))
  (Variables|Default|SetCurrentPipeRotation "0, 0, 0")
  (Variables|Default|SetPreviousSocketTransform (Transformation|GetSocketTransform (Variables|/Game/Batyscaphe/PipeSystem/BP_Pipe.BP_Pipe_C|GetSM_Pipe _output) _outsocketname "RTS_World"))
  (Utilities|IsValid (Variables|Default|GetPreviousPipee)
    (:Is%20Valid
      (Transformation|AttachActorToActor _output self _outsocketname "KeepWorld" "KeepWorld" "KeepRelative" true)
      (Variables|Default|SetPreviousPipee _output))
    (:Is%20Not%20Valid
      (bind _output_get (Variables|Default|SetPreviousPipee _output))
      (Transformation|AttachComponentToComponent _output_get (Variables|Default|GetSM_StartCrossroad) _outsocketname "SnapToTarget" "KeepWorld" "KeepRelative" true))))

(fn SwitchPipeMesh
  (params (PipeType :type E_PipeType%20Enum :default "NewEnumerator0"))
  (bind _pipes (Variables|Default|GetPipes))
  (bind _pipetypetomesh (Variables|Default|GetPipeTypeToMesh))
  (bind _returnvalue (Utilities|Array|LastIndex _pipes))
  (bind _value (Utilities|Map|Find _pipetypetomesh PipeType))
  (bind _output (Utilities|Array|Get(acopy) _pipes _returnvalue))
  (Variables|Default|SetCurrentPipeType PipeType)
  (if (> (Utilities|Array|Length _pipes) 0)
    (Components|StaticMesh|SetStaticMesh (Variables|/Game/Batyscaphe/PipeSystem/BP_Pipe.BP_Pipe_C|GetSM_Pipe _output) _value)
    (Variables|/Game/Batyscaphe/PipeSystem/BP_Pipe.BP_Pipe_C|SetPipeMesh _output _value)))

(fn SwitchAttachSocket
  (params (IsRight :type Boolean))
  (bind _pipes (Variables|Default|GetPipes))
  (bind _returnvalue (Utilities|Array|LastIndex _pipes))
  (bind _output (Utilities|Array|Get(acopy) _pipes _returnvalue))
  (bind _returnvalue_2 (- _returnvalue 1))
  (bind _output_2 (Utilities|Array|Get(acopy) _pipes _returnvalue_2))
  (bind _output_get (Variables|Default|SetIsRight IsRight))
  (LocalVariables|SetAttachSocketName (PipeTool|GetSocketName _output_get))
  (Utilities|IsValid _output_2
    (:Is%20Valid
      (Transformation|SetActorLocation _output (Transformation|GetSocketLocation (Variables|/Game/Batyscaphe/PipeSystem/BP_Pipe.BP_Pipe_C|GetSM_Pipe _output_2) (LocalVariables|GetAttachSocketName)) false false))
    (:Is%20Not%20Valid
      (Transformation|SetActorLocation _output (Transformation|GetSocketLocation (Variables|Default|GetSM_StartCrossroad) (LocalVariables|GetAttachSocketName)) false false))))

(fn SwitchMeshRotation
  (params (RotationToAdd :type Rotator))
  (bind _pipes (Variables|Default|GetPipes))
  (bind _output_get (Variables|Default|SetCurrentPipeRotation (Math|Rotator|CombineRotators (Variables|Default|GetCurrentPipeRotation) RotationToAdd)))
  (Transformation|SetActorRotation (Utilities|Array|Get(acopy) _pipes (Utilities|Array|LastIndex _pipes)) _output_get))

(fn GetSocketName
  (params (bFirstSocket :type Boolean))
  (return (Utilities|String|SelectName "Socket2" "Socket1" bFirstSocket)))