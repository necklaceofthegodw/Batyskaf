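; Spline-driven pipe actor for the submarine, able to glide it back to the spline start with a timeline.
; The construction script loads spline data from a data asset once and rebuilds length-spaced spline meshes with clamped tangents.
; SpawnObjectsAlongSpline, unwired in this graph, places eel spawners and randomly picks gas clouds, discs, choice discs or collectible clusters per segment.
; Disc and collectible types depend on depth.
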(event Custom|MoveSubmarineAlongSpline
  (params (InLocation :type Vector%20%28by%20ref%29))
  (bind _pipesplinecomp (Variables|Default|GetPipeSplineComp))
  (Variables|Default|SetStartDistance (Class|SplineComponent|GetDistanceAlongSplineatLocation _pipesplinecomp InLocation "World"))
  (bind _newtrack_0 (Timeline|MoveSubmarine PlayFromStart)
    (:Update
      (Transformation|SetActorLocation (Variables|Default|GetSubmarinePawn) (Spline|GetLocationatDistanceAlongSpline _pipesplinecomp (Math|Float|Lerp (Variables|Default|GetStartDistance) 0.0 _newtrack_0) "World") false false))
    (:Finished
      (Default|CallSubmarineReturned))))

(event EventBeginPlay
  (|CallParentFunction)
  (Variables|Default|SetSubmarinePawn (CallFunction|GetSubmarinePawn)))

(event Collision|EventActorBeginOverlap
  (params (OtherActor :type Actor%20Object%20Reference)))

(event EventTick
  (params (DeltaSeconds :type Float%20%28single-precision%29)))

(fn ConstructionScript
  (|CallParentFunction)
  (CallFunction|UpdatePipes))

(fn UpdatePipes
  (bind _splinedataasset (Variables|Default|GetSplineDataAsset))
  (CallFunction|DestroyPipes)
  (Utilities|IsValid _splinedataasset
    (:Is%20Valid
      (if (Variables|Default|GetbDataAssetLoaded)
        _
        (else
          (Class|PipeSpline|LoadSplinefromDataAsset _splinedataasset)
          (Variables|Default|SetbDataAssetLoaded true))))
    (:Is%20Not%20Valid
      _))
  (CallFunction|SpawnPipesAlongSpline))

(fn SpawnPipesAlongSpline
  (bind _pipemesh (Variables|Default|GetPipeMesh))
  (bind _returnvalue (StaticMesh|GetBoundingBox _pipemesh))
  (Utilities|Array|Clear (Variables|Default|GetSplineMeshes))
  (Utilities|Array|Clear (Variables|Default|GetPipeMeshes))
  (Variables|Default|SetPipeLength (.x (+ (Math|Vector|VectorGetAbs (.min _returnvalue)) (Math|Vector|VectorGetAbs (.max _returnvalue)))))
  (for _index (range 0 (Math|Float|Truncate (/ (Spline|GetSplineLength (Variables|Default|GetPipeSplineComp)) (Variables|Default|GetPipeLength))))
    (bind (_outspawnedmesh _outsplinemesh) (CallFunction|AddPipeMeshtoSpline _index (Variables|Default|GetPipeMesh)))
    (Utilities|Array|Add (Variables|Default|GetPipeMeshes) _outspawnedmesh)
    (Utilities|Array|Add (Variables|Default|GetSplineMeshes) _outsplinemesh)))

(fn AddPipeMeshtoSpline
  (params (PointIndex :type Integer) (MeshToAdd :type Static%20Mesh%20Object%20Reference))
  (bind _returnvalue (+ PointIndex 1))
  (bind _pipelength (Variables|Default|GetPipeLength))
  (bind _pipelength_2 (Variables|Default|GetPipeLength))
  (bind _pipesplinecomp (Variables|Default|GetPipeSplineComp))
  (bind _pipesplinecomp_2 (Variables|Default|GetPipeSplineComp))
  (bind _returnvalue_2 (* _returnvalue _pipelength))
  (bind _returnvalue_3 (* PointIndex _pipelength_2))
  (bind _returnvalue_4 (AddComponent|AddSplineMeshComponent false))
  (Collision|SetCollisionEnabled _returnvalue_4 "QueryAndPhysics")
  (SplineMesh|SetForwardAxis _returnvalue_4 "X" true)
  (Components|StaticMesh|SetStaticMesh _returnvalue_4 MeshToAdd)
  (Rendering|Material|SetMaterial _returnvalue_4 0 (Variables|Default|GetMaterialToSet))
  (SplineMesh|SetStartandEnd _returnvalue_4 (Spline|GetLocationatDistanceAlongSpline _pipesplinecomp _returnvalue_3 "Local") (Math|Vector|ClampVectorSize (Spline|GetTangentatDistanceAlongSpline _pipesplinecomp _returnvalue_3 "Local") 0.0 (Variables|Default|GetPipeLength)) (Spline|GetLocationatDistanceAlongSpline _pipesplinecomp_2 _returnvalue_2 "Local") (Math|Vector|ClampVectorSize (Spline|GetTangentatDistanceAlongSpline _pipesplinecomp_2 _returnvalue_2 "Local") 0.0 (Variables|Default|GetPipeLength)) true :!class /Script/Engine.SplineMeshComponent)
  (return _returnvalue_4 _returnvalue_4))

(fn DestroyPipes
  (for _array_element (Variables|Default|GetPipeMeshes)
    (Transformation|DetachFromComponent _array_element "KeepRelative" "KeepRelative" "KeepRelative" true)
    (Components|DestroyComponent _array_element))
  (Utilities|Array|Clear (Variables|Default|GetPipeMeshes)))

(fn SetupSplinePoints)

(fn SpawnObjectsAlongSpline
  (SpawnObstacles|SpawnEels)
  (for _array_element (Variables|Default|GetSplineMeshes)
    (bind _returnvalue (Class|SplineHelperLibrary|GetSplineMeshCenterPositions _array_element 10))
    (LocalVariables|SetCurrentSpawnTransformL (Math|Transform|MakeTransform (.Center (Utilities|Struct|BreakCircleData (Utilities|Array|Get(acopy) _returnvalue 5))) (Math|Rotator|MakeRotfromZ (.Tangent (Utilities|Struct|BreakCircleData (Utilities|Array|Get(acopy) _returnvalue 5))))))
    (LocalVariables|SetRandomValL (Math|Random|RandomFloat))
    (if (> (LocalVariables|GetRandomValL) 0.85)
      (bind _returnvalue_2 (Game|SpawnActorfromClass "/Game/Batyscaphe/Obstacles/GasCloud/BP_GasCloud.BP_GasCloud_C" (LocalVariables|GetCurrentSpawnTransformL) "Undefined" "MultiplyWithRoot" (Game|Player|GetPlayerPawn 0) 0))
      (Utilities|Array|Add (Variables|Default|GetActorsSpawned) _returnvalue_2)
      (elif (> (LocalVariables|GetRandomValL) 0.7)
        (bind _returnvalue_3 (Game|SpawnActorfromClass "/Game/Batyscaphe/Obstacles/Disc/BP_Disc.BP_Disc_C" (LocalVariables|GetCurrentSpawnTransformL) "Undefined" "MultiplyWithRoot" (Game|Player|GetPlayerPawn 0) (CallFunction|GetDiscTypebyDepth (CallFunction|ConvertLocationZtoDepth (.Z (Math|Vector|BreakVector (.Location (Math|Transform|BreakTransform (LocalVariables|GetCurrentSpawnTransformL))))))) 0))
        (Utilities|Array|Add (Variables|Default|GetActorsSpawned) _returnvalue_3)
        (elif (> (LocalVariables|GetRandomValL) 0.5)
          (SpawnObstacles|SpawnCollectiblesatLocation (.Location (Math|Transform|BreakTransform (LocalVariables|GetCurrentSpawnTransformL))) (CallFunction|GetCollectableTypebyDepth (CallFunction|ConvertLocationZtoDepth (.Z (Math|Vector|BreakVector (.Location (Math|Transform|BreakTransform (LocalVariables|GetCurrentSpawnTransformL))))))))
          (else
            (bind _returnvalue_4 (Game|SpawnActorfromClass "/Game/Batyscaphe/Obstacles/ChoiceObstacle/BP_ChoiceDisc.BP_ChoiceDisc_C" (LocalVariables|GetCurrentSpawnTransformL) "Undefined" "MultiplyWithRoot" (Game|Player|GetPlayerPawn 0) 0))
            (Utilities|Array|Add (Variables|Default|GetActorsSpawned) _returnvalue_4)))))))

(fn SpawnCollectiblesatLocation
  (params (CenterLocation :type Vector) (CollectableType :type E_Collectable%20Enum :default "NewEnumerator0"))
  (for _index (range 0 (Math|Random|RandomIntegerinRange 2 4))
    (bind _returnvalue (Game|SpawnActorfromClass "/Game/Batyscaphe/Collectables/BP_Collectable2.BP_Collectable2_C" (Math|Conversions|ToTransform(Vector) (CallFunction|GetRandomLocationinSphere CenterLocation (Math|Random|RandomFloatinRange 1e+03 8e+03))) "Undefined" "MultiplyWithRoot" (Game|Player|GetPlayerPawn 0) CollectableType 0))
    (Utilities|Array|Add (Variables|Default|GetActorsSpawned) _returnvalue)))

(fn GetNearestSplinePoint
  (params (Point :type Vector))
  (bind _pipesplinecomp (Variables|Default|GetPipeSplineComp))
  (Development|PrintString "Distances: ")
  (LocalVariables|SetCurrentNearestDistL (Math|Vector|Distance(Vector) Point (Spline|GetLocationatSplinePoint _pipesplinecomp 0 "World")))
  (bind _index (Utilities|FlowControl|ForLoopwithBreak 1 (- (Spline|GetNumberOfSplinePoints _pipesplinecomp) 1))
    (:LoopBody
      (Development|PrintString (Utilities|String|Append "    " (Utilities|String|ToString(Float) (Math|Vector|Distance(Vector) Point (Spline|GetLocationatSplinePoint _pipesplinecomp _index "World"))) "    "))
      (if (< (Math|Vector|Distance(Vector) Point (Spline|GetLocationatSplinePoint _pipesplinecomp _index "World")) (LocalVariables|GetCurrentNearestDistL))
        (LocalVariables|SetCurrentNearestDistL (Math|Vector|Distance(Vector) Point (Spline|GetLocationatSplinePoint _pipesplinecomp _index "World")))
        (LocalVariables|SetNearestPointIndexL _index)))
    (:Completed
      (Development|PrintString (Utilities|String|Append " 
 
nearest distance: " (Utilities|String|ToString(Float) (LocalVariables|GetCurrentNearestDistL))))
      (return (Spline|GetLocationatSplinePoint (Variables|Default|GetPipeSplineComp) (LocalVariables|GetNearestPointIndexL) "World")))))

(fn GetSplinePointLocations
  (params (StartingIndex :type Integer))
  (LocalVariables|SetIndexL StartingIndex)
  (while (>= (LocalVariables|GetIndexL) 0)
    (Utilities|Array|Add (LocalVariables|GetSplineLocationsL) (Spline|GetLocationatSplinePoint (Variables|Default|GetPipeSplineComp) (LocalVariables|GetIndexL) "World"))
    (Math|Integer|DecrementInt (LocalVariables|GetIndexL)))
  (return (LocalVariables|GetSplineLocationsL)))

(fn GetDiscTypebyDepth
  (params (SpawnLocationDepth :type Float%20%28double-precision%29))
  (bind _outrownames (DataTable|GetDataTableRowNames "/Game/Batyscaphe/Obstacles/Disc/Data/DT_Discs.DT_Discs"))
  (bind _array_element (Utilities|Array|ForEachLoopwithBreak _outrownames :!label _label)
    (:LoopBody
      (bind _returnvalue (Utilities|GetDataTableRow "/Game/Batyscaphe/Obstacles/Disc/Data/DT_Discs.DT_Discs" _array_element)
        (:then
          (if (< SpawnLocationDepth (.MinDepth (Utilities|Struct|BreakS_Disc _returnvalue)))
            (LocalVariables|SetDiscInfoL _returnvalue)
            (else
              (goto _label Break))))))
    (:Completed
      (return (LocalVariables|GetDiscInfoL)))))

(fn GetLastSplinePointLocation
  (bind _pipesplinecomp (Variables|Default|GetPipeSplineComp))
  (return (Spline|GetLocationatSplinePoint _pipesplinecomp (- (Spline|GetNumberOfSplinePoints _pipesplinecomp) 1) "World")))

(fn SpawnEels
  (bind _output_get (LocalVariables|SetSplineMeshesL (Variables|Default|GetSplineMeshes)))
  (Utilities|Array|Shuffle _output_get)
  (for _index (range 0 1)
    (bind _returnvalue (Class|SplineHelperLibrary|GetSplineMeshCenterPositions (Utilities|Array|Get(acopy) (LocalVariables|GetSplineMeshesL) _index) 10))
    (for _array_element _returnvalue
      (LocalVariables|SetSpawnTransformL (Math|Transform|MakeTransform (.Center (Utilities|Struct|BreakCircleData _array_element)) (Math|Rotator|MakeRotfromZ (.Tangent (Utilities|Struct|BreakCircleData _array_element))))))
    (Game|SpawnActorfromClass "/Game/Batyscaphe/AI/Eel/BP_EelSpawner.BP_EelSpawner_C" (LocalVariables|GetSpawnTransformL) "Undefined" "MultiplyWithRoot" (Game|Player|GetPlayerPawn 0) 0)))