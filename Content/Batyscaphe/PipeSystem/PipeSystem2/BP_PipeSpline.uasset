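; Spline-based pipe in the submarine game that populates its route at BeginPlay and returns the submarine along it.
; Construction rebuilds spline mesh segments sized from the pipe mesh bounds.
; Points sampled along segments randomly spawn collectible clusters and eel spawners, while segment index places discs or gas clouds, with data tables picking collectible and disc types by depth.
; A timeline moves the submarine back to spline start, then signals its return.
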(event Custom|MoveSubmarineAlongSpline
  (params (InLocation :type Vector%20%28by%20ref%29))
  (bind _spline (Variables|Default|GetSpline))
  (Variables|Default|SetStartDistance (Class|SplineComponent|GetDistanceAlongSplineatLocation _spline InLocation "World"))
  (bind _newtrack_0 (Timeline|MoveSubmarine PlayFromStart)
    (:Update
      (Transformation|SetActorLocation (Variables|Default|GetSubmarinePawn) (Spline|GetLocationatDistanceAlongSpline _spline (Math|Float|Lerp (Variables|Default|GetStartDistance) 0.0 _newtrack_0) "World") false false))
    (:Finished
      (Default|CallSubmarineReturned))))

(event EventBeginPlay
  (Variables|Default|SetSubmarinePawn (CallFunction|GetSubmarinePawn))
  (CallFunction|SpawnObjectsAlongSpline))

(event Collision|EventActorBeginOverlap
  (params (OtherActor :type Actor%20Object%20Reference)))

(event EventTick
  (params (DeltaSeconds :type Float%20%28single-precision%29)))

(fn ConstructionScript
  (CallFunction|UpdatePipes))

(fn UpdatePipes
  (CallFunction|DestroyPipes)
  (CallFunction|SpawnPipesAlongSpline))

(fn SpawnPipesAlongSpline
  (bind _pipemesh (Variables|Default|GetPipeMesh))
  (bind _returnvalue (StaticMesh|GetBoundingBox _pipemesh))
  (Utilities|Array|Clear (Variables|Default|GetSplineMeshes))
  (Variables|Default|SetPipeLength (.x (+ (Math|Vector|VectorGetAbs (.min _returnvalue)) (Math|Vector|VectorGetAbs (.max _returnvalue)))))
  (for _index (range 0 (Math|Float|Truncate (/ (Spline|GetSplineLength (Variables|Default|GetSpline)) (Variables|Default|GetPipeLength))))
    (bind (_outspawnedmesh _outsplinemesh) (CallFunction|AddPipeMeshtoSpline _index (Variables|Default|GetPipeMesh)))
    (Utilities|Array|Add (Variables|Default|GetPipeMeshes) _outspawnedmesh)
    (Utilities|Array|Add (Variables|Default|GetSplineMeshes) _outsplinemesh)))

(fn AddPipeMeshtoSpline
  (params (PointIndex :type Integer) (MeshToAdd :type Static%20Mesh%20Object%20Reference))
  (bind _returnvalue (+ PointIndex 1))
  (bind _pipelength (Variables|Default|GetPipeLength))
  (bind _spline (Variables|Default|GetSpline))
  (bind _spline_2 (Variables|Default|GetSpline))
  (bind _pipelength_2 (Variables|Default|GetPipeLength))
  (bind _returnvalue_2 (* _returnvalue _pipelength))
  (bind _returnvalue_3 (* PointIndex _pipelength_2))
  (bind _returnvalue_4 (AddComponent|AddSplineMeshComponent false))
  (Collision|SetCollisionEnabled _returnvalue_4 "QueryAndPhysics")
  (SplineMesh|SetForwardAxis _returnvalue_4 "X" true)
  (Components|StaticMesh|SetStaticMesh _returnvalue_4 MeshToAdd)
  (SplineMesh|SetStartandEnd _returnvalue_4 (Spline|GetLocationatDistanceAlongSpline _spline_2 _returnvalue_3 "Local") (Math|Vector|ClampVectorSize (Spline|GetTangentatDistanceAlongSpline _spline_2 _returnvalue_3 "Local") 0.0 (Variables|Default|GetPipeLength)) (Spline|GetLocationatDistanceAlongSpline _spline _returnvalue_2 "Local") (Math|Vector|ClampVectorSize (Spline|GetTangentatDistanceAlongSpline _spline _returnvalue_2 "Local") 0.0 (Variables|Default|GetPipeLength)) true :!class /Script/Engine.SplineMeshComponent)
  (return _returnvalue_4 _returnvalue_4))

(fn DestroyPipes
  (for _array_element (Variables|Default|GetPipeMeshes)
    (Transformation|DetachFromComponent _array_element "KeepRelative" "KeepRelative" "KeepRelative" true)
    (Components|DestroyComponent _array_element))
  (Utilities|Array|Clear (Variables|Default|GetPipeMeshes)))

(fn SetupSplinePoints)

(fn SpawnObjectsAlongSpline
  (for (_array_element _array_index) (Variables|Default|GetSplineMeshes)
    (bind _returnvalue (Class|SplineHelperLibrary|GetSplineMeshCenterPositions _array_element 10))
    (for _array_element_2 _returnvalue
      (LocalVariables|SetCurrentSpawnTransform (Math|Transform|MakeTransform (.Center (Utilities|Struct|BreakCircleData _array_element_2)) (Math|Rotator|MakeRotfromZ (.Tangent (Utilities|Struct|BreakCircleData _array_element_2)))))
      (if (> (Math|Random|RandomFloat) 0.77)
        (CallFunction|SpawnCollectiblesatLocation (.Center (Utilities|Struct|BreakCircleData _array_element_2)) (CallFunction|GetCollectableTypebyDepth (CallFunction|ConvertLocationZtoDepth (.Z (Math|Vector|BreakVector (.Center (Utilities|Struct|BreakCircleData _array_element_2)))))))
        (if (> (Math|Random|RandomFloat) 0.5)
          (Game|SpawnActorfromClass "/Game/Batyscaphe/AI/Eel/BP_EelSpawner.BP_EelSpawner_C" (LocalVariables|GetCurrentSpawnTransform) "Undefined" "MultiplyWithRoot" 0 0))))
    (if (== (Math|Integer|%(Integer) _array_index 3) 0)
      (Game|SpawnActorfromClass "/Game/Batyscaphe/Obstacles/Disc/BP_Disc.BP_Disc_C" (LocalVariables|GetCurrentSpawnTransform) "Undefined" "MultiplyWithRoot" 0 (CallFunction|GetDiscTypebyDepth (CallFunction|ConvertLocationZtoDepth (.Z (Math|Vector|BreakVector (.Location (Math|Transform|BreakTransform (LocalVariables|GetCurrentSpawnTransform))))))) 0)
      (elif (== (Math|Integer|%(Integer) _array_index 2) 0)
        (Game|SpawnActorfromClass "/Game/Batyscaphe/Obstacles/GasCloud/BP_GasCloud.BP_GasCloud_C" (LocalVariables|GetCurrentSpawnTransform) "Undefined" "MultiplyWithRoot" 0 0)))))

(fn SpawnCollectiblesatLocation
  (params (CenterLocation :type Vector) (CollectableType :type E_Collectable%20Enum :default "NewEnumerator0"))
  (for _index (range 0 (Math|Random|RandomIntegerinRange 2 4))
    (Game|SpawnActorfromClass "/Game/Batyscaphe/Collectables/BP_Collectable2.BP_Collectable2_C" (Math|Conversions|ToTransform(Vector) (CallFunction|GetRandomLocationinSphere CenterLocation (Math|Random|RandomFloatinRange 1e+03 8e+03))) "Undefined" "MultiplyWithRoot" 0 CollectableType 0)))

(fn GetCollectableTypebyDepth
  (params (SpawnLocationDepth :type Float%20%28double-precision%29))
  (bind _outrownames (DataTable|GetDataTableRowNames "/Game/Batyscaphe/Collectables/Data/DT_Collectables.DT_Collectables"))
  (bind _array_element (Utilities|Array|ForEachLoopwithBreak _outrownames :!label _label)
    (:LoopBody
      (bind _returnvalue (Utilities|GetDataTableRow "/Game/Batyscaphe/Collectables/Data/DT_Collectables.DT_Collectables" _array_element)
        (:then
          (if (< SpawnLocationDepth (.MinDepth (Utilities|Struct|BreakS_Collectable _returnvalue)))
            (LocalVariables|SetFoundItemType (.Type (Utilities|Struct|BreakS_Collectable _returnvalue)))
            (else
              (goto _label Break))))))
    (:Completed
      (return (LocalVariables|GetFoundItemType)))))

(fn GetNearestSplinePoint
  (params (Point :type Vector))
  (bind _spline (Variables|Default|GetSpline))
  (Development|PrintString "Distances: ")
  (LocalVariables|SetCurrentNearestDistL (Math|Vector|Distance(Vector) Point (Spline|GetLocationatSplinePoint _spline 0 "World")))
  (bind _index (Utilities|FlowControl|ForLoopwithBreak 1 (- (Spline|GetNumberOfSplinePoints _spline) 1))
    (:LoopBody
      (Development|PrintString (Utilities|String|Append "    " (Utilities|String|ToString(Float) (Math|Vector|Distance(Vector) Point (Spline|GetLocationatSplinePoint _spline _index "World"))) "    "))
      (if (< (Math|Vector|Distance(Vector) Point (Spline|GetLocationatSplinePoint _spline _index "World")) (LocalVariables|GetCurrentNearestDistL))
        (LocalVariables|SetCurrentNearestDistL (Math|Vector|Distance(Vector) Point (Spline|GetLocationatSplinePoint _spline _index "World")))
        (LocalVariables|SetNearestPointIndexL _index)))
    (:Completed
      (Development|PrintString (Utilities|String|Append " 
 
nearest distance: " (Utilities|String|ToString(Float) (LocalVariables|GetCurrentNearestDistL))))
      (return (Spline|GetLocationatSplinePoint (Variables|Default|GetSpline) (LocalVariables|GetNearestPointIndexL) "World")))))

(fn GetSplinePointLocations
  (params (StartingIndex :type Integer))
  (LocalVariables|SetIndexL StartingIndex)
  (while (>= (LocalVariables|GetIndexL) 0)
    (Utilities|Array|Add (LocalVariables|GetSplineLocationsL) (Spline|GetLocationatSplinePoint (Variables|Default|GetSpline) (LocalVariables|GetIndexL) "World"))
    (Math|Integer|DecrementInt (LocalVariables|GetIndexL)))
  (return (LocalVariables|GetSplineLocationsL)))

(fn GetDiscTypebyDepth
  (params (SpawnLocationDepth :type Float%20%28double-precision%29))
  (bind _outrownames (DataTable|GetDataTableRowNames "/Game/Batyscaphe/Obstacles/Disc/Data/DT_Discs.DT_Discs"))
  (bind _array_element (Utilities|Array|ForEachLoopwithBreak _outrownames :!label _label)
    (:LoopBody
      (bind _returnvalue (Utilities|GetDataTableRow "/Game/Batyscaphe/Obstacles/Disc/Data/DT_Discs.DT_Discs" _array_element)
        (:then
          (if (< SpawnLocationDepth (.MinDepth (Utilities|Struct|BreakS_Disc _returnvalue)))
            (LocalVariables|SetDiscInfo _returnvalue)
            (else
              (goto _label Break))))))
    (:Completed
      (return (LocalVariables|GetDiscInfo)))))