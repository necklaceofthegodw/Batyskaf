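; Scriptable editor tool for building pipe systems through a BP_CrossroadPipeSystemManager actor.
; A click traces under the cursor to spawn the manager, if none exists, with a translation-only gizmo that moves it.
; A draggable overlay widget adds pipes and rotates meshes in 90-degree steps, while watched settings switch pipe type and attach socket.
; Edits are delegated to the manager, and tool shutdown calls its AttachPipe.
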(event EventOnScriptSetup
  (Utilities|FlowControl|Sequence
    (:then_0
      (bind _returnvalue (Class|ScriptableInteractiveTool|AddPropertySetOfType "/Game/Batyscaphe/PipeSystem/PipeTool/BP_PipeToolPropertySet.BP_PipeToolPropertySet_C" "Settings")
        (:Success
          (bind _output_get (Variables|Default|SetPropertySet _returnvalue))
          (Class|ScriptableInteractiveTool|WatchEnumProperty _output_get "PipeType" (EventDispatchers|CreateEvent :!event PipeMeshSelected))
          (Class|ScriptableInteractiveTool|WatchBoolProperty _output_get "bSpawnMeshAtStart" (EventDispatchers|CreateEvent :!event SpawnSocketSwitched)))))
    (:then_1
      (bind _returnvalue_2 (UserInterface|CreateWidget "/Game/Batyscaphe/PipeSystem/PipeTool/WBP_PipeTool.WBP_PipeTool_C"))
      (Class|ScriptableInteractiveTool|SetOverlayWidget _returnvalue_2 true)
      (Variables|UI|SetButton%20Next (Variables|/Game/Batyscaphe/PipeSystem/PipeTool/WBP_PipeTool.WBP_PipeTool_C|GetButtonNext _returnvalue_2))
      (Variables|Default|SetButton%20Pitch%20Left (Variables|/Game/Batyscaphe/PipeSystem/PipeTool/WBP_PipeTool.WBP_PipeTool_C|GetButtonPitchLeft _returnvalue_2))
      (Variables|Default|SetButton%20Pitch%20Right (Variables|/Game/Batyscaphe/PipeSystem/PipeTool/WBP_PipeTool.WBP_PipeTool_C|GetButtonPitchRight _returnvalue_2))
      (Variables|Default|SetButton%20Yaw%20Left (Variables|/Game/Batyscaphe/PipeSystem/PipeTool/WBP_PipeTool.WBP_PipeTool_C|GetButtonYawLeft _returnvalue_2))
      (Variables|Default|SetButton%20Yaw%20Right (Variables|/Game/Batyscaphe/PipeSystem/PipeTool/WBP_PipeTool.WBP_PipeTool_C|GetButtonYawRight _returnvalue_2))
      (Variables|Default|SetButton%20Roll%20Right (Variables|/Game/Batyscaphe/PipeSystem/PipeTool/WBP_PipeTool.WBP_PipeTool_C|GetButtonRollRight _returnvalue_2))
      (Variables|Default|SetButton%20Roll%20Left (Variables|/Game/Batyscaphe/PipeSystem/PipeTool/WBP_PipeTool.WBP_PipeTool_C|GetButtonRollLeft _returnvalue_2)))
    (:then_2
      (EventDispatchers|BindEventtoOnClicked (Variables|UI|GetButton%20Next) (EventDispatchers|CreateEvent :!event NextClicked))
      ;[0.15 0.15 0.15 0.5] Rotation buttons
      (EventDispatchers|BindEventtoOnClicked (Variables|Default|GetButton%20Pitch%20Left) (EventDispatchers|CreateEvent :!event DecreasePitch))
      (EventDispatchers|BindEventtoOnClicked (Variables|Default|GetButton%20Pitch%20Right) (EventDispatchers|CreateEvent :!event AddPitch))
      (EventDispatchers|BindEventtoOnClicked (Variables|Default|GetButton%20Yaw%20Left) (EventDispatchers|CreateEvent :!event DecreaseYaw))
      (EventDispatchers|BindEventtoOnClicked (Variables|Default|GetButton%20Yaw%20Right) (EventDispatchers|CreateEvent :!event AddYaw))
      (EventDispatchers|BindEventtoOnClicked (Variables|Default|GetButton%20Roll%20Left) (EventDispatchers|CreateEvent :!event DecreaseRoll))
      (EventDispatchers|BindEventtoOnClicked (Variables|Default|GetButton%20Roll%20Right) (EventDispatchers|CreateEvent :!event AddRoll)))
    (:then_3
      (Class|ScriptableModularBehaviorTool|AddSingleClickBehavior (EventDispatchers|CreateEvent :!event Clicked)))))

(event EventOnScriptShutdown
  (params (ShutdownType :type EToolShutdownType%20Enum :default "Completed"))
  (Default|AttachPipe (Variables|Default|GetPipeSystemManager)))

(event EventOnGizmoTransformChanged
  (params (GizmoIdentifier :type String) (NewTransform :type Transform))
  (bind _pipesystemmanager (Variables|Default|GetPipeSystemManager))
  (Utilities|IsValid _pipesystemmanager
    (:Is%20Valid
      (Transformation|SetActorTransform _pipesystemmanager NewTransform))))

(fn SpawnPipeSystemManager
  (params (SpawnLocation :type Vector))
  (bind _returnvalue (Math|Transform|MakeTransform SpawnLocation))
  (bind _returnvalue_2 (Game|SpawnActorfromClass "/Game/Batyscaphe/PipeSystem/BP_CrossroadPipeSystemManager.BP_CrossroadPipeSystemManager_C" _returnvalue "Undefined" "MultiplyWithRoot" 0 0))
  (Variables|Default|SetPipeSystemManager _returnvalue_2)
  (Class|ScriptableInteractiveTool|CreateTRSGizmo "LocationGizmo" _returnvalue (Utilities|Struct|MakeScriptableToolGizmoOptions "TranslationOnly" 255)))

(fn GetLocationUnderCursor
  (params (InputDeviceRay :type Input%20Device%20Ray%20Structure%20%28by%20ref%29))
  (bind _worldray (Utilities|Struct|BreakInputDeviceRay InputDeviceRay))
  (bind (_origin _direction) (Utilities|Struct|BreakRay _worldray))
  (bind (_outhit _returnvalue) (Collision|LineTraceByChannel _origin (+ _origin (* _direction (LocalVariables|GetRayDistanceL))) "TraceTypeQuery1" false (Utilities|Array|MakeArray (Variables|Default|GetPipeSystemManager)) "None"))
  (if _returnvalue
    (return (.Location (Collision|BreakHitResult _outhit)))
    (else
      (return "0, 0, 0"))))

(fn NextClicked
  (Default|AddPipe (Variables|Default|GetPipeSystemManager)))

(fn PipeMeshSelected
  (params (PropertySet :type Scriptable%20Interactive%20Tool%20Property%20Set%20Object%20Reference) (PropertyName :type String) (NewValue :type Byte))
  (Default|SwitchPipeMesh (Variables|Default|GetPipeSystemManager) (Utilities|Enum|ByteToEnumE_PipeType NewValue)))

(fn SpawnSocketSwitched
  (params (PropertySet :type Scriptable%20Interactive%20Tool%20Property%20Set%20Object%20Reference) (PropertyName :type String) (bNewValue :type Boolean))
  (bind _pipesystemmanager (Variables|Default|GetPipeSystemManager))
  (Utilities|IsValid _pipesystemmanager
    (:Is%20Valid
      (Default|SwitchAttachSocket _pipesystemmanager bNewValue))))

(fn Clicked
  (params (ClickPos :type Input%20Device%20Ray%20Structure) (MouseButton :type EScriptableToolMouseButton%20Enum :default "LeftButton"))
  (Utilities|IsValid (Variables|Default|GetPipeSystemManager)
    (:Is%20Not%20Valid
      (bind _location (CallFunction|GetLocationUnderCursor ClickPos))
      (CallFunction|SpawnPipeSystemManager _location)
      (return ""))))

(fn AddPitch
  (Default|SwitchMeshRotation (Variables|Default|GetPipeSystemManager) "0.000000,0.000000,90.000000"))

(fn DecreasePitch
  (Default|SwitchMeshRotation (Variables|Default|GetPipeSystemManager) "0.000000,0.000000,-90.000000"))

(fn AddYaw
  (Default|SwitchMeshRotation (Variables|Default|GetPipeSystemManager) "90.000000,0.000000,0.000000"))

(fn DecreaseYaw
  (Default|SwitchMeshRotation (Variables|Default|GetPipeSystemManager) "-90.000000,0.000000,0.000000"))

(fn AddRoll
  (Default|SwitchMeshRotation (Variables|Default|GetPipeSystemManager) "0.000000,90.000000,0.000000"))

(fn DecreaseRoll
  (Default|SwitchMeshRotation (Variables|Default|GetPipeSystemManager) "0.000000,-90.000000,0.000000"))