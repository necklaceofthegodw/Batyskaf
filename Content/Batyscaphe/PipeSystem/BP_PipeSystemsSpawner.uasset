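; Spawner that assembles a chain of pipe systems at BeginPlay, alternating crossroad managers and spline pipes.
; A flip-flop loop feeds paired datatables and spline data assets into spawned BP_PipeSystemManager1 and BP_PipeSpline1 actors, attached to itself.
; Each piece's transform comes from the previous one's end socket or last spline point, corrected by the crossroad start-socket offset.
; ChooseRandomData, meant to pick random datatables, is unfinished and unused.
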(event EventBeginPlay
  (CallFunction|SpawnPipeSystems))

(event Collision|EventActorBeginOverlap
  (params (OtherActor :type Actor%20Object%20Reference)))

(event EventTick
  (params (DeltaSeconds :type Float%20%28single-precision%29)))

(fn ConstructionScript)

(fn SpawnPipeSystems
  (for _index (range 0 (- (* (Math|Integer|Min(Integer) (Utilities|Array|Length (Variables|Default|GetCrossroadDatatables)) (Utilities|Array|Length (Variables|Default|GetSplineDataAssets))) 2) 1))
    (Utilities|FlowControl|FlipFlop
      (:A
        (LocalVariables|SetPreviousTransformL (Math|Transform|SelectTransform (Transformation|GetActorTransform) (LocalVariables|GetPreviousTransformL) (== _index 0)))
        (bind _returnvalue (Game|SpawnActorfromClass "/Game/Batyscaphe/PipeSystem/CrossroadPipeSystem/BP_PipeSystemManager1.BP_PipeSystemManager1_C" (LocalVariables|GetPreviousTransformL) "Undefined" "MultiplyWithRoot" 0 (Utilities|Array|Get(acopy) (Variables|Default|GetCrossroadDatatables) (Utilities|Array|Length (LocalVariables|GetCrossroadPipeSystemsL))) 0))
        (bind _output_get (LocalVariables|SetPreviousCrossroadL _returnvalue))
        (Utilities|Array|Add (LocalVariables|GetCrossroadPipeSystemsL) _output_get)
        (Transformation|AttachActorToActor _output_get self "" "KeepWorld" "KeepWorld" "KeepWorld" true)
        (LocalVariables|SetPreviousTransformL (Math|Conversions|ToTransform(Vector) (Transformation|GetSocketLocation (Variables|/Game/Batyscaphe/PipeSystem/BP_Pipe.BP_Pipe_C|GetSM_Pipe (Variables|/Game/Batyscaphe/PipeSystem/CrossroadPipeSystem/BP_PipeSystemManager1.BP_PipeSystemManager1_C|GetEndCrossroad (LocalVariables|GetPreviousCrossroadL))) "Socket3"))))
      (:B
        (bind _returnvalue_2 (Game|SpawnActorfromClass "/Game/Batyscaphe/PipeSystem/SplinePipeSystem/BP_PipeSpline1.BP_PipeSpline1_C" (Math|Transform|MakeTransform (.Location (Math|Transform|BreakTransform (LocalVariables|GetPreviousTransformL))) "-90.000000,0.000000,0.000000" (.Scale (Math|Transform|BreakTransform (LocalVariables|GetPreviousTransformL)))) "Undefined" "MultiplyWithRoot" 0 (Utilities|Array|Get(acopy) (Variables|Default|GetSplineDataAssets) (Utilities|Array|Length (LocalVariables|GetSplinePipeSystemsL))) 0))
        (bind _output_get_2 (LocalVariables|SetPreviousSplineL _returnvalue_2))
        (Utilities|Array|Add (LocalVariables|GetSplinePipeSystemsL) _output_get_2)
        (Transformation|AttachActorToActor _output_get_2 self "" "KeepWorld" "KeepWorld" "KeepRelative" true)
        (bind _outlocation (Default|GetLastSplinePointLocation _output_get_2))
        (LocalVariables|SetPreviousTransformL (Math|Conversions|ToTransform(Vector) (+ _outlocation (- (Transformation|GetActorLocation (LocalVariables|GetPreviousCrossroadL)) (Transformation|GetSocketLocation (Variables|/Game/Batyscaphe/PipeSystem/CrossroadPipeSystem/BP_PipeSystemManager1.BP_PipeSystemManager1_C|GetSM_StartCrossroad (LocalVariables|GetPreviousCrossroadL)) "Socket3")))))))))

(fn ChooseRandomData
  (params (ItemsMax :type Integer))
  (bind _outcrossroaddatatables (LocalVariables|GetOutCrossroadDatatables))
  (bind _outcrossroaddatatables_2 (LocalVariables|GetOutCrossroadDatatables))
  ;[0.15 0.15 0.15 0.5] TODO FInish this
  (while (< (Utilities|Array|Length _outcrossroaddatatables_2) ItemsMax)
    (Utilities|Array|AddUnique _outcrossroaddatatables_2 (.OutItem (Utilities|Array|Random (Variables|Default|GetCrossroadDatatables)))))
  (while (< (Utilities|Array|Length _outcrossroaddatatables) 0)
    (Utilities|Array|AddUnique _outcrossroaddatatables (.OutItem (Utilities|Array|Random (Variables|Default|GetCrossroadDatatables))))))