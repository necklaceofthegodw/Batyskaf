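; Pipe system manager actor that builds a pipe network at BeginPlay from data table rows, starting at a crossroad mesh socket.
; Each row spawns a BP_Pipe with its type's mesh and the row's rotation at the previous socket, then supplies the socket name for the next link.
; Spawned pipes are stored and attached to the manager.
; A routine scattering collectibles around pipe "Spawn" sockets exists but is never called.
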(event EventBeginPlay
  (CallFunction|SpawnPipes))

(event Collision|EventActorBeginOverlap
  (params (OtherActor :type Actor%20Object%20Reference)))

(event EventTick
  (params (DeltaSeconds :type Float%20%28single-precision%29)))

(fn ConstructionScript)

(fn SpawnPipes
  (bind _pipetable (Variables|Default|GetPipeTable))
  (Variables|Default|SetPreviousSocketTransform (Transformation|GetSocketTransform (Variables|Default|GetSM_StartCrossroad) "Socket2" "RTS_World"))
  (bind _outrownames (DataTable|GetDataTableRowNames _pipetable))
  (for _array_element _outrownames
    (bind _returnvalue (Utilities|GetDataTableRow _pipetable _array_element)
      (:then
        (bind _returnvalue_2 (Game|SpawnActorfromClass "/Game/Batyscaphe/PipeSystem/BP_Pipe.BP_Pipe_C" (Math|Transform|MakeTransform (.Location (Math|Transform|BreakTransform (Variables|Default|GetPreviousSocketTransform))) (.PipeRotation (Utilities|Struct|BreakS_PipeAttachmentInfo _returnvalue)) (.Scale (Math|Transform|BreakTransform (Variables|Default|GetPreviousSocketTransform)))) "Undefined" "MultiplyWithRoot" 0 (.Value (Utilities|Map|Find (Variables|Default|GetPipeTypeToMesh) (.PipeType (Utilities|Struct|BreakS_PipeAttachmentInfo _returnvalue)))) (.PipeType (Utilities|Struct|BreakS_PipeAttachmentInfo _returnvalue)) true 0))
        (CallFunction|SetActorLocationtoSocket (.PreviousPipeSocket (Utilities|Struct|BreakS_PipeAttachmentInfo _returnvalue)))
        (Utilities|Array|Add (Variables|Default|GetPipes) _returnvalue_2)
        (Variables|Default|SetPreviousSocketTransform (Transformation|GetSocketTransform (Variables|/Game/Batyscaphe/PipeSystem/BP_Pipe.BP_Pipe_C|GetSM_Pipe _returnvalue_2) (.PreviousPipeSocket (Utilities|Struct|BreakS_PipeAttachmentInfo _returnvalue)) "RTS_World"))
        (Transformation|AttachActorToActor _returnvalue_2 self (.PreviousPipeSocket (Utilities|Struct|BreakS_PipeAttachmentInfo _returnvalue)) "KeepWorld" "KeepWorld" "KeepRelative" true)))))

(fn SpawnCollectibles
  (for _array_element (Variables|Default|GetPipes)
    (for _array_element_2 (Transformation|GetAllSocketNames (Variables|/Game/Batyscaphe/PipeSystem/BP_Pipe.BP_Pipe_C|GetSM_Pipe _array_element))
      (if (Utilities|String|Contains (Utilities|String|ToString(Name) _array_element_2) "Spawn")
        (for _index (range 0 10)
          (Game|SpawnActorfromClass "/Game/Batyscaphe/Collectables/BP_Collectable2.BP_Collectable2_C" (Math|Conversions|ToTransform(Vector) (CallFunction|GetRandomLocationinSphere (Transformation|GetSocketLocation (Variables|/Game/Batyscaphe/PipeSystem/BP_Pipe.BP_Pipe_C|GetSM_Pipe _array_element) _array_element_2) 3e+03)) "Undefined" "MultiplyWithRoot" 0 "NewEnumerator0" 0))))))

(fn GetSocketName
  (params (bFirstSocket :type Boolean))
  (return (Utilities|String|SelectName "Socket2" "Socket1" bFirstSocket)))

(fn SetActorLocationtoSocket
  (params (AttachSocketName1 :type Name))
  (bind _pipes (Variables|Default|GetPipes))
  (bind _returnvalue (Utilities|Array|LastIndex _pipes))
  (bind _returnvalue_2 (- _returnvalue 1))
  (bind _output (Utilities|Array|Get(acopy) _pipes _returnvalue_2))
  (LocalVariables|SetAttachSocketName AttachSocketName1)
  (Utilities|IsValid _output
    (:Is%20Valid
      (Transformation|SetActorLocation (Utilities|Array|Get(acopy) _pipes _returnvalue) (Transformation|GetSocketLocation (Variables|/Game/Batyscaphe/PipeSystem/BP_Pipe.BP_Pipe_C|GetSM_Pipe _output) (LocalVariables|GetAttachSocketName)) false false))))