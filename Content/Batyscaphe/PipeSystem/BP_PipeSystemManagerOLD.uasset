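; Pipe system manager (marked OLD) that assembles a chained pipe layout from a data table during construction when SpawnFromTable is set.
; SpawnPipes spawns a BP_Pipe per row, picks its mesh by type and attaches it to the previous pipe's named socket, keeping the row's world rotation.
; SpawnCollectibles scatters collectables randomly around pipe sockets named with "Spawn", but nothing in this graph calls it.
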(event EventBeginPlay)

(event Collision|EventActorBeginOverlap
  (params (OtherActor :type Actor%20Object%20Reference)))

(event EventTick
  (params (DeltaSeconds :type Float%20%28single-precision%29)))

(fn ConstructionScript
  (if (Variables|Default|GetbSpawnFromTable)
    (CallFunction|SpawnPipes)))

(fn SpawnPipes
  (bind _pipetable (Variables|Default|GetPipeTable))
  (Variables|Default|SetPreviousSocketTransfo (Transformation|GetActorTransform))
  (bind _outrownames (DataTable|GetDataTableRowNames _pipetable))
  (for _array_element _outrownames
    (bind _returnvalue (Utilities|GetDataTableRow _pipetable _array_element)
      (:then
        (bind _returnvalue_2 (Game|SpawnActorfromClass "/Game/Batyscaphe/PipeSystem/BP_Pipe.BP_Pipe_C" (Math|Transform|MakeTransform (.Location (Math|Transform|BreakTransform (Variables|Default|GetPreviousSocketTransfo))) (.PipeRotation (Utilities|Struct|BreakS_PipeAttachmentInfo _returnvalue)) (.Scale (Math|Transform|BreakTransform (Variables|Default|GetPreviousSocketTransfo)))) "Undefined" "MultiplyWithRoot" 0 (.Value (Utilities|Map|Find (Variables|Default|GetPipeTypeToMesh) (.PipeType (Utilities|Struct|BreakS_PipeAttachmentInfo _returnvalue)))) "NewEnumerator6" false 0))
        (Utilities|Array|Add (Variables|Default|GetPipes) _returnvalue_2)
        (Utilities|IsValid (LocalVariables|GetPreviousMesh)
          (:Is%20Valid
            (Variables|Default|SetPreviousSocketTransfo (Transformation|GetSocketTransform (Variables|/Game/Batyscaphe/PipeSystem/BP_Pipe.BP_Pipe_C|GetSM_Pipe (LocalVariables|GetPreviousMesh)) (.PreviousPipeSocket (Utilities|Struct|BreakS_PipeAttachmentInfo _returnvalue)) "RTS_World"))
            (Transformation|AttachActorToActor _returnvalue_2 (LocalVariables|GetPreviousMesh) (.PreviousPipeSocket (Utilities|Struct|BreakS_PipeAttachmentInfo _returnvalue)) "SnapToTarget" "KeepWorld" "KeepRelative" true)
            (LocalVariables|SetPreviousMesh _returnvalue_2))
          (:Is%20Not%20Valid
            (bind _output_get (LocalVariables|SetPreviousMesh _returnvalue_2))
            (Variables|Default|SetPreviousSocketTransfo (Transformation|GetSocketTransform (Variables|/Game/Batyscaphe/PipeSystem/BP_Pipe.BP_Pipe_C|GetSM_Pipe _output_get) "None" "RTS_World"))))))))

(fn SpawnCollectibles
  (for _array_element (Variables|Default|GetPipes)
    (for _array_element_2 (Transformation|GetAllSocketNames (Variables|/Game/Batyscaphe/PipeSystem/BP_Pipe.BP_Pipe_C|GetSM_Pipe _array_element))
      (if (Utilities|String|Contains (Utilities|String|ToString(Name) _array_element_2) "Spawn")
        (for _index (range 0 10)
          (Game|SpawnActorfromClass "/Game/Batyscaphe/Collectables/BP_Collectable2.BP_Collectable2_C" (Math|Conversions|ToTransform(Vector) (CallFunction|GetRandomLocationinSphere (Transformation|GetSocketLocation (Variables|/Game/Batyscaphe/PipeSystem/BP_Pipe.BP_Pipe_C|GetSM_Pipe _array_element) _array_element_2) 3e+03)) "Undefined" "MultiplyWithRoot" 0 "NewEnumerator0" 0))))))