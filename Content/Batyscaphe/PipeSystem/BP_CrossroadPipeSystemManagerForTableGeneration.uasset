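; Crossroad pipe system manager that builds chains of BP_Pipe actors from a start crossroad mesh, interactively or from a data table.
; Editing functions add a highlighted pipe, switch its mesh, socket or rotation, then record type, socket and rotation in PipeAttachmentsInfos on attach.
; Chains can be respawned from that array or from PipeTable, optionally in the Construction Script, using mesh sockets to place and attach each pipe.
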(event EventBeginPlay
  (|CallParentFunction))

(event Collision|EventActorBeginOverlap
  (params (OtherActor :type Actor%20Object%20Reference))
  (|CallParentFunction OtherActor) ; This node is disabled and will not be called.\nDrag off pins to build functionality.
)

(event EventTick
  (params (DeltaSeconds :type Float%20%28single-precision%29))
  (|CallParentFunction DeltaSeconds) ; This node is disabled and will not be called.\nDrag off pins to build functionality.
)

(fn ConstructionScript
  (if (Variables|Default|GetbSpawnFromTable)
    (CallFunction|SpawnPipesfromTable (Variables|Default|GetPipeTable) false)))

(fn SpawnPipesfromTable
  (params (DataTable :type Data%20Table%20Object%20Reference) (IsRight :type Boolean))
  (LocalVariables|SetPreviousSocketTransformL (Transformation|GetActorTransform))
  (bind _outrownames (DataTable|GetDataTableRowNames DataTable))
  (for _array_element _outrownames
    (bind _returnvalue (Utilities|GetDataTableRow DataTable _array_element)
      (:then
        (bind _returnvalue_2 (Game|SpawnActorfromClass "/Game/Batyscaphe/PipeSystem/BP_Pipe.BP_Pipe_C" (Math|Transform|MakeTransform (.Location (Math|Transform|BreakTransform (LocalVariables|GetPreviousSocketTransformL))) (.PipeRotation (Utilities|Struct|BreakS_PipeAttachmentInfo _returnvalue)) (.Scale (Math|Transform|BreakTransform (LocalVariables|GetPreviousSocketTransformL)))) "Undefined" "MultiplyWithRoot" 0 (.Value (Utilities|Map|Find (Variables|Default|GetPipeTypeToMesh) (.PipeType (Utilities|Struct|BreakS_PipeAttachmentInfo _returnvalue)))) "/Game/Fab/Megascans/3D/Painted_Pipe_Straight_tiwidimhx/Medium/MI_tiwidimhx.MI_tiwidimhx" "NewEnumerator6" false 0))
        (Utilities|Array|Add (Variables|Default|GetPipes) _returnvalue_2)
        (Utilities|IsValid (Variables|Default|GetPreviousPIpee)
          (:Is%20Valid
            (LocalVariables|SetPreviousSocketTransformL (Transformation|GetSocketTransform (Variables|/Game/Batyscaphe/PipeSystem/BP_Pipe.BP_Pipe_C|GetSM_Pipe (Variables|Default|GetPreviousPIpee)) (.PreviousPipeSocket (Utilities|Struct|BreakS_PipeAttachmentInfo _returnvalue)) "RTS_World"))
            (Transformation|AttachActorToActor _returnvalue_2 (Variables|Default|GetPreviousPIpee) (.PreviousPipeSocket (Utilities|Struct|BreakS_PipeAttachmentInfo _returnvalue)) "SnapToTarget" "KeepWorld" "KeepRelative" true)
            (Variables|Default|SetPreviousPIpee _returnvalue_2))
          (:Is%20Not%20Valid
            (bind _output_get (Variables|Default|SetPreviousPIpee _returnvalue_2))
            (LocalVariables|SetPreviousSocketTransformL (Transformation|GetSocketTransform (Variables|/Game/Batyscaphe/PipeSystem/BP_Pipe.BP_Pipe_C|GetSM_Pipe _output_get) (.PreviousPipeSocket (Utilities|Struct|BreakS_PipeAttachmentInfo _returnvalue)) "RTS_World"))
            ;[0.15 0.15 0.15 0.5] Socket1 - right
            (Transformation|AttachComponentToComponent _output_get (Variables|Default|GetSM_StartCrossroad) (.PreviousPipeSocket (Utilities|Struct|BreakS_PipeAttachmentInfo _returnvalue)) "SnapToTarget" "KeepWorld" "KeepRelative" true)))))))

(fn AddPipe
  (bind _outendsockettransform (CallFunction|GetEndSocketTransform))
  (bind (_location _rotation _scale) (Math|Transform|BreakTransform _outendsockettransform))
  (if (> (Utilities|Array|Length (Variables|Default|GetPipes)) 0)
    (Pipetool|AttachPipe)
    (LocalVariables|SetSpawnTransformL (Math|Transform|MakeTransform _location "0, 0, 0" _scale))
    (else
      (LocalVariables|SetSpawnTransformL (Transformation|GetSocketTransform (Variables|Default|GetSM_StartCrossroad) (PipeTool|GetSocketName (Variables|Default|GetIsRight)) "RTS_World"))))
  (bind _returnvalue (Game|SpawnActorfromClass "/Game/Batyscaphe/PipeSystem/BP_Pipe.BP_Pipe_C" (LocalVariables|GetSpawnTransformL) "Undefined" "MultiplyWithRoot" 0 (.Value (Utilities|Map|Find (Variables|Default|GetPipeTypeToMesh) (Variables|Default|GetCurrentPipeType))) "/Game/Fab/Megascans/3D/Painted_Pipe_Straight_tiwidimhx/Medium/MI_tiwidimhx.MI_tiwidimhx" "NewEnumerator6" false 0))
  (Utilities|Array|Add (Variables|Default|GetPipes) _returnvalue)
  (Default|HighlightPipe _returnvalue true)
  (PipeTool|SwitchPipeMesh (Variables|Default|GetCurrentPipeType))
  (PipeTool|SwitchAttachSocket (Variables|Default|GetIsRight)))

(fn AttachPipe
  (bind _pipes (Variables|Default|GetPipes))
  (bind _returnvalue (Utilities|Array|LastIndex _pipes))
  (bind _output (Utilities|Array|Get(acopy) _pipes _returnvalue))
  (Utilities|Array|Add (Variables|Default|GetPipeAttachmentsInfos) (Utilities|Struct|MakeS_PipeAttachmentInfo (Variables|Default|GetCurrentPipeType) (PipeTool|GetSocketName (Variables|Default|GetIsRight)) (Variables|Default|GetCurrentPipeRotation)))
  (Variables|Default|SetCurrentPipeRotation "0, 0, 0")
  (Default|HighlightPipe _output false)
  (Variables|Default|SetPreviousActorTransform (Transformation|GetActorTransform _output))
  (Transformation|AttachActorToActor _output self (PipeTool|GetSocketName (Variables|Default|GetIsRight)) "KeepWorld" "KeepWorld" "KeepRelative" true)
  (if (Utilities|Enum|Equal(Enum) (Variables|Default|GetCurrentPipeType) "NewEnumerator4")
    (Variables|Default|SetCrossroadPipe _output)))

(fn SwitchPipeMesh
  (params (PipeType :type E_PipeType%20Enum :default "NewEnumerator0"))
  (bind _pipes (Variables|Default|GetPipes))
  (bind _pipetypetomesh (Variables|Default|GetPipeTypeToMesh))
  (bind _returnvalue (Utilities|Array|LastIndex _pipes))
  (bind _value (Utilities|Map|Find _pipetypetomesh PipeType))
  (bind _output (Utilities|Array|Get(acopy) _pipes _returnvalue))
  (Variables|Default|SetCurrentPipeType PipeType)
  (if (> (Utilities|Array|Length _pipes) 0)
    (Components|StaticMesh|SetStaticMesh (Variables|/Game/Batyscaphe/PipeSystem/BP_Pipe.BP_Pipe_C|GetSM_Pipe _output) _value)
    (Variables|/Game/Batyscaphe/PipeSystem/BP_Pipe.BP_Pipe_C|SetPipeMesh _output _value)))

(fn SwitchAttachSocket
  (params (IsRight :type Boolean))
  (bind _pipes (Variables|Default|GetPipes))
  (bind _returnvalue (Utilities|Array|LastIndex _pipes))
  (bind _output (Utilities|Array|Get(acopy) _pipes _returnvalue))
  (bind _returnvalue_2 (- _returnvalue 1))
  (bind _output_2 (Utilities|Array|Get(acopy) _pipes _returnvalue_2))
  (bind _output_get (Variables|Default|SetIsRight IsRight))
  (LocalVariables|SetAttachSocketName (PipeTool|GetSocketName _output_get))
  (Utilities|IsValid _output_2
    (:Is%20Valid
      (Transformation|SetActorLocation _output (Transformation|GetSocketLocation (Variables|/Game/Batyscaphe/PipeSystem/BP_Pipe.BP_Pipe_C|GetSM_Pipe _output_2) (LocalVariables|GetAttachSocketName)) false false))
    (:Is%20Not%20Valid
      (Transformation|SetActorLocation _output (Transformation|GetSocketLocation (Variables|Default|GetSM_StartCrossroad) (LocalVariables|GetAttachSocketName)) false false))))

(fn SwitchMeshRotation
  (params (RotationToAdd :type Rotator))
  (bind _pipes (Variables|Default|GetPipes))
  (bind _output_get (Variables|Default|SetCurrentPipeRotation (Math|Rotator|CombineRotators (Variables|Default|GetCurrentPipeRotation) RotationToAdd)))
  (Transformation|SetActorRotation (Utilities|Array|Get(acopy) _pipes (Utilities|Array|LastIndex _pipes)) _output_get))

(fn GetSocketName
  (params (bFirstSocket :type Boolean))
  (return (Utilities|String|SelectName "Socket1" "Socket2" bFirstSocket)))

(fn AttachLastPipe
  (bind _pipes (Variables|Default|GetPipes))
  (bind _returnvalue (Utilities|Array|LastIndex _pipes))
  (bind _output (Utilities|Array|Get(acopy) _pipes _returnvalue))
  (Utilities|IsValid _output
    (:Is%20Valid
      (Transformation|AttachActorToActor _output self (PipeTool|GetSocketName (Variables|Default|GetIsRight)) "KeepWorld" "KeepWorld" "KeepRelative" true))))

(fn DetachLastPipe
  (bind _pipes (Variables|Default|GetPipes))
  (bind _returnvalue (Utilities|Array|LastIndex _pipes))
  (bind _output (Utilities|Array|Get(acopy) _pipes _returnvalue))
  (Utilities|IsValid _output
    (:Is%20Valid
      (Transformation|DetachFromActor _output "KeepWorld" "KeepWorld" "KeepRelative"))))

(fn GetEndSocketTransform
  (bind _pipes (Variables|Default|GetPipes))
  (bind _returnvalue (Utilities|Array|LastIndex _pipes))
  (bind _output (Utilities|Array|Get(acopy) _pipes _returnvalue))
  (bind _sm_pipe (Variables|/Game/Batyscaphe/PipeSystem/BP_Pipe.BP_Pipe_C|GetSM_Pipe _output))
  (bind _output_get (Variables|Default|SetIsRight (> (Math|Vector|Distance(Vector) (.Location (Math|Transform|BreakTransform (Variables|Default|GetPreviousActorTransform))) (.Location (Math|Transform|BreakTransform (Transformation|GetSocketTransform _sm_pipe "Socket1" "RTS_World")))) 2e+02)))
  (return (Transformation|GetSocketTransform _sm_pipe (PipeTool|GetSocketName _output_get) "RTS_World")))

(fn SpawnPipesfromAttachmentInfos
  (bind _pipes (Variables|Default|GetPipes))
  (for _array_element _pipes
    (Transformation|DetachFromActor _array_element "KeepRelative" "KeepRelative" "KeepRelative")
    (Actor|DestroyActor _array_element))
  (Utilities|Array|Clear _pipes)
  (LocalVariables|SetPreviousSocketTransform (Transformation|GetActorTransform))
  (for _array_element_2 (Variables|Default|GetPipeAttachmentsInfos)
    (bind _returnvalue (Game|SpawnActorfromClass "/Game/Batyscaphe/PipeSystem/BP_Pipe.BP_Pipe_C" (Math|Transform|MakeTransform (.Location (Math|Transform|BreakTransform (LocalVariables|GetPreviousSocketTransform))) (.PipeRotation (Utilities|Struct|BreakS_PipeAttachmentInfo _array_element_2)) (.Scale (Math|Transform|BreakTransform (LocalVariables|GetPreviousSocketTransform)))) "Undefined" "MultiplyWithRoot" 0 (.Value (Utilities|Map|Find (Variables|Default|GetPipeTypeToMesh) (.PipeType (Utilities|Struct|BreakS_PipeAttachmentInfo _array_element_2)))) "/Game/Fab/Megascans/3D/Painted_Pipe_Straight_tiwidimhx/Medium/MI_tiwidimhx.MI_tiwidimhx" "NewEnumerator6" false 0))
    (Utilities|Array|Add (Variables|Default|GetPipes) _returnvalue)
    (LocalVariables|SetPreviousSocketTransform (Transformation|GetSocketTransform (Variables|/Game/Batyscaphe/PipeSystem/BP_Pipe.BP_Pipe_C|GetSM_Pipe _returnvalue) (.PreviousPipeSocket (Utilities|Struct|BreakS_PipeAttachmentInfo _array_element_2)) "RTS_World"))
    (Transformation|AttachActorToActor _returnvalue self (.PreviousPipeSocket (Utilities|Struct|BreakS_PipeAttachmentInfo _array_element_2)) "KeepWorld" "KeepWorld" "KeepRelative" true)))

(fn SpawnPipes
  (bind _pipetable (Variables|Default|GetPipeTable))
  (Variables|Default|SetPreviousSocketTransfo (Transformation|GetActorTransform))
  (bind _outrownames (DataTable|GetDataTableRowNames _pipetable))
  (for _array_element _outrownames
    (bind _returnvalue (Utilities|GetDataTableRow _pipetable _array_element)
      (:then
        (bind _returnvalue_2 (Game|SpawnActorfromClass "/Game/Batyscaphe/PipeSystem/BP_Pipe.BP_Pipe_C" (Math|Transform|MakeTransform (.Location (Math|Transform|BreakTransform (Variables|Default|GetPreviousSocketTransfo))) (.PipeRotation (Utilities|Struct|BreakS_PipeAttachmentInfo _returnvalue)) (.Scale (Math|Transform|BreakTransform (Variables|Default|GetPreviousSocketTransfo)))) "Undefined" "MultiplyWithRoot" 0 (.Value (Utilities|Map|Find (Variables|Default|GetPipeTypeToMesh) (.PipeType (Utilities|Struct|BreakS_PipeAttachmentInfo _returnvalue)))) "/Game/Fab/Megascans/3D/Painted_Pipe_Straight_tiwidimhx/Medium/MI_tiwidimhx.MI_tiwidimhx" "NewEnumerator6" false 0))
        (Utilities|Array|Add (Variables|Default|GetPipes) _returnvalue_2)
        (Utilities|IsValid (LocalVariables|GetPreviousMeshL)
          (:Is%20Valid
            (Variables|Default|SetPreviousSocketTransfo (Transformation|GetSocketTransform (Variables|/Game/Batyscaphe/PipeSystem/BP_Pipe.BP_Pipe_C|GetSM_Pipe (LocalVariables|GetPreviousMeshL)) (.PreviousPipeSocket (Utilities|Struct|BreakS_PipeAttachmentInfo _returnvalue)) "RTS_World"))
            (Transformation|AttachActorToActor _returnvalue_2 (LocalVariables|GetPreviousMeshL) (.PreviousPipeSocket (Utilities|Struct|BreakS_PipeAttachmentInfo _returnvalue)) "SnapToTarget" "KeepWorld" "KeepRelative" true)
            (LocalVariables|SetPreviousMeshL _returnvalue_2))
          (:Is%20Not%20Valid
            (LocalVariables|SetPreviousMeshL _returnvalue_2)
            (Variables|Default|SetPreviousSocketTransfo (Transformation|GetSocketTransform (Variables|Default|GetSM_StartCrossroad) (.PreviousPipeSocket (Utilities|Struct|BreakS_PipeAttachmentInfo _returnvalue)) "RTS_World"))))))))