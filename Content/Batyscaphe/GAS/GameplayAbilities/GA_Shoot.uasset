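; Gameplay ability that lets the submarine pawn shoot whatever shootable object sits under the screen center.
; After committing, it line-traces on the Visibility channel from the deprojected viewport center of player controller 0.
; A hit actor implementing I_Shootable triggers the GameplayCue.Shot cue at the impact point and receives OnShot with the submarine.
; The ability ends immediately after the shot attempt, with a debug print on success.
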(event Ability|EventActivateAbility
  (bind _returnvalue (Ability|CommitAbility))
  (if _returnvalue
    (bind _asbp_submarine_pawn (Utilities|Casting|CastToBP_SubmarinePawn (Ability|GetAvatarActorfromActorInfo)))
    (Variables|Default|SetSubmarineOwning _asbp_submarine_pawn)
    (bind _asi_shootable (CallFunction|IsShootableUnderCrosshair))
    (if (Utilities|IsValidInterface _asi_shootable)
      (Default|OnShot _asi_shootable (Variables|Default|GetSubmarineOwning))
      (Development|PrintString "Shoot"))
    (Ability|EndAbility)))

(event Ability|EventOnEndAbility
  (params (bWasCancelled :type Boolean)))

(fn IsShootableUnderCrosshair
  (bind _returnvalue (Viewport|GetViewportSize))
  (bind _returnvalue_2 (Game|GetPlayerController 0))
  (bind (_x _y) (Math|Vector2D|BreakVector2D _returnvalue))
  (bind _returnvalue_3 (* _y 0.5))
  (bind _returnvalue_4 (* _x 0.5))
  (bind _returnvalue_5 (Math|Vector2D|MakeVector2D _returnvalue_4 _returnvalue_3))
  (bind (_worldposition _worlddirection) (Class|GameplayStatics|DeprojectScreentoWorld _returnvalue_2 _returnvalue_5))
  (bind (_outhit _returnvalue_6) (Collision|LineTraceByChannel _worldposition (+ _worldposition (* _worlddirection (LocalVariables|GetLineTraceLengthL))) "TraceTypeQuery1" false 0 "None" true "(R=1.000000,G=0.000000,B=0.000000,A=1.000000)" "(R=0.000000,G=1.000000,B=0.000000,A=1.000000)" 0.0))
  (if _returnvalue_6
    (bind _asi_shootable (Utilities|Casting|CastToI_Shootable (.HitActor (Collision|BreakHitResult _outhit)))
      (:then
        (Class|GameplayAbility|ExecuteGameplayCuewithParams "(TagName=\"GameplayCue.Shot\")" (Ability|GameplayCue|MakeGameplayCueParameters :Location (.Location (Collision|BreakHitResult _outhit))))
        (return _asi_shootable))
      (:CastFailed
        _)))
  (return 0))