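; Rocket projectile actor that, once shot, flies toward a given target location with a Niagara effect.
; Shot activates the effect and ProjectileMovement, then Tick steps the actor toward the fixed point by Speed per frame, without delta-time scaling, re-aiming it each step.
; It destroys itself shortly after nearing the target or after a timeout.
; A timeline-based MoveToTarget alternative exists but is not called here.
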(event Custom|Shot
  (params (TargetLocation :type Vector))
  (Variables|Default|SetTargetLocation TargetLocation)
  (Variables|Default|SetStartLocation (Transformation|GetActorLocation))
  (Components|Activation|SetActive (Variables|Default|GetNS_Niagara) true true)
  (Transformation|SetActorRotation (Math|Rotator|FindLookatRotation (Variables|Default|GetStartLocation) (Variables|Default|GetTargetLocation)))
  (Variables|Default|SetIsMoving true)
  (Utilities|FlowControl|Delay 5.0)
  (Variables|Default|SetIsMoving false)
  (CallFunction|DestroyProjectile))

(event Custom|MoveToTarget
  ;[0.15 0.15 0.15 0.5] Move in 2 seconds to target
  (bind _position (Timeline|MoveTimeline PlayFromStart)
    (:Update
      (Transformation|SetActorLocation (Math|Vector|Lerp(Vector) (Variables|Default|GetStartLocation) (Variables|Default|GetTargetLocation) _position) true false))))

(event Custom|DestroyProjectile
  (Components|Activation|Deactivate (Variables|Default|GetNS_Niagara))
  (Components|Activation|SetActive (Variables|Default|GetProjectileMovement) false true)
  (Utilities|Time|ClearandInvalidateTimerbyHandle (Variables|Default|GetMoveHandle))
  (Actor|DestroyActor))

(event Custom|DestroyDelayed
  (Utilities|FlowControl|Delay 0.2)
  (Components|Activation|Deactivate (Variables|Default|GetNS_Niagara))
  (Components|Activation|SetActive (Variables|Default|GetProjectileMovement) false true)
  (Utilities|Time|ClearandInvalidateTimerbyHandle (Variables|Default|GetMoveHandle))
  (Actor|DestroyActor))

(event Custom|MoveTowardsTarget
  (bind _returnvalue (Transformation|GetActorLocation))
  ;[0.15 0.15 0.15 0.5] Move with constant speed towards target
  (Transformation|SetActorLocation (+ _returnvalue (* (Math|Vector|GetUnitDirection(Vector) _returnvalue (Variables|Default|GetTargetLocation)) (Variables|Default|GetSpeed))) true false)
  (Transformation|SetActorRotation (Math|Rotator|FindLookatRotation _returnvalue (Variables|Default|GetTargetLocation)))
  (if (Utilities|Operators|EqualEqual (Transformation|GetActorLocation) (Variables|Default|GetTargetLocation) 2e+02)
    (Variables|Default|SetIsMoving false)
    (CallFunction|DestroyDelayed)))

(event EventBeginPlay)

(event EventTick
  (params (DeltaSeconds :type Float%20%28single-precision%29))
  (if (Variables|Default|GetIsMoving)
    (CallFunction|MoveTowardsTarget)))

(fn ConstructionScript)