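; Gameplay ability that fires the submarine's loaded rocket at whatever lies under the screen-center crosshair.
; On activation it commits, then line-traces from the deprojected viewport center, using the hit point or trace end as the target.
; A Shot gameplay cue plays only on I_Shootable hits, whose OnShot call is disconnected.
; The current rocket is detached, launched at the target and cleared, with debug sphere and print left in.
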(event Ability|EventActivateAbility
  (bind _returnvalue (Ability|CommitAbility))
  (if _returnvalue
    (bind _asbp_submarine_pawn (Utilities|Casting|CastToBP_SubmarinePawn (Ability|GetAvatarActorfromActorInfo)))
    (Variables|Default|SetSubmarineOwning _asbp_submarine_pawn)
    (bind (_asi_shootable _outshootlocation) (CallFunction|IsShootableUnderCrosshair))
    (Rendering|Debug|DrawDebugSphere _outshootlocation 1e+02 12 "(R=1.000000,G=0.174955,B=0.110435,A=1.000000)" 5.0 5.0)
    (CallFunction|ShootRocket _outshootlocation)
    (if (Utilities|IsValidInterface _asi_shootable)
      (Development|PrintString "Shoot"))
    (Ability|EndAbility)))

(event Ability|EventOnEndAbility
  (params (bWasCancelled :type Boolean)))

(fn IsShootableUnderCrosshair
  (bind _returnvalue (Viewport|GetViewportSize))
  (bind _returnvalue_2 (Game|GetPlayerController 0))
  (bind _linetracelengthl (LocalVariables|GetLineTraceLengthL))
  (bind (_x _y) (Math|Vector2D|BreakVector2D _returnvalue))
  (bind _returnvalue_3 (* _y 0.5))
  (bind _returnvalue_4 (* _x 0.5))
  (bind _returnvalue_5 (Math|Vector2D|MakeVector2D _returnvalue_4 _returnvalue_3))
  (bind (_worldposition _worlddirection) (Class|GameplayStatics|DeprojectScreentoWorld _returnvalue_2 _returnvalue_5))
  (bind _returnvalue_6 (* _worlddirection _linetracelengthl))
  (bind _returnvalue_7 (+ _worldposition _returnvalue_6))
  (bind (_outhit _returnvalue_8) (Collision|LineTraceByChannel _worldposition _returnvalue_7 "TraceTypeQuery3" false 0 "None" true "(R=1.000000,G=0.000000,B=0.000000,A=1.000000)" "(R=0.000000,G=1.000000,B=0.000000,A=1.000000)" 0.0))
  (if _returnvalue_8
    (bind _asi_shootable (Utilities|Casting|CastToI_Shootable (.HitActor (Collision|BreakHitResult _outhit)))
      (:then
        (Class|GameplayAbility|ExecuteGameplayCuewithParams "(TagName=\"GameplayCue.Shot\")" (Ability|GameplayCue|MakeGameplayCueParameters :Location (.Location (Collision|BreakHitResult _outhit))))
        (LocalVariables|SetShootLocationL (.Location (Collision|BreakHitResult _outhit)))
        (return _asi_shootable (LocalVariables|GetShootLocationL)))
      (:CastFailed
        (LocalVariables|SetShootLocationL (.Location (Collision|BreakHitResult _outhit)))))
    (else
      (bind _output_get (LocalVariables|SetShootLocationL _returnvalue_7))))
  (return 0 _output_get))

(fn ShootRocket
  (params (TargetLocation :type Vector))
  (bind _submarineowning (Variables|Default|GetSubmarineOwning))
  (Utilities|IsValid (Variables|/Game/Batyscaphe/submarine/BP_SubmarinePawn.BP_SubmarinePawn_C|GetCurrentRocket _submarineowning)
    (:Is%20Valid
      (Transformation|DetachFromActor (Variables|/Game/Batyscaphe/submarine/BP_SubmarinePawn.BP_SubmarinePawn_C|GetCurrentRocket _submarineowning) "KeepWorld" "KeepWorld" "KeepWorld")
      (Default|Shot (Variables|/Game/Batyscaphe/submarine/BP_SubmarinePawn.BP_SubmarinePawn_C|GetCurrentRocket _submarineowning) TargetLocation)
      (Variables|/Game/Batyscaphe/submarine/BP_SubmarinePawn.BP_SubmarinePawn_C|SetCurrentRocket _submarineowning 0))))