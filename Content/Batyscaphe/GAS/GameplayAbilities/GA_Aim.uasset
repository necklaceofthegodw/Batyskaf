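; Gameplay ability that puts the submarine into aiming mode, showing a HUD crosshair that reflects whether a shootable target is under it.
; After committing, it loops on a short delay, tracing from screen center along the Visibility channel and coloring the crosshair when the hit actor implements I_Shootable.
; A tag-change listener on Abilities.Shoot hides the crosshair and ends the ability.
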(event Custom|OnShoot
  (params (Tag :type Gameplay%20Tag%20Structure%20%28by%20ref%29) (TagCount :type Integer))
  (if (== Tag "(TagName=\"Abilities.Shoot\")")
    (Default|ShowCrosshair (CallFunction|GetSubmarineHUDWidget) false)
    (Ability|EndAbility)))

(event Ability|EventActivateAbility
  (bind _returnvalue (Ability|GetAvatarActorfromActorInfo))
  (bind _wbp_hud (CallFunction|GetSubmarineHUDWidget))
  (bind _returnvalue_2 (Ability|CommitAbility))
  (if _returnvalue_2
    (bind _asbp_submarine_pawn (Utilities|Casting|CastToBP_SubmarinePawn _returnvalue))
    (Variables|Default|SetSubmarineOwning _asbp_submarine_pawn)
    (GameplayTags|BindEventWrappertoGameplayTagChanged (Ability|GetAbilitySystemComponent _returnvalue) "(TagName=\"Abilities.Shoot\")" (EventDispatchers|CreateEvent :!event Custom|OnShoot))
    (Default|ShowCrosshair _wbp_hud true)
    (Default|SetCrosshairColor _wbp_hud false)
    (bind _asi_shootable (CallFunction|IsShootableUnderCrosshair :!label _label))
    (Default|SetCrosshairColor _wbp_hud (Utilities|IsValidInterface _asi_shootable))
    (Utilities|FlowControl|Delay 0.05)
    (goto _label)))

(event Ability|EventOnEndAbility
  (params (bWasCancelled :type Boolean)))

(fn IsShootableUnderCrosshair
  (bind _returnvalue (Viewport|GetViewportSize))
  (bind _returnvalue_2 (Game|GetPlayerController 0))
  (bind (_x _y) (Math|Vector2D|BreakVector2D _returnvalue))
  (bind _returnvalue_3 (* _y 0.5))
  (bind _returnvalue_4 (* _x 0.5))
  (bind _returnvalue_5 (Math|Vector2D|MakeVector2D _returnvalue_4 _returnvalue_3))
  (bind (_worldposition _worlddirection) (Class|GameplayStatics|DeprojectScreentoWorld _returnvalue_2 _returnvalue_5))
  (bind (_outhit _returnvalue_6) (Collision|LineTraceByChannel _worldposition (+ _worldposition (* _worlddirection (LocalVariables|GetLineTraceLengthL))) "TraceTypeQuery1" false 0 "None" true "(R=1.000000,G=0.000000,B=0.000000,A=1.000000)" "(R=0.000000,G=1.000000,B=0.000000,A=1.000000)" 0.0))
  (if _returnvalue_6
    (bind _asi_shootable (Utilities|Casting|CastToI_Shootable (.HitActor (Collision|BreakHitResult _outhit)))
      (:then
        (return _asi_shootable))
      (:CastFailed
        _)))
  (return 0))