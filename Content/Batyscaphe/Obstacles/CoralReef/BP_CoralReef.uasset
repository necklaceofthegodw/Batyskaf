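; Coral reef obstacle for the submarine that grows when approached and explodes unless a rocket destroys it first.
; On spawn it sphere-traces for a surface and sets its pitch from the hit normal.
; Entering the trigger radius starts a scale timeline, which ends in a blast that penalizes a nearby submarine with a failed choice and negative stat-over-time.
; A rocket hit destroys both actors and reports a successful choice.
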(event OnComponentBeginOverlap(CollisionTrigger)
  (params (OverlappedComponent :type Primitive%20Component%20Object%20Reference) (OtherActor :type Actor%20Object%20Reference) (OtherComp :type Primitive%20Component%20Object%20Reference) (OtherBodyIndex :type Integer) (bFromSweep :type Boolean) (SweepResult :type Hit%20Result%20Structure%20%28by%20ref%29))
  (Utilities|Casting|CastToBP_SubmarinePawn OtherActor)
  (CallFunction|Grow))

(event Custom|Grow
  (bind _outsubmarinepawn (CallFunction|GetSubmarinePawn))
  (bind _scaletrack (Timeline|GrowTimeline PlayFromStart)
    (:Update
      (Transformation|SetActorScale3D (Math|Vector|Lerp(Vector) "10.000000,10.000000,10.000000" (Variables|Default|GetMaxScale) _scaletrack)))
    (:Finished
      (if (< (Transformation|GetDistanceTo _outsubmarinepawn) (Variables|Default|GetMinDistanceToEscape))
        (Default|CallOnChoiceMade _outsubmarinepawn false)
        (Default|AddStatDOT (Variables|/Game/Batyscaphe/submarine/BP_SubmarinePawn.BP_SubmarinePawn_C|GetBP_AttributeManager _outsubmarinepawn) "NewEnumerator2" -3e+02))
      (GameplayCue|ExecuteGameplayCueOnActor(Burst) _outsubmarinepawn "(TagName=\"GameplayCue.ShotBig\")" (Ability|GameplayCue|MakeGameplayCueParameters :Location (+ (Transformation|GetActorLocation) (* (Transformation|GetActorUpVector) 2e+03))))
      (Actor|DestroyActor))))

(event Custom|OnActorHit_Event
  (params (SelfActor :type Actor%20Object%20Reference) (OtherActor :type Actor%20Object%20Reference) (NormalImpulse :type Vector) (Hit :type Hit%20Result%20Structure%20%28by%20ref%29))
  (bind _asbp_rocket (Utilities|Casting|CastToBP_Rocket OtherActor))
  (Default|DestroyProjectile _asbp_rocket)
  (CallFunction|OnShot (CallFunction|GetSubmarinePawn)))

(event Custom|FindSpawnDirection
  (bind _returnvalue (Transformation|GetActorLocation))
  (bind _outhit (Collision|SphereTraceByChannel _returnvalue (+ _returnvalue (* (Transformation|GetActorForwardVector) 1e+02)) 8e+03 "TraceTypeQuery1" false 0 "Persistent"))
  (if (.bBlockingHit (Collision|BreakHitResult _outhit))
    (Variables|Default|SetProjectedRotation (Math|Rotator|MakeRotator 0.0 (+ (.Pitch (Math|Rotator|BreakRotator (Math|Rotator|MakeRotfromXY (.ImpactNormal (Collision|BreakHitResult _outhit)) (Math|Vector|NegateVector (Math|Vector|ProjectVectorontoPlane (Transformation|GetActorUpVector) (.ImpactNormal (Collision|BreakHitResult _outhit))))))) -9e+01) 0.0))
    (if (< (Math|Vector|DotProduct (Math|Vector|GetUpVector (Math|Rotator|MakeRotator 0.0 (+ (.Pitch (Math|Rotator|BreakRotator (Math|Rotator|MakeRotfromXY (.ImpactNormal (Collision|BreakHitResult _outhit)) (Math|Vector|NegateVector (Math|Vector|ProjectVectorontoPlane (Transformation|GetActorUpVector) (.ImpactNormal (Collision|BreakHitResult _outhit))))))) -9e+01) 0.0)) (Math|Vector|GetUpVector "0, 0, 0")) 0.0)
      (Transformation|SetActorRotation (Variables|Default|GetProjectedRotation))
      (Development|PrintString "FLIP")
      (else
        (Transformation|SetActorRotation (Variables|Default|GetProjectedRotation))
        (Development|PrintString "DONT FLIP")))))

(event EventBeginPlay
  (EventDispatchers|BindEventtoOnActorHit (delegate Custom|OnActorHit_Event))
  (CallFunction|FindSpawnDirection))

(event Collision|EventActorBeginOverlap
  (params (OtherActor :type Actor%20Object%20Reference)))

(event EventOnShot
  (params (SubmarineShooting :type BP%20Submarine%20Pawn%20Object%20Reference))
  (Audio|PlaySoundatLocation "/Game/Batyscaphe/Sounds/13_water_explosion_sheyvan.13_water_explosion_sheyvan" (Transformation|GetActorLocation) "0, 0, 0" 1.0 1.0 0.0 0 0 0 0)
  (Default|CallOnChoiceMade SubmarineShooting true)
  (GameplayCue|ExecuteGameplayCueOnActor(Burst) (CallFunction|GetSubmarinePawn) "(TagName=\"GameplayCue.ShotBig\")" (Ability|GameplayCue|MakeGameplayCueParameters :Location (Transformation|GetActorLocation)))
  (Actor|DestroyActor))

(fn ConstructionScript
  (Components|Sphere|SetSphereRadius (Variables|Default|GetCollisionTrigger) (Variables|Default|GetMinDistanceToTrigger) false))