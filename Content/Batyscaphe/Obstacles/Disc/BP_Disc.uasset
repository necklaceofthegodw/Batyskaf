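; Disc obstacle for the submarine that cycles open and closed, and shatters when rammed above its required speed.
; A looping timer drives the montage forward or reversed, with the material async-loaded from DiscInfo.
; Slower hits push the submarine back; fast hits swap the skeletal mesh for an impulsed Geometry Collection, temporarily alter speed and aerodynamics stats, then shrink and destroy the actor.
; Hits and box overlaps report the player's choice once.
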(event OnComponentHit(SkeletalMesh)
  (params (HitComponent :type Primitive%20Component%20Object%20Reference) (OtherActor :type Actor%20Object%20Reference) (OtherComp :type Primitive%20Component%20Object%20Reference) (NormalImpulse :type Vector :default "0, 0, 0") (Hit :type Hit%20Result%20Structure%20%28by%20ref%29))
  (if (not (Variables|Default|GetIsDestroyed))
    (bind _asbp_submarine_pawn (Utilities|Casting|CastToBP_SubmarinePawn OtherActor))
    (Variables|Default|SetSubmarineHit _asbp_submarine_pawn)
    (if (Variables|Default|GetChoiceMade)
      _
      (else
        (Default|CallOnChoiceMade (Variables|Default|GetSubmarineHit) true)
        (Variables|Default|SetChoiceMade true)))
    (Development|PrintString (Utilities|String|Append (Utilities|GetDisplayName OtherActor) " hit with speed: " (Utilities|String|ToString(Float) (Math|Vector|VectorLength (Variables|/Script/Engine.MovementComponent|GetVelocity (Variables|/Game/Batyscaphe/submarine/BP_SubmarinePawn.BP_SubmarinePawn_C|GetFloatingPawnMovement (Variables|Default|GetSubmarineHit)))))))
    (if (> (Math|Vector|VectorLength (Variables|/Script/Engine.MovementComponent|GetVelocity (Variables|/Game/Batyscaphe/submarine/BP_SubmarinePawn.BP_SubmarinePawn_C|GetFloatingPawnMovement (Variables|Default|GetSubmarineHit)))) (.RequiredSpeed (Utilities|Struct|BreakS_Disc (Variables|Default|GetDiscInfo))))
      (Components|Movement|StopMovementImmediately (Variables|/Game/Batyscaphe/submarine/BP_SubmarinePawn.BP_SubmarinePawn_C|GetFloatingPawnMovement (Variables|Default|GetSubmarineHit)))
      (Components|Tick|SetComponentTickEnabled (Variables|/Game/Batyscaphe/submarine/BP_SubmarinePawn.BP_SubmarinePawn_C|GetFloatingPawnMovement (Variables|Default|GetSubmarineHit)) false)
      (CallFunction|TearIntoPieces)
      (Variables|Default|SetIsDestroyed true)
      (else
        (Components|Movement|StopMovementImmediately (Variables|/Game/Batyscaphe/submarine/BP_SubmarinePawn.BP_SubmarinePawn_C|GetFloatingPawnMovement (Variables|Default|GetSubmarineHit)))
        (Components|Tick|SetComponentTickEnabled (Variables|/Game/Batyscaphe/submarine/BP_SubmarinePawn.BP_SubmarinePawn_C|GetFloatingPawnMovement (Variables|Default|GetSubmarineHit)) false)
        (CallFunction|MoveSubmarineBack)))
    (Components|Tick|SetComponentTickEnabled (Variables|/Game/Batyscaphe/submarine/BP_SubmarinePawn.BP_SubmarinePawn_C|GetFloatingPawnMovement (Variables|Default|GetSubmarineHit)) true)))

(event OnComponentBeginOverlap(Box)
  (params (OverlappedComponent :type Primitive%20Component%20Object%20Reference) (OtherActor :type Actor%20Object%20Reference) (OtherComp :type Primitive%20Component%20Object%20Reference) (OtherBodyIndex :type Integer) (bFromSweep :type Boolean) (SweepResult :type Hit%20Result%20Structure%20%28by%20ref%29))
  (bind _asbp_submarine_pawn (Utilities|Casting|CastToBP_SubmarinePawn OtherActor))
  (Utilities|FlowControl|DoOnce false
    (:Completed
      (if (not (Variables|Default|GetChoiceMade))
        (Default|CallOnChoiceMade _asbp_submarine_pawn (Utilities|IsValid (Variables|Default|GetSubmarineHit)))
        (Variables|Default|SetChoiceMade true)))))

(event Custom|PlayOpenCloseMontage
  (bind _montagehandle (Variables|Default|GetMontageHandle))
  (bind _skeletalmesh (Variables|Default|GetSkeletalMesh))
  (bind _returnvalue (Components|SkeletalMesh|GetAnimInstance _skeletalmesh))
  (if (not (Animation|Montage|MontageIsPlaying _returnvalue (Variables|Default|GetMontage%20to%20Play)))
    (Variables|Default|SetStartPos (Animation|Montage|MontageGetPosition _returnvalue (Variables|Default|GetMontage%20to%20Play)))
    (Variables|Default|SetIsClosing (not (Variables|Default|GetIsClosing)))
    (Utilities|Time|PauseTimerbyHandle _montagehandle)
    (if (Variables|Default|GetIsClosing)
      _
      (else
        (Utilities|FlowControl|Delay 3.0)))
    (Animation|Montage|MontageStop _returnvalue 0.0 (Variables|Default|GetMontage%20to%20Play))
    (Utilities|Time|UnpauseTimerbyHandle _montagehandle)
    (CallFunction|PlayDiscMontage)))

(event Custom|PlayDiscMontage
  (Animation|Montage|PlayMontage (Variables|Default|GetSkeletalMesh) (Variables|Default|GetMontage%20to%20Play) (Math|Float|SelectFloat 1.0 -1.0 (Variables|Default|GetIsClosing)) (Variables|Default|GetStartPos) "None" false))

(event Custom|MoveSubmarineBack
  (bind _submarinehit (Variables|Default|GetSubmarineHit))
  (Utilities|IsValid _submarinehit
    (:Is%20Valid
      (Timeline|MoveBack PlayFromStart
        (:Update
          (Pawn|Input|AddMovementInput _submarinehit (Math|Vector|NegateVector (Transformation|GetActorForwardVector _submarinehit)) 1e+03 false))))))

(event Custom|TearIntoPieces
  (bind _gc_disc (Variables|Default|GetGC_Disc))
  (bind _skeletalmesh (Variables|Default|GetSkeletalMesh))
  (Animation|Montage|MontageStop (Components|SkeletalMesh|GetAnimInstance (Variables|Default|GetSkeletalMesh)) 0.0 (Variables|Default|GetMontage%20to%20Play))
  (Utilities|Time|ClearandInvalidateTimerbyHandle (Variables|Default|GetMontageHandle))
  (Rendering|SetVisibility _skeletalmesh false false)
  (Physics|SetSimulatePhysics _skeletalmesh false)
  (Collision|SetCollisionEnabled _skeletalmesh "NoCollision")
  (Development|SetHiddeninGame _gc_disc false false)
  (Rendering|SetVisibility _gc_disc true false)
  (Collision|SetCollisionEnabled _gc_disc "QueryAndPhysics")
  (CallFunction|SetSubmarineStats false)
  (Physics|SetSimulatePhysics _gc_disc true)
  (Physics|AddRadialImpulse _gc_disc (+ (.Origin (Collision|GetComponentBounds _gc_disc)) "0.000000,0.000000,350.000000") 3e+02 (* (Math|Random|RandomFloatinRange 1.7e+03 3.4e+03) 0.2) "RIF_Constant" true)
  (Utilities|FlowControl|Delay 1.0)
  (Variables|Default|SetStartScale (Transformation|GetActorScale3D))
  (bind _size (Timeline|ShrinkPieces PlayFromStart)
    (:Update
      (Transformation|SetActorScale3D (Math|Vector|Lerp(Vector) (Variables|Default|GetStartScale) "0, 0, 0" _size)))
    (:Finished
      (CallFunction|SetSubmarineStats true)
      (Components|DestroyComponent _gc_disc)
      (Actor|DestroyActor))))

(event EventBeginPlay
  (bind _object (Utilities|AsyncLoadAsset (.DiscMaterial (Utilities|Struct|BreakS_Disc (Variables|Default|GetDiscInfo))))
    (:then
      (bind _returnvalue (Utilities|Time|SetTimerbyEvent (EventDispatchers|CreateEvent :!event Custom|PlayOpenCloseMontage) 0.5 true))
      (Variables|Default|SetMontageHandle _returnvalue))
    (:Completed
      (bind _asmaterial_instance (Utilities|Casting|CastToMaterialInstance _object))
      (Rendering|Material|SetMaterial (Variables|Default|GetSkeletalMesh) 0 _asmaterial_instance)
      (Rendering|Material|SetMaterial (Variables|Default|GetGC_Disc) 0 _asmaterial_instance))))

(event Collision|EventActorBeginOverlap
  (params (OtherActor :type Actor%20Object%20Reference)))

(event EventTick
  (params (DeltaSeconds :type Float%20%28single-precision%29)))

(fn ConstructionScript)

(fn GetRequiredSpeedValues
  (bind _outrownames (DataTable|GetDataTableRowNames "/Game/Batyscaphe/UI/UpgradeSystem/Data/DT_Upgrades.DT_Upgrades"))
  (for _array_element _outrownames
    (bind _returnvalue (Utilities|GetDataTableRow "/Game/Batyscaphe/UI/UpgradeSystem/Data/DT_Upgrades.DT_Upgrades" _array_element)
      (:then
        (if (Utilities|Enum|Equal(Enum) (.UpgradeType (Utilities|Struct|BreakS_UpgradeRow _returnvalue)) "NewEnumerator0")
          (Variables|Default|SetRequiredSpeedValues (.Value (Utilities|Struct|BreakS_UpgradeRow _returnvalue))))))))

(fn SetSubmarineStats
  (params (SetBack :type Boolean))
  (bind _submarinehit (Variables|Default|GetSubmarineHit))
  (bind _returnvalue (Ability|GetAbilitySystemComponent _submarinehit))
  (bind _bp_attributemanager (Variables|/Game/Batyscaphe/submarine/BP_SubmarinePawn.BP_SubmarinePawn_C|GetBP_AttributeManager _submarinehit))
  (bind _returnvalue_2 (Class|AbilitySystemComponent|GetGameplayAttributeValue _returnvalue "(AttributeName=\"Aerodynamics\",Attribute=/Script/Batyskaf.SubmarineAttributeSet:Aerodynamics,AttributeOwner=\"/Script/CoreUObject.Class'/Script/Batyskaf.SubmarineAttributeSet'\")"))
  (bind _returnvalue_3 (Class|AbilitySystemComponent|GetGameplayAttributeValue _returnvalue "(AttributeName=\"MaxSpeed\",Attribute=/Script/Batyskaf.SubmarineAttributeSet:MaxSpeed,AttributeOwner=\"/Script/CoreUObject.Class'/Script/Batyskaf.SubmarineAttributeSet'\")"))
  (if SetBack
    (Default|SetStat _bp_attributemanager "NewEnumerator0" (Variables|Default|GetMaxSpeed))
    (Default|SetStat _bp_attributemanager "NewEnumerator1" (Variables|Default|GetMaxAerodynamics))
    (else
      (Variables|Default|SetMaxSpeed _returnvalue_3)
      (Variables|Default|SetMaxAerodynamics _returnvalue_2)
      (Default|SetStat _bp_attributemanager "NewEnumerator0" (* _returnvalue_3 0.3))
      (Default|SetStat _bp_attributemanager "NewEnumerator1" (* _returnvalue_2 3.0)))))