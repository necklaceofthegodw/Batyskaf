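; Disc obstacle that repeatedly opens and closes through an animation montage and shatters when hit.
; A looping timer drives the montage, which alternates forward and reverse play with a pause before each reverse run.
; The first hit from any actor (the SubmarinePawn cast is unwired) stops the cycle, hides the skeletal mesh and reveals GCDisc, simulated with a random-strength radial impulse.
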(event OnComponentHit(SkeletalMesh)
  (params (HitComponent :type Primitive%20Component%20Object%20Reference) (OtherActor :type Actor%20Object%20Reference) (OtherComp :type Primitive%20Component%20Object%20Reference) (NormalImpulse :type Vector :default "0, 0, 0") (Hit :type Hit%20Result%20Structure%20%28by%20ref%29))
  (if (not (Variables|Default|GetIsDestroyed))
    (Development|PrintString (Utilities|GetDisplayName OtherActor))
    (CallFunction|TearIntoPieces)
    (Variables|Default|SetIsDestroyed true)))

(event Custom|PlayOpenCloseMontage
  (bind _montagehandle (Variables|Default|GetMontageHandle))
  (bind _skeletalmesh (Variables|Default|GetSkeletalMesh))
  (bind _returnvalue (Components|SkeletalMesh|GetAnimInstance _skeletalmesh))
  (if (not (Animation|Montage|MontageIsPlaying _returnvalue (Variables|Default|GetMontage%20to%20Play)))
    (Variables|Default|SetStartPos (Animation|Montage|MontageGetPosition _returnvalue (Variables|Default|GetMontage%20to%20Play)))
    (Variables|Default|SetIsClosing (not (Variables|Default|GetIsClosing)))
    (Utilities|Time|PauseTimerbyHandle _montagehandle)
    (if (Variables|Default|GetIsClosing)
      _
      (else
        (Utilities|FlowControl|Delay 3.0)))
    (Animation|Montage|MontageStop _returnvalue 0.0 (Variables|Default|GetMontage%20to%20Play))
    (Utilities|Time|UnpauseTimerbyHandle _montagehandle)
    (CallFunction|PlayDiscMontage)))

(event Custom|PlayDiscMontage
  (Animation|Montage|PlayMontage (Variables|Default|GetSkeletalMesh) (Variables|Default|GetMontage%20to%20Play) (Math|Float|SelectFloat 1.0 -1.0 (Variables|Default|GetIsClosing)) (Variables|Default|GetStartPos) "None" false))

(event EventBeginPlay
  (CallFunction|PlayOpenCloseMontage)
  (bind _returnvalue (Utilities|Time|SetTimerbyEvent (EventDispatchers|CreateEvent :!event Custom|PlayOpenCloseMontage) 0.5 true))
  (Variables|Default|SetMontageHandle _returnvalue))

(event Collision|EventActorBeginOverlap
  (params (OtherActor :type Actor%20Object%20Reference)))

(event EventTick
  (params (DeltaSeconds :type Float%20%28single-precision%29)))

(fn ConstructionScript)

(fn TearIntoPieces
  (bind _skeletalmesh (Variables|Default|GetSkeletalMesh))
  (bind _gc_disc (Variables|Default|GetGC_Disc))
  (Animation|Montage|MontageStop (Components|SkeletalMesh|GetAnimInstance (Variables|Default|GetSkeletalMesh)) 0.0 (Variables|Default|GetMontage%20to%20Play))
  (Utilities|Time|ClearandInvalidateTimerbyHandle (Variables|Default|GetMontageHandle))
  (Rendering|SetVisibility _skeletalmesh false false)
  (Physics|SetSimulatePhysics _skeletalmesh false)
  (Collision|SetCollisionEnabled _skeletalmesh "NoCollision")
  (Development|SetHiddeninGame _gc_disc false false)
  (Rendering|SetVisibility _gc_disc true false)
  (Collision|SetCollisionEnabled _gc_disc "QueryAndPhysics")
  (Physics|SetSimulatePhysics _gc_disc true)
  (Physics|AddRadialImpulse _gc_disc (+ (.Origin (Collision|GetComponentBounds _gc_disc)) "0.000000,0.000000,350.000000") 3e+02 (Math|Random|RandomFloatinRange 1.7e+03 3.4e+03) "RIF_Constant" true))