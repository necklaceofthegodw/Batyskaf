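; BP_ChoiceDisc is an obstacle that offers a choice between two different random upgrades.
; On BeginPlay it shuffles all upgrade enum indices and takes the first two, so the options never repeat.
; It spawns a BP_PowerUp at each of its two spawn points, passing the type and choice index, with the player pawn as owner.
; When destroyed, it also destroys any remaining spawned power-ups.
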(event EventBeginPlay
  (bind _outupgradetypes (CallFunction|GetTwoRandomUpgradeTypes))
  (Variables|Default|SetUpgradeTypes _outupgradetypes)
  (CallFunction|SpawnPowerUps))

(event Collision|EventActorBeginOverlap
  (params (OtherActor :type Actor%20Object%20Reference)))

(event EventTick
  (params (DeltaSeconds :type Float%20%28single-precision%29)))

(event EventDestroyed
  (for _array_element (Variables|Default|GetSpawnedPowerups)
    (Utilities|IsValid _array_element
      (:Is%20Valid
        (Actor|DestroyActor _array_element))))
  (|CallParentFunction))

(fn ConstructionScript)

(fn SpawnPowerUps
  (bind _output_get (LocalVariables|SetSpawnPointsL (Utilities|Array|MakeArray (Variables|Default|GetSpawn1) (Variables|Default|GetSpawn2))))
  (for (_array_element _array_index) _output_get
    (bind _returnvalue (Game|SpawnActorfromClass "/Game/Batyscaphe/Obstacles/ChoiceObstacle/BP_PowerUp.BP_PowerUp_C" (Math|Transform|MakeTransform (Transformation|GetWorldLocation _array_element) (Math|Rotator|MakeRotfromX (Transformation|GetActorForwardVector))) "Undefined" "MultiplyWithRoot" (Game|Player|GetPlayerPawn 0) (Utilities|Array|Get(acopy) (Variables|Default|GetUpgradeTypes) _array_index) 5.0 _array_index 0))
    (Utilities|Array|Add (Variables|Default|GetSpawnedPowerups) _returnvalue)))

(fn GetTwoRandomUpgradeTypes
  (bind _upgradeindicesl (LocalVariables|GetUpgradeIndicesL))
  (for _index (range 0 (- (|GetNumEnumEntries) 1))
    (Utilities|Array|Add _upgradeindicesl _index))
  (Utilities|Array|Shuffle _upgradeindicesl)
  (return (Utilities|Array|MakeArray (Utilities|Enum|ByteToEnumE_UpgradeType (Math|Conversions|ToByte(Integer) (Utilities|Array|Get(acopy) (LocalVariables|GetUpgradeIndicesL)))) (Utilities|Enum|ByteToEnumE_UpgradeType (Math|Conversions|ToByte(Integer) (Utilities|Array|Get(acopy) (LocalVariables|GetUpgradeIndicesL) 1))))))