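; BP_PowerUp is a submarine pickup that grants one upgrade, chosen by its UpgradeType.
; On the first overlap of its disc by BP_SubmarinePawn, it charges the battery for one type or passes the mapped value to the attribute manager's AddStatDOT, then destroys itself.
; The construction script searches DT_Upgrades for the matching type and sets that row's image on a dynamic decal material.
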(event OnComponentBeginOverlap(SM_Disc)
  (params (OverlappedComponent :type Primitive%20Component%20Object%20Reference) (OtherActor :type Actor%20Object%20Reference) (OtherComp :type Primitive%20Component%20Object%20Reference) (OtherBodyIndex :type Integer) (bFromSweep :type Boolean) (SweepResult :type Hit%20Result%20Structure%20%28by%20ref%29))
  (bind _upgradetype (Variables|Default|GetUpgradeType))
  (bind _asbp_submarine_pawn (Utilities|Casting|CastToBP_SubmarinePawn OtherActor))
  (Utilities|FlowControl|DoOnce false
    (:Completed
      (if (Utilities|Enum|Equal(Enum) _upgradetype "NewEnumerator3")
        (Default|ChargeBattery _asbp_submarine_pawn)
        (else
          (Default|AddStatDOT (Variables|/Game/Batyscaphe/submarine/BP_SubmarinePawn.BP_SubmarinePawn_C|GetBP_AttributeManager _asbp_submarine_pawn) _upgradetype (.Value (Utilities|Map|Find (Variables|Default|GetUpgradesToValues) _upgradetype)))))
      (Actor|DestroyActor))))

(event EventBeginPlay)

(event Collision|EventActorBeginOverlap
  (params (OtherActor :type Actor%20Object%20Reference)))

(event EventTick
  (params (DeltaSeconds :type Float%20%28single-precision%29)))

(fn ConstructionScript
  (CallFunction|SetDecalTexturebyUpgradeType))

(fn SetDecalTexturebyUpgradeType
  (bind _returnvalue (Rendering|Material|CreateDynamicMaterialInstance (Variables|Default|GetDecal) :!class /Script/Engine.DecalComponent))
  (bind _outrownames (DataTable|GetDataTableRowNames "/Game/Batyscaphe/UI/UpgradeSystem/Data/DT_Upgrades.DT_Upgrades"))
  (for _array_element _outrownames
    (bind _returnvalue_2 (Utilities|GetDataTableRow "/Game/Batyscaphe/UI/UpgradeSystem/Data/DT_Upgrades.DT_Upgrades" _array_element)
      (:then
        (if (Utilities|Enum|Equal(Enum) (.UpgradeType (Utilities|Struct|BreakS_UpgradeRow _returnvalue_2)) (Variables|Default|GetUpgradeType))
          (Rendering|Material|SetTextureParameterValue _returnvalue "PowerupTexture" (.Image (Utilities|Struct|BreakS_UpgradeRow _returnvalue_2))))))))