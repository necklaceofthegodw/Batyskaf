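; BP_MeteorSpawner is an obstacle actor that hurls BP_Meteor actors at the submarine when it comes within MinDistanceToPlayer.
; Tick checks distance and starts a looping one-second timer that spawns meteors at random points in a surrounding sphere.
; Each gets a velocity-change impulse aimed ahead of the submarine along its forward vector, scaled by speed.
; Leaving range clears the timer and destroys spawned meteors; un-reset DoOnce gates make this a one-time cycle.
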(event Custom|MoveMeteorTowardsPlayer
  (params (MeteorToMove :type BP%20Meteor%20Object%20Reference))
  (bind _outsubmarinepawn (CallFunction|GetSubmarinePawn))
  (Physics|AddImpulse (Variables|/Game/Batyscaphe/Obstacles/MeteorObstacle/BP_Meteor.BP_Meteor_C|GetSM_Meteor MeteorToMove) (* (Math|Vector|Normalize (- (+ (Transformation|GetActorLocation _outsubmarinepawn) (* (Transformation|GetActorForwardVector _outsubmarinepawn) (Math|Vector|VectorLength (Variables|/Script/Engine.MovementComponent|GetVelocity (Variables|/Game/Batyscaphe/submarine/BP_SubmarinePawn.BP_SubmarinePawn_C|GetFloatingPawnMovement _outsubmarinepawn))))) (Transformation|GetActorLocation MeteorToMove))) (Variables|Default|GetForceToApply)) "None" true))

(event EventBeginPlay)

(event Collision|EventActorBeginOverlap
  (params (OtherActor :type Actor%20Object%20Reference)))

(event EventTick
  (params (DeltaSeconds :type Float%20%28single-precision%29))
  (if (< (Transformation|GetDistanceTo (CallFunction|GetSubmarinePawn) self) (Variables|Default|GetMinDistanceToPlayer))
    (if (not (Variables|Default|GetSpawnerActive))
      (Utilities|FlowControl|DoOnce false
        (:Completed
          (Variables|Default|SetSpawnerActive true)
          (Development|PrintString "ACTIVATE SPAWNER")
          (bind _returnvalue (Utilities|Time|SetTimerbyFunctionName 0 "SpawnMeteors" 1.0 true))
          (Variables|Default|SetMeteorSpawnerHandle _returnvalue))))
    (elif (Variables|Default|GetSpawnerActive)
      (Utilities|FlowControl|DoOnce false
        (:Completed
          (CallFunction|DespawnMeteors)
          (Development|PrintString "DEACTIVATE SPAWNER"))))))

(fn ConstructionScript)

(fn SpawnMeteors
  (bind _returnvalue (Game|SpawnActorfromClass "/Game/Batyscaphe/Obstacles/MeteorObstacle/BP_Meteor.BP_Meteor_C" (Math|Conversions|ToTransform(Vector) (CallFunction|GetRandomLocationinSphere (Transformation|GetActorLocation) 5e+03)) "Undefined" "MultiplyWithRoot" 0 0))
  (Utilities|Array|Add (Variables|Default|GetSpawnedMeteors) _returnvalue)
  (CallFunction|MoveMeteorTowardsPlayer _returnvalue))

(fn DespawnMeteors
  (Utilities|Time|ClearandInvalidateTimerbyHandle (Variables|Default|GetMeteorSpawnerHandle))
  (for _array_element (Variables|Default|GetSpawnedMeteors)
    (Utilities|IsValid _array_element
      (:Is%20Valid
        (Actor|DestroyActor _array_element)))))