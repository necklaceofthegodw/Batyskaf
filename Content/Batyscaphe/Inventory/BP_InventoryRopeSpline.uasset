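; Inventory rope actor that displays collected items as a chain trailing along a spline.
; AddItemAtEnd extends the spline along the actor's forward vector, alternating between spawning a BP_TestRope3 segment with the item as base mesh and hanging the item on the last segment.
; Each segment attaches to the previous one.
; An older static-mesh path with socket-to-socket cables remains, but its entry calls are disconnected.
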(event Custom|AddItemAtEnd
  (params (CollectableToAdd :type BP%20Collectable%202%20Object%20Reference))
  (bind _spline (Variables|Default|GetSpline))
  (bind _ropes (Variables|Default|GetRopes))
  (bind _returnvalue (Utilities|Array|Length _ropes))
  (bind _returnvalue_2 (Spline|GetNumberOfSplinePoints _spline))
  (Variables|Default|SetSplinePoints _returnvalue_2)
  (Spline|AddSplinePoint _spline (+ (Transformation|GetActorLocation) (* (Transformation|GetActorForwardVector) (Variables|Default|GetCableLength) _returnvalue_2)) "World" true)
  (if (== (Math|Integer|%(Integer) (Utilities|Array|Length (Variables|Default|GetCollectedItems)) 2) 0)
    (CallFunction|AddRopeFragmenttoSpline (Variables|Default|GetSplinePoints) CollectableToAdd)
    (Development|PrintString (Utilities|String|Append "add base item: " (Utilities|GetDisplayName CollectableToAdd)))
    (Utilities|Array|Add (Variables|Default|GetCollectedItems) CollectableToAdd :!label _label)
    (elif (> _returnvalue 0)
      (Default|SetandEnableHangingMesh (Utilities|Array|Get(acopy) _ropes (- _returnvalue 1)) CollectableToAdd)
      (Development|PrintString (Utilities|String|Append "add hanging item: " (Utilities|GetDisplayName CollectableToAdd)))
      (goto _label))))

(event EventBeginPlay)

(event Collision|EventActorBeginOverlap
  (params (OtherActor :type Actor%20Object%20Reference)))

(event EventTick
  (params (DeltaSeconds :type Float%20%28single-precision%29)))

(fn ConstructionScript)

(fn SetCableProperties
  (params (cableInfoToSet :type S%20Cable%20Info%20Structure))
  (bind (_cableref _splineposition _mesh _cablesocket _endpoint _cablelength) (Utilities|Struct|BreakS_CableInfo cableInfoToSet))
  (Variables|/Script/CableComponent.CableComponent|SetEndLocation _cableref _endpoint)
  (Variables|/Script/CableComponent.CableComponent|SetCableLength _cableref _cablelength)
  (Variables|/Script/CableComponent.CableComponent|SetSolverIterations _cableref 10)
  (Variables|/Script/CableComponent.CableComponent|SetbEnableStiffness _cableref false))

(fn SpawnMeshesAlongtheSpline
  (Spline|ClearSplinePoints (Variables|Default|GetSpline) true)
  (for _index (range 0 (- (Variables|Default|GetInitialItemsNum) 1))
    (Spline|AddSplinePoint (Variables|Default|GetSpline) (+ (Transformation|GetActorLocation) (* (Transformation|GetActorForwardVector) (Variables|Default|GetCableLength) _index)) "World" true)
    (bind _spawnedmesh (CallFunction|AddMeshtoSpline _index (Variables|Default|GetInitialMesh)))
    (Utilities|Array|Add (LocalVariables|GetMeshesL) _spawnedmesh))
  (return (LocalVariables|GetMeshesL)))

(fn AddMeshtoSpline
  (params (PointIndex :type Integer) (MeshToAdd :type Static%20Mesh%20Object%20Reference))
  (bind _spline (Variables|Default|GetSpline))
  (bind _returnvalue (AddComponent|AddStaticMeshComponent false (Math|Conversions|ToTransform(Vector) (Spline|GetLocationatSplinePoint _spline PointIndex "Local"))))
  (Components|StaticMesh|SetStaticMesh _returnvalue MeshToAdd)
  (Transformation|SetRelativeRotation _returnvalue (Spline|GetRotationatSplinePoint _spline PointIndex "Local") false false)
  (return _returnvalue))

(fn UpdateItems
  (bind _outmeshcomponents (CallFunction|SpawnMeshesAlongtheSpline))
  (bind _output_get (Variables|Default|SetMeshes _outmeshcomponents))
  (for (_ _array_index) _output_get
    (CallFunction|AddCableatIndex _array_index)))

(fn AddCableatIndex
  (params (Index :type Integer))
  (LocalVariables|SetCurrentIndexL Index)
  (for _array_element (Transformation|GetAllSocketNames (Utilities|Array|Get(acopy) (Variables|Default|GetMeshes) (LocalVariables|GetCurrentIndexL)))
    (LocalVariables|SetCurrentSocketNameL _array_element)
    (Utilities|IsValid (Utilities|Array|Get(acopy) (Variables|Default|GetMeshes) (+ (LocalVariables|GetCurrentIndexL) 1))
      (:Is%20Valid
        (bind _returnvalue (AddComponent|AddCableComponent false (Math|Conversions|ToTransform(Vector) (Math|Transform|InverseTransformLocation (Transformation|GetActorTransform) (Transformation|GetSocketLocation (Utilities|Array|Get(acopy) (Variables|Default|GetMeshes) (LocalVariables|GetCurrentIndexL)) (LocalVariables|GetCurrentSocketNameL))))))
        (CallFunction|SetCableProperties (Utilities|Struct|MakeS_CableInfo _returnvalue (LocalVariables|GetCurrentIndexL) 0 (LocalVariables|GetCurrentSocketNameL) (Math|Transform|InverseTransformLocation (Transformation|GetActorTransform) (Transformation|GetSocketLocation (Utilities|Array|Get(acopy) (Variables|Default|GetMeshes) (+ (LocalVariables|GetCurrentIndexL) 1)) (LocalVariables|GetCurrentSocketNameL))) (Math|Vector|VectorLength (- (Math|Transform|InverseTransformLocation (Transformation|GetActorTransform) (Transformation|GetSocketLocation (Utilities|Array|Get(acopy) (Variables|Default|GetMeshes) (LocalVariables|GetCurrentIndexL)) (LocalVariables|GetCurrentSocketNameL))) (Math|Transform|InverseTransformLocation (Transformation|GetActorTransform) (Transformation|GetSocketLocation (Utilities|Array|Get(acopy) (Variables|Default|GetMeshes) (+ (LocalVariables|GetCurrentIndexL) 1)) (LocalVariables|GetCurrentSocketNameL)))))))))))

(fn AddCollectabletoSpline
  (params (PointIndex :type Integer) (CollectableActor :type BP%20Collectable%202%20Object%20Reference))
  (bind _spline (Variables|Default|GetSpline))
  (bind _returnvalue (AddComponent|AddStaticMeshComponent false (Math|Conversions|ToTransform(Vector) (Spline|GetLocationatSplinePoint _spline PointIndex "Local"))))
  (Components|StaticMesh|SetStaticMesh _returnvalue (Variables|/Script/Engine.StaticMeshComponent|GetStaticMesh (Variables|/Game/Batyscaphe/Collectables/BP_Collectable2.BP_Collectable2_C|GetSM_CollectableMesh CollectableActor)))
  (Transformation|SetRelativeRotation _returnvalue (Spline|GetRotationatSplinePoint _spline PointIndex "Local") false false)
  (Transformation|AttachActorToActor CollectableActor self "None" "SnapToTarget" "SnapToTarget" "SnapToTarget" true)
  (Physics|SetSimulatePhysics _returnvalue false)
  (return _returnvalue))

(fn AddRopeFragmenttoSpline
  (params (PointIndex :type Integer) (CurrentCollectable :type BP%20Collectable%202%20Object%20Reference))
  (bind _spline (Variables|Default|GetSpline))
  (bind _ropes (Variables|Default|GetRopes))
  (bind _returnvalue (Utilities|Array|Length _ropes))
  (bind _returnvalue_2 (Game|SpawnActorfromClass "/Game/Batyscaphe/Inventory/BP_TestRope3.BP_TestRope3_C" (Math|Transform|MakeTransform (Spline|GetLocationatSplinePoint _spline PointIndex "World") (Spline|GetRotationatSplinePoint _spline PointIndex "World")) "Undefined" "MultiplyWithRoot" 0 0))
  (Default|SetBaseMesh _returnvalue_2 CurrentCollectable)
  (if (== _returnvalue 0)
    (Transformation|AttachActorToActor _returnvalue_2 self "None" "KeepWorld" "KeepWorld" "KeepWorld" true)
    (else
      (Transformation|AttachActorToActor _returnvalue_2 (Utilities|Array|Get(acopy) _ropes (- _returnvalue 1)) "None" "KeepWorld" "KeepWorld" "KeepWorld" true)))
  (Utilities|Array|Add (Variables|Default|GetRopes) _returnvalue_2))