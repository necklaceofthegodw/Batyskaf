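; Test actor for a rope in the bathyscaphe inventory that displays collectable meshes on a base and a hanging component.
; SetBaseMesh copies a collectable's static mesh onto the base.
; SetAndEnableHangingMesh copies one onto the hanging object, shows it and enables actor collision.
; After a short delay it turns on physics simulation for the hanging object, then reattaches it to the base with relative transforms.
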(event Custom|SetAndEnableHangingMesh
  (params (Collectable :type BP%20Collectable%202%20Object%20Reference))
  (bind _sm_hangingobject (Variables|Default|GetSM_HangingObject))
  (Components|StaticMesh|SetStaticMesh _sm_hangingobject (Variables|/Script/Engine.StaticMeshComponent|GetStaticMesh (Variables|/Game/Batyscaphe/Collectables/BP_Collectable2.BP_Collectable2_C|GetSM_CollectableMesh Collectable)))
  (Rendering|SetVisibility _sm_hangingobject true false)
  (Collision|SetActorEnableCollision true)
  (Utilities|FlowControl|Delay 5.0)
  (Physics|SetSimulatePhysics _sm_hangingobject true)
  (Transformation|AttachComponentToComponent (Variables|Default|GetSM_HangingObject) (Variables|Default|GetSM_Base) "None" "KeepRelative" "KeepRelative" "KeepRelative" true))

(event EventBeginPlay)

(event Collision|EventActorBeginOverlap
  (params (OtherActor :type Actor%20Object%20Reference)))

(event EventTick
  (params (DeltaSeconds :type Float%20%28single-precision%29)))

(fn ConstructionScript)

(fn SetBaseMesh
  (params (Collectable :type BP%20Collectable%202%20Object%20Reference))
  (Components|StaticMesh|SetStaticMesh (Variables|Default|GetSM_Base) (Variables|/Script/Engine.StaticMeshComponent|GetStaticMesh (Variables|/Game/Batyscaphe/Collectables/BP_Collectable2.BP_Collectable2_C|GetSM_CollectableMesh Collectable))))