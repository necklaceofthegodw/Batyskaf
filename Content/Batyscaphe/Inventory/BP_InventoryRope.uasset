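; BP_InventoryRope is a bathyscaphe inventory actor that procedurally builds a rope-linked row of meshes.
; Its construction script resets the spline to evenly spaced points along the actor's forward vector and adds InitialMesh at each.
; UpdateItems then links same-named sockets on neighboring meshes with cable components, sized to the socket distance with stiffness disabled.
; AddItemAtEnd is an empty stub, and the branch that reuses existing spline points never runs.
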(event Custom|AddItemAtEnd)

(event EventBeginPlay)

(event Collision|EventActorBeginOverlap
  (params (OtherActor :type Actor%20Object%20Reference)))

(event EventTick
  (params (DeltaSeconds :type Float%20%28single-precision%29)))

(fn ConstructionScript
  (CallFunction|UpdateItems))

(fn SetCableProperties
  (params (cableInfoToSet :type S%20Cable%20Info%20Structure))
  (bind (_cableref _splineposition _mesh _cablesocket _endpoint _cablelength) (Utilities|Struct|BreakS_CableInfo cableInfoToSet))
  (Variables|/Script/CableComponent.CableComponent|SetEndLocation _cableref _endpoint)
  (Variables|/Script/CableComponent.CableComponent|SetCableLength _cableref _cablelength)
  (Variables|/Script/CableComponent.CableComponent|SetSolverIterations _cableref 10)
  (Variables|/Script/CableComponent.CableComponent|SetbEnableStiffness _cableref false))

(fn SpawnMeshesAlongtheSpline
  (Spline|ClearSplinePoints (Variables|Default|GetSpline) true)
  (for _index (range 0 (- (Variables|Default|GetInitialItemsNum) 1))
    (Spline|AddSplinePoint (Variables|Default|GetSpline) (+ (Transformation|GetActorLocation) (* (Transformation|GetActorForwardVector) (Variables|Default|GetCableLength) _index)) "World" true)
    (bind _spawnedmesh (CallFunction|AddMeshtoSpline _index (Variables|Default|GetInitialMesh)))
    (Utilities|Array|Add (LocalVariables|GetMeshesL) _spawnedmesh))
  (return (LocalVariables|GetMeshesL)))

(fn AddMeshtoSpline
  (params (PointIndex :type Integer) (MeshToAdd :type Static%20Mesh%20Object%20Reference))
  (bind _spline (Variables|Default|GetSpline))
  (bind _returnvalue (AddComponent|AddStaticMeshComponent false (Math|Conversions|ToTransform(Vector) (Spline|GetLocationatSplinePoint _spline PointIndex "Local"))))
  (Components|StaticMesh|SetStaticMesh _returnvalue MeshToAdd)
  (Transformation|SetRelativeRotation _returnvalue (Spline|GetRotationatSplinePoint _spline PointIndex "Local") false false)
  (return _returnvalue))

(fn UpdateItems
  (bind _outmeshcomponents (CallFunction|SpawnMeshesAlongtheSpline))
  (bind _output_get (LocalVariables|SetMeshesL _outmeshcomponents))
  ;[1 1 1] Setup cables
  (for (_array_element _array_index) _output_get
    (LocalVariables|SetCurrentMeshL _array_element)
    (LocalVariables|SetCurrentIndexL _array_index)
    (for _array_element_2 (Transformation|GetAllSocketNames (LocalVariables|GetCurrentMeshL))
      (LocalVariables|SetCurrentSocketNameL _array_element_2)
      (Utilities|IsValid (Utilities|Array|Get(acopy) (LocalVariables|GetMeshesL) (+ (LocalVariables|GetCurrentIndexL) 1))
        (:Is%20Valid
          (bind _returnvalue (AddComponent|AddCableComponent false (Math|Conversions|ToTransform(Vector) (Math|Transform|InverseTransformLocation (Transformation|GetActorTransform) (Transformation|GetSocketLocation (LocalVariables|GetCurrentMeshL) (LocalVariables|GetCurrentSocketNameL))))))
          (LocalVariables|SetCurrentCableL _returnvalue)
          (CallFunction|SetCableProperties (Utilities|Struct|MakeS_CableInfo (LocalVariables|GetCurrentCableL) (LocalVariables|GetCurrentIndexL) 0 (LocalVariables|GetCurrentSocketNameL) (Math|Transform|InverseTransformLocation (Transformation|GetActorTransform) (Transformation|GetSocketLocation (Utilities|Array|Get(acopy) (LocalVariables|GetMeshesL) (+ (LocalVariables|GetCurrentIndexL) 1)) (LocalVariables|GetCurrentSocketNameL))) (Math|Vector|VectorLength (- (Math|Transform|InverseTransformLocation (Transformation|GetActorTransform) (Transformation|GetSocketLocation (LocalVariables|GetCurrentMeshL) (LocalVariables|GetCurrentSocketNameL))) (Math|Transform|InverseTransformLocation (Transformation|GetActorTransform) (Transformation|GetSocketLocation (Utilities|Array|Get(acopy) (LocalVariables|GetMeshesL) (+ (LocalVariables|GetCurrentIndexL) 1)) (LocalVariables|GetCurrentSocketNameL))))))))))))